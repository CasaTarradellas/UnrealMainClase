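; Ashe's weapon Blueprint, a hitscan gun that extends a parent weapon class's initialize, fire and reload logic.
; Fire traces from Ashe's camera within the current spread cone, damages HealthSystem components with head-bone headshot detection, charges the ultimate and pushes physics objects.
; Each shot also triggers the animation, cooldown and vertical recoil.
; Reload picks a long or short time and animation based on whether ammo is empty.
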(event EventFire
  (bind _currentspread (Variables|Default|GetCurrentSpread))
  (bind _owningcharacter (Variables|Default|GetOwningCharacter))
  (bind _firedistance (Variables|Default|GetFireDistance))
  (bind _asashe_bp (Utilities|Casting|CastToAshe_BP _owningcharacter))
  (bind _camera (Variables|/Game/_Project/Characters/BaseCharacter_BP.BaseCharacter_BP_C|GetCamera _asashe_bp))
  (bind _returnvalue (Transformation|GetWorldLocation _camera))
  (bind _returnvalue_2 (Math|Vector|GetForwardVector _camera))
  (bind _returnvalue_3 (Math|Random|RandomUnitVectorinConeinDegrees _returnvalue_2 _currentspread))
  (bind _returnvalue_4 (* _returnvalue_3 _firedistance))
  (bind _returnvalue_5 (+ _returnvalue _returnvalue_4))
  (Utilities|FlowControl|Sequence
    (:then_0
      (bind (_outhit _returnvalue_6) (Collision|LineTraceByChannel _returnvalue _returnvalue_5 "TraceTypeQuery1" false 0 "ForDuration"))
      (if _returnvalue_6
        (Utilities|FlowControl|Sequence
          (:then_0
            (Utilities|IsValid (Actor|GetComponentbyClass (.HitActor (Collision|BreakHitResult _outhit)) "/Game/_Project/CommonSystems/HealthSystem/HealthSystem.HealthSystem_C")
              (:Is%20Valid
                (Default|TakeDamage (Actor|GetComponentbyClass (.HitActor (Collision|BreakHitResult _outhit)) "/Game/_Project/CommonSystems/HealthSystem/HealthSystem.HealthSystem_C") (== (.HitBoneName (Collision|BreakHitResult _outhit)) "Head") (Variables|Default|GetDamage))
                (Default|AddCharge (Variables|/Game/_Project/Characters/BaseCharacter_BP.BaseCharacter_BP_C|GetUltimate (Variables|Default|GetOwningCharacter)) (Math|Float|SelectFloat (Variables|Default|GetUltimate%20Charge%20Per%20Headshot) (Variables|Default|GetUltimate%20Charge%20Per%20Hit) (== (.HitBoneName (Collision|BreakHitResult _outhit)) "Head"))))))
          (:then_1
            (Utilities|IsValid (.HitComponent (Collision|BreakHitResult _outhit))
              (:Is%20Valid
                (if (Physics|IsSimulatingPhysics (.HitComponent (Collision|BreakHitResult _outhit)) "None")
                  (Physics|AddImpulseatLocation (.HitComponent (Collision|BreakHitResult _outhit)) _returnvalue_5 (.ImpactPoint (Collision|BreakHitResult _outhit)) "None"))))))))
    (:then_1
      (|CallParentFunction))
    (:then_2
      (Default|Fire (Variables|Default|GetAnimator))
      (CallFunction|EnterFireCooldown))
    (:then_3
      (CallFunction|AddRecoil 0.2 0.0))))

(event EventInitialize
  (params (WeaponUI :type Weapon%20UI%20Object%20Reference) (OwningCharacter :type Base%20Character%20BP%20Object%20Reference))
  (|CallParentFunction WeaponUI OwningCharacter)
  (Variables|Default|SetAnimator (.AsRecruit%20Animation%20BP (Utilities|Casting|CastToRecruit_AnimationBP (Components|SkeletalMesh|GetAnimInstance (Variables|/Script/Engine.Character|GetMesh OwningCharacter))))))

(event EventReload
  (bind _currentammo (Variables|Default|GetCurrentAmmo))
  (bind _returnvalue (== _currentammo 0))
  (Utilities|FlowControl|Sequence
    (:then_0
      (Variables|Default|SetReloadTime (Math|Float|SelectFloat (Variables|Default|GetLong%20Reload%20Time) (Variables|Default|GetShort%20Reload%20Time) _returnvalue))
      (Default|DoReload (Variables|Default|GetAnimator) _returnvalue))
    (:then_1
      (|CallParentFunction))))