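; Ashe's ultimate ability, which spawns a Bob_BP actor above the owning character when fired.
; The spawn follows the capsule's yaw, roll and scale, and is refused if colliding, which only prints an error after the parent fire logic.
; On success it stores the Bob reference, empties the charge and UI, then calls Finish after a fixed delay.
; An invalid-Bob check also calls Finish, but runs only once, right after spawning.
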(event EventTick
  (params (DeltaSeconds :type Float%20%28single-precision%29))
  (|CallParentFunction DeltaSeconds))

(event EventFire
  (bind _owningcharacter (Variables|Default|GetOwningCharacter))
  (bind _capsulecomponent (Variables|/Script/Engine.Character|GetCapsuleComponent _owningcharacter))
  (bind _returnvalue (Transformation|GetWorldTransform _capsulecomponent))
  (|CallParentFunction)
  (bind _returnvalue_2 (Game|SpawnActorfromClass "/Game/_Project/Characters/Ashe/Ultimate/Bob_BP.Bob_BP_C" (Math|Transform|MakeTransform (+ (.location _returnvalue) "0.000000,0.000000,200.000000") (Math|Rotator|MakeRotator (.roll (.rotation _returnvalue)) 0.0 (.yaw (.rotation _returnvalue))) (.scale _returnvalue)) "DontSpawnIfColliding" "MultiplyWithRoot" 0 0))
  (Utilities|IsValid _returnvalue_2
    (:Is%20Valid
      (Variables|Default|SetBob%20Reference _returnvalue_2)
      (Utilities|FlowControl|Sequence
        (:then_0
          (bind _output_get (Variables|Default|SetCurrentCharge 0.0))
          (Default|SetUltimateAmount (Variables|Default|GetUltimateUI) _output_get))
        (:then_1
          (Utilities|FlowControl|Delay 6.0)
          (CallFunction|Finish))
        (:then_2
          (Utilities|IsValid (Variables|Default|GetBob%20Reference)
            (:Is%20Not%20Valid
              (CallFunction|Finish))))))
    (:Is%20Not%20Valid
      (Development|PrintString "cant not spawn bob"))))