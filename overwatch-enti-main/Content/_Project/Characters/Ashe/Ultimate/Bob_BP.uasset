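; Bob_BP is Bob, the AI-controlled unit of Ashe's ultimate, which charges into obstacles and knocks characters into the air.
; While its Bob_AI_Controller is running, a roughly head-on hit, filtered by a normal-versus-forward dot product, notifies the controller through OnCollisionBob.
; A hit Character is also launched up and slightly forward, triggering a second notification.
; Separately, Detector overlaps maintain a list of nearby Dummy actors.
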(event OnComponentBeginOverlap(detector)
  (params (OverlappedComponent :type Primitive%20Component%20Object%20Reference) (OtherActor :type Actor%20Object%20Reference) (OtherComp :type Primitive%20Component%20Object%20Reference) (OtherBodyIndex :type Integer) (bFromSweep :type Boolean) (SweepResult :type Hit%20Result%20Structure%20%28by%20ref%29))
  (bind _asdummy (Utilities|Casting|CastToDummy OtherActor))
  (Utilities|Set|Add (Variables|Default|Getdummys) _asdummy))

(event OnComponentEndOverlap(detector)
  (params (OverlappedComponent :type Primitive%20Component%20Object%20Reference) (OtherActor :type Actor%20Object%20Reference) (OtherComp :type Primitive%20Component%20Object%20Reference) (OtherBodyIndex :type Integer))
  (bind _asdummy (Utilities|Casting|CastToDummy OtherActor))
  (Utilities|Set|Remove (Variables|Default|Getdummys) _asdummy))

(event Collision|EventHit
  (params (MyComp :type Primitive%20Component%20Object%20Reference) (Other :type Actor%20Object%20Reference) (OtherComp :type Primitive%20Component%20Object%20Reference) (bSelfMoved :type Boolean) (HitLocation :type Vector :default "0, 0, 0") (HitNormal :type Vector :default "0, 0, 0") (NormalImpulse :type Vector :default "0, 0, 0") (Hit :type Hit%20Result%20Structure%20%28by%20ref%29))
  (if (and (< (Math|Vector|DotProduct HitNormal (Transformation|GetActorForwardVector)) -0.5) (Variables|/Game/_Project/Characters/Ashe/Ultimate/Bob_AI_Controller.Bob_AI_Controller_C|GetIsrunning (.AsBob%20AI%20Controller (Utilities|Casting|CastToBob_AI_Controller (Pawn|GetController)))))
    (Utilities|FlowControl|Sequence
      (:then_0
        (Default|OnCollisionBob (.AsBob%20AI%20Controller (Utilities|Casting|CastToBob_AI_Controller (Pawn|GetController)))))
      (:then_1
        (bind _ascharacter (Utilities|Casting|CastToCharacter Other))
        (Character|LaunchCharacter _ascharacter (+ (* (Math|Vector|GetUpVector (Variables|/Script/Engine.Character|GetCapsuleComponent _ascharacter)) 1e+03) (* (Transformation|GetActorForwardVector self) 2e+02)) true true)
        (Default|OnCollisionBob (.AsBob%20AI%20Controller (Utilities|Casting|CastToBob_AI_Controller (Pawn|GetController))))))))

(fn ConstructionScript)