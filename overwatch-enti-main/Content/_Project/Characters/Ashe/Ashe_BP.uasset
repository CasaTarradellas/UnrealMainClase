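; Ashe is a playable character Blueprint that sets up her health, two skills and an aim-down-sights zoom.
; BeginPlay initializes health, then registers the shotgun jump and dynamite skills with their key labels in the Skills list.
; Skill inputs fire those skills, with dynamite first taking its transform from DynamiteSpawn.
; Secondary fire narrows the camera FOV and swaps the first weapon's reticle, recreating the widget on every Started or Triggered event, and restores both on release.
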(event Input|EnhancedActionEvents|EnhancedInputActionSkill_0
  (params (ActionValue :type Boolean) (ElapsedSeconds :type Float%20%28double-precision%29) (TriggeredSeconds :type Float%20%28double-precision%29) (InputAction :type Input%20Action%20Object%20Reference :default "/Game/_Project/CommonSystems/Input/Skill_0.Skill_0"))
  (Default|Fire (Variables|Default|GetShotgunJumpSkill_Ashe_BP)))

(event Input|EnhancedActionEvents|EnhancedInputActionSkill_1
  (params (ActionValue :type Boolean) (ElapsedSeconds :type Float%20%28double-precision%29) (TriggeredSeconds :type Float%20%28double-precision%29) (InputAction :type Input%20Action%20Object%20Reference :default "/Game/_Project/CommonSystems/Input/Skill_1.Skill_1"))
  (bind _dynamiteskill_ashe_bp (Variables|Default|GetDynamiteSkill_Ashe_BP))
  (Variables|/Game/_Project/Characters/Ashe/Skills/Dynamite/DynamiteSkill_Ashe_BP.DynamiteSkill_Ashe_BP_C|SetLocation _dynamiteskill_ashe_bp (Transformation|GetWorldTransform (Variables|Default|GetDynamiteSpawn)))
  (Default|Fire _dynamiteskill_ashe_bp))

(event Input|EnhancedActionEvents|EnhancedInputActionSecondaryFire
  (params (ActionValue :type Boolean) (ElapsedSeconds :type Float%20%28double-precision%29) (TriggeredSeconds :type Float%20%28double-precision%29) (InputAction :type Input%20Action%20Object%20Reference :default "/Game/_Project/CommonSystems/Input/SecondaryFire.SecondaryFire"))
  (bind _camera (Variables|Default|GetCamera))
  (bind _weapons (Variables|Default|GetWeapons))
  (bind _output (Utilities|Array|Get(acopy) _weapons))
  (:Triggered
    (Camera|SetFieldOfView _camera 6e+01 :!label _label)
    (Widget|RemovefromParent (Variables|/Game/_Project/CommonSystems/Weapon/BaseWeapon.BaseWeapon_C|GetReticle _output))
    (bind _returnvalue (UserInterface|CreateWidget "/Game/Reticles/Widgets/WBP_Reticle_TypeF_2_v05.WBP_Reticle_TypeF_2_v05_C"))
    (bind _output_get (Variables|/Game/_Project/CommonSystems/Weapon/BaseWeapon.BaseWeapon_C|SetReticle _output _returnvalue))
    (UserInterface|Viewport|AddtoViewport _output_get 0))
  (:Started
    (goto _label))
  (:Canceled
    (Camera|SetFieldOfView _camera 9e+01 :!label _label_2)
    (Widget|RemovefromParent (Variables|/Game/_Project/CommonSystems/Weapon/BaseWeapon.BaseWeapon_C|GetReticle _output))
    (bind _returnvalue_2 (UserInterface|CreateWidget "/Game/Reticles/Widgets/WBP_Reticle_TypeE_4_v04.WBP_Reticle_TypeE_4_v04_C"))
    (bind _output_get_2 (Variables|/Game/_Project/CommonSystems/Weapon/BaseWeapon.BaseWeapon_C|SetReticle (Utilities|Array|Get(acopy) (Variables|Default|GetWeapons)) _returnvalue_2))
    (UserInterface|Viewport|AddtoViewport _output_get_2 0))
  (:Completed
    (goto _label_2)))

(event EventBeginPlay
  (bind _shotgunjumpskill_ashe_bp (Variables|Default|GetShotgunJumpSkill_Ashe_BP))
  (bind _dynamiteskill_ashe_bp (Variables|Default|GetDynamiteSkill_Ashe_BP))
  (|CallParentFunction)
  (Utilities|FlowControl|Sequence
    (:then_0
      (CallFunction|InitializeHealth (Utilities|Struct|MakeHealthData 2.5e+02 2.5e+02 0.0 0.0 0.0 0.0 0.0 false)))
    (:then_1
      (Default|Initialize _shotgunjumpskill_ashe_bp self "L SHIFT")
      (Utilities|Array|Add (Variables|Default|GetSkills) _shotgunjumpskill_ashe_bp))
    (:then_2
      (Default|Initialize _dynamiteskill_ashe_bp self "E")
      (Utilities|Array|Add (Variables|Default|GetSkills) _dynamiteskill_ashe_bp))))

(fn ConstructionScript
  (|CallParentFunction))