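; Ashe's shotgun jump skill, which fires a spread blast and launches the character.
; In the required skill state, Fire runs random cone line traces from the camera, damaging HealthSystem components with distance falloff (floored at 20%) and flagging Head-bone headshots.
; Physics-simulating hit components receive an impulse at the impact point.
; It then launches Ashe along camera forward scaled by Recoil, plus fixed upward velocity, and calls Finish.
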(event EventFire
  (bind _owningcharacter (Variables|Default|GetOwningCharacter))
  (bind _owningcharacter_2 (Variables|Default|GetOwningCharacter))
  (bind _maxspread (Variables|Default|GetMaxSpread))
  (bind _fire_distance (Variables|Default|GetFire%20Distance))
  (bind _asashe_bp (Utilities|Casting|CastToAshe_BP _owningcharacter_2))
  (bind _camera (Variables|/Game/_Project/Characters/BaseCharacter_BP.BaseCharacter_BP_C|GetCamera _asashe_bp))
  (bind _returnvalue (Transformation|GetWorldLocation _camera))
  (bind _returnvalue_2 (Math|Vector|GetForwardVector _camera))
  (bind _returnvalue_3 (Math|Random|RandomUnitVectorinConeinDegrees _returnvalue_2 _maxspread))
  (bind _returnvalue_4 (* _returnvalue_3 _fire_distance))
  (bind _returnvalue_5 (+ _returnvalue _returnvalue_4))
  (|CallParentFunction)
  (if (Utilities|Enum|Equal(Enum) (Variables|Default|GetState) "NewEnumerator1")
    (Utilities|FlowControl|Sequence
      (:then_0
        (for _index (range 0 (Variables|Default|GetTotalBullets))
          (bind (_outhit _returnvalue_6) (Collision|LineTraceByChannel _returnvalue _returnvalue_5 "TraceTypeQuery1" false 0 "ForDuration"))
          (if _returnvalue_6
            (Utilities|FlowControl|Sequence
              (:then_0
                (Utilities|IsValid (Actor|GetComponentbyClass (.HitActor (Collision|BreakHitResult _outhit)) "/Game/_Project/CommonSystems/HealthSystem/HealthSystem.HealthSystem_C")
                  (:Is%20Valid
                    (Default|TakeDamage (Actor|GetComponentbyClass (.HitActor (Collision|BreakHitResult _outhit)) "/Game/_Project/CommonSystems/HealthSystem/HealthSystem.HealthSystem_C") (== (.HitBoneName (Collision|BreakHitResult _outhit)) "Head") (* (Variables|Default|GetDamage) (Math|Float|Max(Float) (- 1.0 (/ (.Distance (Collision|BreakHitResult _outhit)) (Variables|Default|GetFire%20Distance))) 0.2))))))
              (:then_1
                (if (Physics|IsSimulatingPhysics (.HitComponent (Collision|BreakHitResult _outhit)) "None")
                  (Physics|AddImpulseatLocation (.HitComponent (Collision|BreakHitResult _outhit)) _returnvalue_5 (.ImpactPoint (Collision|BreakHitResult _outhit)) "None")))))))
      (:then_1
        (Character|LaunchCharacter _owningcharacter (+ (* (Math|Vector|GetForwardVector (Variables|/Game/_Project/Characters/BaseCharacter_BP.BaseCharacter_BP_C|GetCamera _owningcharacter)) (Variables|Default|GetRecoil)) "0.000000,0.000000,350.000000") false false))
      (:then_2
        (CallFunction|Finish)))))