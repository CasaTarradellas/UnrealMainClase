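; Cassidy's Deadeye-style ultimate, which slows the owner for a timed window while locks build on targeted enemies.
; Tick gathers visible Dummy actors via camera box and line traces outside the state Fire requires.
; Update grows each lock time up to a cap while active.
; Shooting instakills fully locked targets, damages others by lock time, then finishes; timeout finishes without damage, and disconnected backup logic remains.
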(event Custom|Ev_UltimateTimeout
  (if (Variables|Default|GetHasShoot?)
    (Development|PrintString "Ha disparado")
    (else
      (Development|PrintString "Daño miseria")
      (CallFunction|FinishUltimateCassidy))))

(event Custom|FinishUltimateCassidy
  (Variables|Default|SetCurrentCharge 0.0)
  (Variables|/Script/Engine.CharacterMovementComponent|SetMaxWalkSpeed (Variables|/Script/Engine.Character|GetCharacterMovement (Variables|Default|GetOwningCharacter)) (Variables|Default|GetMax%20Walk%20Speed))
  (CallFunction|Finish)
  (Default|SetUltimateAmount (Variables|Default|GetUltimateUI) (Variables|Default|GetCurrentCharge))
  (Variables|Default|SetIsUltimateActive? false))

(event Input|EnhancedActionEvents|EnhancedInputActionIA_UltimateShoot
  (params (ActionValue :type Boolean) (ElapsedSeconds :type Float%20%28double-precision%29) (TriggeredSeconds :type Float%20%28double-precision%29) (InputAction :type Input%20Action%20Object%20Reference :default "/Game/_Project/Characters/Cassidy/Ultimate/IA_UltimateShoot.IA_UltimateShoot"))
  (:Started
    (if (Variables|Default|GetIsUltimateActive?)
      (Utilities|Time|ClearandInvalidateTimerbyHandle (Variables|Default|GetUltimateTimerHandle))
      (for _array_element (Variables|Default|GetTargetedEnemies)
        (if (>= (.LockOnTime (Utilities|Struct|BreakS_DeadEyeTarget _array_element)) 3.0)
          (Game|Damage|ApplyDamage (.EnemyActor (Utilities|Struct|BreakS_DeadEyeTarget _array_element)) (Variables|Default|GetInstaKill) 0 0)
          (Development|PrintString "llegóa los 3 segundos")
          (else
            (bind _output_get (Variables|Default|SetMissShootDamage (.LockOnTime (Utilities|Struct|BreakS_DeadEyeTarget _array_element))))
            (Game|Damage|ApplyDamage (.EnemyActor (Utilities|Struct|BreakS_DeadEyeTarget _array_element)) (* _output_get 5e+01) 0 0)
            (Development|PrintString "no llegó a los 3 segundos"))))
      (CallFunction|FinishUltimateCassidy))))

(event Input|EnhancedActionEvents|EnhancedInputActionIA_UltimateShoot
  (params (ActionValue :type Boolean) (ElapsedSeconds :type Float%20%28double-precision%29) (TriggeredSeconds :type Float%20%28double-precision%29) (InputAction :type Input%20Action%20Object%20Reference :default "/Game/_Project/Characters/Cassidy/Ultimate/IA_UltimateShoot.IA_UltimateShoot")))

(event EventUpdate
  (params (DeltaTime :type Float%20%28double-precision%29))
  (if (Variables|Default|GetIsUltimateActive?)
    (for (_array_element _array_index) (Variables|Default|GetTargetedEnemies)
      (Development|PrintString (Utilities|String|ToString(Float) (Math|Float|Clamp(Float) (+ (.LockOnTime (Utilities|Struct|BreakS_DeadEyeTarget _array_element)) DeltaTime) 0.0 3.0)) true true "(R=0.000000,G=0.660000,B=1.000000,A=1.000000)" (Math|Float|Clamp(Float) (+ (.LockOnTime (Utilities|Struct|BreakS_DeadEyeTarget _array_element)) DeltaTime) 0.0 3.0))
      (Utilities|Array|SetArrayElem (Variables|Default|GetTargetedEnemies) _array_index (Utilities|Struct|MakeS_DeadEyeTarget (.EnemyActor (Utilities|Struct|BreakS_DeadEyeTarget _array_element)) (Math|Float|Clamp(Float) (+ (.LockOnTime (Utilities|Struct|BreakS_DeadEyeTarget _array_element)) DeltaTime) 0.0 3.0))))))

(event EventFinish
  (|CallParentFunction))

(event EventFire
  (|CallParentFunction)
  (if (Utilities|Enum|Equal(Enum) (Variables|Default|GetState) "NewEnumerator2")
    (Variables|Default|SetIsUltimateActive? true)
    (Variables|/Script/Engine.CharacterMovementComponent|SetMaxWalkSpeed (Variables|/Script/Engine.Character|GetCharacterMovement (Variables|Default|GetOwningCharacter)) (Variables|Default|GetReduced%20Walk%20Speed))
    (bind _returnvalue (Utilities|Time|SetTimerbyEvent (delegate Custom|Ev_UltimateTimeout) (Variables|Default|GetUltimateDuration)))
    (Variables|Default|SetUltimateTimerHandle _returnvalue)))

(event EventTick
  (params (DeltaSeconds :type Float%20%28single-precision%29))
  (bind _owningcharacter (Variables|Default|GetOwningCharacter))
  (bind _camera (Variables|/Game/_Project/Characters/BaseCharacter_BP.BaseCharacter_BP_C|GetCamera _owningcharacter))
  (if (not (Utilities|Enum|Equal(Enum) (Variables|Default|GetState) "NewEnumerator2"))
    (bind _outhits (Class|KismetSystemLibrary|BoxTraceMulti (Transformation|GetWorldLocation _camera) (* (Math|Vector|GetForwardVector _camera) (Variables|Default|GetMaxDistance)) "0.000000,0.000000,0.000000" "0, 0, 0" "TraceTypeQuery1" false 0 "ForOneFrame" true))
    (for _array_element _outhits
      (bind _outhit (Collision|LineTraceByChannel (Transformation|GetWorldLocation (Variables|/Game/_Project/Characters/BaseCharacter_BP.BaseCharacter_BP_C|GetCamera (Variables|Default|GetOwningCharacter))) (Transformation|GetActorLocation (.HitActor (Collision|BreakHitResult _array_element))) "TraceTypeQuery1" false 0 "ForOneFrame"))
      (Utilities|FlowControl|Sequence
        (:then_0
          (Utilities|Array|Clear (Variables|Default|GetDetectedActors)))
        (:then_1
          (bind _asdummy (Utilities|Casting|CastToDummy (.HitActor (Collision|BreakHitResult _outhit))))
          (if (not (Utilities|Array|ContainsItem (Variables|Default|GetActoresFijados) _asdummy))
            (Utilities|Array|Add (Variables|Default|GetTargetedEnemies) (Utilities|Struct|MakeS_DeadEyeTarget _asdummy 0.0))
            (Utilities|Array|Add (Variables|Default|GetActoresFijados) _asdummy)))))))