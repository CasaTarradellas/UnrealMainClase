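; Projectile for Bastion's Configuration Assault skill that destroys itself on hit and explodes.
; On destruction it fires a radial force impulse, then overlaps pawns within the same radius and spawns a scaled-up explosion emitter.
; Overlapped pawns with a HealthSystem component receive a TakeDamage call, though the amount shown is zero.
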(event OnComponentHit(Sphere)
  (params (HitComponent :type Primitive%20Component%20Object%20Reference) (OtherActor :type Actor%20Object%20Reference) (OtherComp :type Primitive%20Component%20Object%20Reference) (NormalImpulse :type Vector :default "0, 0, 0") (Hit :type Hit%20Result%20Structure%20%28by%20ref%29))
  (Actor|DestroyActor))

(event EventDestroyed
  (Utilities|FlowControl|Sequence
    (:then_0
      (Class|RadialForceComponent|FireImpulse (Variables|Default|GetRadialForce)))
    (:then_1
      (bind (_outactors _returnvalue) (Collision|SphereOverlapActors (Transformation|GetActorLocation) (Variables|/Script/Engine.RadialForceComponent|GetRadius (Variables|Default|GetRadialForce)) (Utilities|Array|MakeArray "ObjectTypeQuery3") 0))
      (if _returnvalue
        (for _array_element _outactors
          (Utilities|IsValid (Actor|GetComponentbyClass _array_element "/Game/_Project/CommonSystems/HealthSystem/HealthSystem.HealthSystem_C")
            (:Is%20Valid
              (Default|TakeDamage (Actor|GetComponentbyClass _array_element "/Game/_Project/CommonSystems/HealthSystem/HealthSystem.HealthSystem_C") false 0.0)
              (Utilities|IsValid 0))))))
    (:then_2
      (Effects|SpawnEmitteratLocation "/Game/StarterContent/Particles/P_Explosion.P_Explosion" (Transformation|GetActorLocation) "0, 0, 0" "5.000000,5.000000,5.000000"))))

(fn ConstructionScript)