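; Bastion skill Blueprint for Configuration Assault, which switches the Bastion character to its assault weapon.
; On Fire it runs the parent logic, then, if the skill is in a specific state, calls ChangeAssaultWeapon on the owning BastionBP.
; It also adds charge to the owner's Ultimate and then finishes the skill.
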(event EventFire
  (|CallParentFunction)
  (if (Utilities|Enum|Equal(Enum) (Variables|Default|GetState) "NewEnumerator1")
    (Default|ChangeAssaultWeapon (.AsBastion%20BP (Utilities|Casting|CastToBastionBP (Variables|Default|GetOwningCharacter))))
    (Default|AddCharge (Variables|/Game/_Project/Characters/BaseCharacter_BP.BaseCharacter_BP_C|GetUltimate (Variables|Default|GetOwningCharacter)) 1e+02)
    (CallFunction|Finish)))