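; Bastion playable hero character that sets up health and wires input to its grenade, assault configuration and ultimate abilities.
; Grenade and assault skills register in the Skills list at BeginPlay, and grenades launch from a spawn point component.
; Weapon-change events store the current weapon, then timelines roll both meshes and use an event track to swap visibility between regular and ultimate meshes and draw the new weapon.
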(event Custom|ChangeAssaultWeapon
  (Default|Store (Utilities|Array|Get(acopy) (Variables|Default|GetWeapons)))
  (bind _rotationx (Timeline|Timeline_1 PlayFromStart)
    (:Update
      (Transformation|SetRelativeRotation (Variables|Character|GetMesh) (Math|Rotator|MakeRotator _rotationx 0.0 -9e+01) false false)
      (Transformation|SetRelativeRotation (Variables|Default|GetUltimateMesh) (Math|Rotator|MakeRotator (+ -1.1 _rotationx) -1e+01 -9e+01) false false))
    (:ChangeWeapons
      (Rendering|SetVisibility (Variables|Character|GetMesh) false false)
      (Rendering|SetVisibility (Variables|Default|GetUltimateMesh) true false)
      (CallFunction|ChangeWeapon 1)
      (Default|Draw (Utilities|Array|Get(acopy) (Variables|Default|GetWeapons) 1)))))

(event Custom|ChangeToRegularWeapon
  (Default|Store (Utilities|Array|Get(acopy) (Variables|Default|GetWeapons) 2))
  (bind _rotationx (Timeline|Timeline_0 PlayFromStart)
    (:Update
      (Transformation|SetRelativeRotation (Variables|Character|GetMesh) (Math|Rotator|MakeRotator _rotationx 0.0 -9e+01) false false)
      (Transformation|SetRelativeRotation (Variables|Default|GetUltimateMesh) (Math|Rotator|MakeRotator (+ -1.1 _rotationx) -1e+01 -9e+01) false false))
    (:ChangeWeapons
      (Rendering|SetVisibility (Variables|Character|GetMesh) true false)
      (Rendering|SetVisibility (Variables|Default|GetUltimateMesh) false false)
      (CallFunction|ChangeWeapon)
      (Default|Draw (Utilities|Array|Get(acopy) (Variables|Default|GetWeapons))))))

(event Custom|ChangeToUltimateWeapon
  (Default|Store (Utilities|Array|Get(acopy) (Variables|Default|GetWeapons)))
  (bind _rotationx (Timeline|Timeline PlayFromStart)
    (:Update
      (Transformation|SetRelativeRotation (Variables|Character|GetMesh) (Math|Rotator|MakeRotator _rotationx 0.0 -9e+01) false false)
      (Transformation|SetRelativeRotation (Variables|Default|GetUltimateMesh) (Math|Rotator|MakeRotator (+ -1.1 _rotationx) -1e+01 -9e+01) false false))
    (:ChangeWeapons
      (Rendering|SetVisibility (Variables|Character|GetMesh) false false)
      (Rendering|SetVisibility (Variables|Default|GetUltimateMesh) true false)
      (CallFunction|ChangeWeapon 1)
      (Default|Draw (Utilities|Array|Get(acopy) (Variables|Default|GetWeapons) 2)))))

(event Input|EnhancedActionEvents|EnhancedInputActionSkill_1
  (params (ActionValue :type Boolean) (ElapsedSeconds :type Float%20%28double-precision%29) (TriggeredSeconds :type Float%20%28double-precision%29) (InputAction :type Input%20Action%20Object%20Reference :default "/Game/_Project/CommonSystems/Input/Skill_1.Skill_1"))
  (bind _bastion_grenade_skill_bpc (Variables|Default|GetBastion_Grenade_Skill_BPC))
  (Variables|/Game/_Project/Characters/Bastion/Skills/TacticalGrenade/Bastion_Grenade_Skill_BPC.Bastion_Grenade_Skill_BPC_C|SetSpawnPoint _bastion_grenade_skill_bpc (Transformation|GetWorldTransform (Variables|Default|GetGrenadeSpawnPoint)))
  (Default|Fire _bastion_grenade_skill_bpc))

(event Input|EnhancedActionEvents|EnhancedInputActionUltimate
  (params (ActionValue :type Boolean) (ElapsedSeconds :type Float%20%28double-precision%29) (TriggeredSeconds :type Float%20%28double-precision%29) (InputAction :type Input%20Action%20Object%20Reference :default "/Game/_Project/CommonSystems/Input/Ultimate.Ultimate"))
  (:Triggered
    (Default|Fire (Variables|Default|GetBastion_Ultimate_BP) :!label _label))
  (:Started
    (goto _label)))

(event Input|EnhancedActionEvents|EnhancedInputActionSkill_0
  (params (ActionValue :type Boolean) (ElapsedSeconds :type Float%20%28double-precision%29) (TriggeredSeconds :type Float%20%28double-precision%29) (InputAction :type Input%20Action%20Object%20Reference :default "/Game/_Project/CommonSystems/Input/Skill_0.Skill_0"))
  (Default|Fire (Variables|Default|GetBastion_ConfigurationAssaultBP)))

(event EventBeginPlay
  (bind _bastion_grenade_skill_bpc (Variables|Default|GetBastion_Grenade_Skill_BPC))
  (bind _bastion_configurationassaultbp (Variables|Default|GetBastion_ConfigurationAssaultBP))
  (|CallParentFunction)
  (Utilities|FlowControl|Sequence
    (:then_0
      (CallFunction|InitializeHealth (Utilities|Struct|MakeHealthData 225.0 225.0 0.0 0.0 0.0 0.0 0.0 false)))
    (:then_1
      (Default|Initialize _bastion_grenade_skill_bpc self "E")
      (Utilities|Array|Add (Variables|Default|GetSkills) _bastion_grenade_skill_bpc))
    (:then_2
      (Default|Initialize _bastion_configurationassaultbp self "RIGHT SHIFT")
      (Utilities|Array|Add (Variables|Default|GetSkills) _bastion_configurationassaultbp))))

(fn ConstructionScript)