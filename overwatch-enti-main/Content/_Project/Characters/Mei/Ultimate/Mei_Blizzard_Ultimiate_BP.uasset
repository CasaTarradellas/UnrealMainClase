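; Mei's Blizzard ultimate actor, which freezes and damages pawns around it, excluding its owning character.
; After its sphere hits something, Tick raises it to TargetZ, then runs a one-time debug-drawn sphere overlap that disables input on those found.
; A looping timer at InitialLifeSpan intervals damages the loop's current element through its HealthSystem.
; On destruction it restores input to frozen characters and finishes the owner's Ultimate.
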(event OnComponentHit(Sphere)
  (params (HitComponent :type Primitive%20Component%20Object%20Reference) (OtherActor :type Actor%20Object%20Reference) (OtherComp :type Primitive%20Component%20Object%20Reference) (NormalImpulse :type Vector :default "0, 0, 0") (Hit :type Hit%20Result%20Structure%20%28by%20ref%29))
  (Variables|Default|SetHit? true))

(event Custom|Freeze
  (bind _returnvalue (Transformation|GetActorLocation))
  ;[0.15 0.15 0.15 0.5] Makes damage and freezes chracters inside sphere
  (Rendering|Debug|DrawDebugSphere _returnvalue 5e+02 12 "(R=0.020754,G=0.988063,B=1.000000,A=1.000000)" 5.35 1.0)
  (bind (_outactors _returnvalue_2) (Collision|SphereOverlapActors _returnvalue 5e+02 (Utilities|Array|MakeArray "ObjectTypeQuery3") 0 (Utilities|Array|MakeArray (Variables|Default|GetOwningCharacter))))
  (if _returnvalue_2
    (for _array_element _outactors
      (Utilities|IsValid _array_element
        (:Is%20Valid
          (Development|PrintString "Detected someone, Freezing")
          (Utilities|FlowControl|Sequence
            (:then_0
              (Utilities|Array|Add (Variables|Default|GetFrozenCharacters) _array_element)
              (Input|DisableInput _array_element (.AsPlayer%20Controller (Utilities|Casting|CastToPlayerController (Pawn|GetController (.AsCharacter (Utilities|Casting|CastToCharacter _array_element)))))))
            (:then_1
              (Utilities|Time|SetTimerbyEvent (delegate Custom|DealDamage) (Variables|Actor|GetInitialLifeSpan) true))))))))

(event Custom|DealDamage
  (Default|TakeDamage (Actor|GetComponentbyClass (stale Custom|Freeze _array_element) "/Game/_Project/CommonSystems/HealthSystem/HealthSystem.HealthSystem_C") false 1e+01))

(event EventDestroyed
  (Utilities|FlowControl|Sequence
    (:then_0
      (for _array_element (Variables|Default|GetFrozenCharacters)
        (Utilities|IsValid _array_element
          (:Is%20Valid
            (Input|EnableInput _array_element (.AsPlayer%20Controller (Utilities|Casting|CastToPlayerController (Pawn|GetController (.AsCharacter (Utilities|Casting|CastToCharacter _array_element))))))))))
    (:then_1
      (Default|Finish (Variables|/Game/_Project/Characters/BaseCharacter_BP.BaseCharacter_BP_C|GetUltimate (Variables|Default|GetOwningCharacter))))))

(event EventTick
  (params (DeltaSeconds :type Float%20%28single-precision%29))
  (bind _returnvalue (Transformation|GetActorLocation))
  (if (Variables|Default|GetHit?)
    (if (>= (.z (Transformation|GetActorLocation)) (Variables|Default|GetTargetZ))
      (Utilities|FlowControl|DoOnce false
        (:Completed
          (CallFunction|Freeze)))
      (else
        ;[0.15 0.15 0.15 0.5] Going up
        (Transformation|SetActorLocation (Math|Vector|MakeVector (.x _returnvalue) (.y _returnvalue) (+ (.z _returnvalue) (* DeltaSeconds 2.5e+02))) false false)))))

(fn ConstructionScript)