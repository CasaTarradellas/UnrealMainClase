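; Mei's Cryo-Freeze skill actor, which makes its owning character immobile and invulnerable while it heals them.
; Initialize zeroes walk speed and jump velocity; Destroy restores hard-coded defaults, removes the actor and lifts invulnerability.
; Tick checks a Destroy flag, adds frame-rate-dependent health and ultimate charge while health is below maximum, and follows the owner's location and yaw.
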(event Custom|Destroy
  (bind _owningcharacter (Variables|Default|GetOwningCharacter))
  (bind _charactermovement (Variables|/Script/Engine.Character|GetCharacterMovement _owningcharacter))
  (Variables|/Script/Engine.CharacterMovementComponent|SetMaxWalkSpeed _charactermovement 6e+02)
  (Variables|/Script/Engine.CharacterMovementComponent|SetJumpZVelocity _charactermovement 4.2e+02)
  (Actor|DestroyActor)
  (Default|SetInvulnerable (Variables|/Game/_Project/Characters/BaseCharacter_BP.BaseCharacter_BP_C|GetHealthSystem (Variables|Default|GetOwningCharacter)) false))

(event Custom|Initialize
  (bind _owningcharacter (Variables|Default|GetOwningCharacter))
  (bind _charactermovement (Variables|/Script/Engine.Character|GetCharacterMovement _owningcharacter))
  (Variables|/Script/Engine.CharacterMovementComponent|SetMaxWalkSpeed _charactermovement 0.0)
  (Variables|/Script/Engine.CharacterMovementComponent|SetJumpZVelocity _charactermovement 0.0)
  ;[0.15 0.15 0.15 0.5] Fix invulnerability
  (Default|SetInvulnerable (Variables|/Game/_Project/Characters/BaseCharacter_BP.BaseCharacter_BP_C|GetHealthSystem (Variables|Default|GetOwningCharacter)) true))

(event EventDestroyed
  (CallFunction|Destroy))

(event EventTick
  (params (DeltaSeconds :type Float%20%28single-precision%29))
  (bind _owningcharacter (Variables|Default|GetOwningCharacter))
  (bind _owningcharacter_2 (Variables|Default|GetOwningCharacter))
  (bind _owningcharacter_3 (Variables|Default|GetOwningCharacter))
  (bind _healthsystem (Variables|/Game/_Project/Characters/BaseCharacter_BP.BaseCharacter_BP_C|GetHealthSystem _owningcharacter_2))
  (bind _healthdata (Default|GetHealthData _healthsystem))
  (Utilities|FlowControl|Sequence
    (:then_0
      (if (Variables|Default|GetDestroy?)
        (CallFunction|Destroy)))
    (:then_1
      ;[0.15 0.15 0.15 0.5] Set timer by event??
      (if (< (.currenthealth _healthdata) (.maxhealth _healthdata))
        (Default|AddHealthType (Variables|/Game/_Project/Characters/BaseCharacter_BP.BaseCharacter_BP_C|GetHealthSystem _owningcharacter_3) "NewEnumerator0" 0.5)
        (Default|AddCharge (Variables|/Game/_Project/Characters/BaseCharacter_BP.BaseCharacter_BP_C|GetUltimate _owningcharacter_3) 0.15)))
    (:then_2
      ;[0.15 0.15 0.15 0.5] Simulate physics -> follows player location and locks rotation on X and Y
      (Transformation|SetActorLocation (Transformation|GetActorLocation _owningcharacter) false false)
      (Transformation|SetActorRotation (Math|Rotator|MakeRotator 0.0 0.0 (.yaw (Transformation|GetActorRotation _owningcharacter)))))))

(fn ConstructionScript)