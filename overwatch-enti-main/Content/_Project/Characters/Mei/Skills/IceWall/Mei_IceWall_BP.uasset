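; Mei's ice wall skill Blueprint, a wall of five cube segments that break individually under repeated hits.
; ReceiveDamage takes the hit component and runs CheckHits against each cube in sequence.
; The matching segment's counter in HitsArray goes up by one, and that cube component is destroyed once the count reaches MaxHits.
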(event Custom|ReceiveDamage
  (params (IceWall :type Static%20Mesh%20Component%20Object%20Reference))
  (Utilities|FlowControl|Sequence
    (:then_0
      (CallFunction|CheckHits 0 IceWall (Variables|Default|GetCube1)))
    (:then_1
      (CallFunction|CheckHits 1 IceWall (Variables|Default|GetCube2)))
    (:then_2
      (CallFunction|CheckHits 2 IceWall (Variables|Default|GetCube3)))
    (:then_3
      (CallFunction|CheckHits 3 IceWall (Variables|Default|GetCube4)))
    (:then_4
      (CallFunction|CheckHits 4 IceWall (Variables|Default|GetCube5)))))

(event Custom|CheckHits
  (params (Index :type Integer) (HitComponent :type Static%20Mesh%20Component%20Object%20Reference) (IceWall :type Static%20Mesh%20Component%20Object%20Reference))
  (if (== HitComponent IceWall)
    (bind _output_get (Variables|Default|SetHitsArray (Variables|Default|GetHitsArray)))
    (Utilities|Array|SetArrayElem _output_get Index (+ (Utilities|Array|Get(acopy) (Variables|Default|GetHitsArray) Index) 1))
    (if (>= (+ (Utilities|Array|Get(acopy) (Variables|Default|GetHitsArray) Index) 1) (Variables|Default|GetMaxHits))
      (Components|DestroyComponent IceWall))))

(fn ConstructionScript)