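; Mei hero character Blueprint for an Overwatch-style game, built on a parent character class with health, skills and an ultimate.
; BeginPlay initializes health and registers the Cryo Freeze and Ice Wall skill components.
; Input fires each skill and disables the other, while the Blizzard ultimate and Cryo Freeze receive spawn points before firing.
; Tick polls health and calls Die, which disables input, hides the mesh and requests a respawn from the GameMode.
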(event Custom|Die
  (bind _returnvalue (Pawn|GetController))
  (Input|DisableInput (.AsPlayer%20Controller (Utilities|Casting|CastToPlayerController _returnvalue)))
  (Components|Movement|StopMovementImmediately (Variables|Character|GetCharacterMovement))
  (Rendering|SetVisibility (Variables|Character|GetMesh) false false)
  (Default|RespawnPlayer (.AsOverwatch%20Game%20Mode (Utilities|Casting|CastToOverwatchGameMode (Game|GetGameMode))) self _returnvalue (Variables|Default|GetUI)))

(event Input|EnhancedActionEvents|EnhancedInputActionSkill_0
  (params (ActionValue :type Boolean) (ElapsedSeconds :type Float%20%28double-precision%29) (TriggeredSeconds :type Float%20%28double-precision%29) (InputAction :type Input%20Action%20Object%20Reference :default "/Game/_Project/CommonSystems/Input/Skill_0.Skill_0"))
  (:Started
    (Utilities|FlowControl|Sequence
      (:then_0
        (Variables|/Game/_Project/Characters/Mei/Skills/CryoFreeze/Mei_CryoFreeze_Skill_BPC.Mei_CryoFreeze_Skill_BPC_C|SetSpawnPoint (Variables|Default|GetMei_CryoFreeze_Skill_BPC) (Transformation|GetWorldTransform (Variables|Default|GetCryoFreezeSpawnPoint))))
      (:then_1
        (Default|Fire (Variables|Default|GetMei_CryoFreeze_Skill_BPC))
        (Default|SetEnabled (Variables|Default|GetMei_IceWall_Skill_BPC) false)))))

(event Input|EnhancedActionEvents|EnhancedInputActionSkill_1
  (params (ActionValue :type Boolean) (ElapsedSeconds :type Float%20%28double-precision%29) (TriggeredSeconds :type Float%20%28double-precision%29) (InputAction :type Input%20Action%20Object%20Reference :default "/Game/_Project/CommonSystems/Input/Skill_1.Skill_1"))
  (:Started
    (Default|Fire (Variables|Default|GetMei_IceWall_Skill_BPC))
    (Default|SetEnabled (Variables|Default|GetMei_CryoFreeze_Skill_BPC) false)))

(event Input|EnhancedActionEvents|EnhancedInputActionUltimate
  (params (ActionValue :type Boolean) (ElapsedSeconds :type Float%20%28double-precision%29) (TriggeredSeconds :type Float%20%28double-precision%29) (InputAction :type Input%20Action%20Object%20Reference :default "/Game/_Project/CommonSystems/Input/Ultimate.Ultimate"))
  (bind _ultimate (Variables|Default|GetUltimate))
  (:Started
    (Variables|/Game/_Project/Characters/Mei/Ultimate/Mei_Blizzard_Ultimate_BPC.Mei_Blizzard_Ultimate_BPC_C|SetSpawnLocation (.AsMei%20Blizzard%20Ultimate%20BPC (Utilities|Casting|CastToMei_Blizzard_Ultimate_BPC _ultimate)) (Transformation|GetWorldLocation (Variables|Default|GetBlizzardSpawnPoint)))
    (Default|Fire _ultimate)))

(event EventTick
  (params (DeltaSeconds :type Float%20%28single-precision%29))
  (|CallParentFunction DeltaSeconds)
  (if (<= (.currenthealth (Default|GetHealthData (Variables|Default|GetHealthSystem))) 0.0)
    (CallFunction|Die)))

(event EventBeginPlay
  (bind _self self)
  (bind _mei_cryofreeze_skill_bpc (Variables|Default|GetMei_CryoFreeze_Skill_BPC))
  (bind _mei_icewall_skill_bpc (Variables|Default|GetMei_IceWall_Skill_BPC))
  (|CallParentFunction)
  (Utilities|FlowControl|Sequence
    (:then_0
      (Default|Initialize (Variables|Default|GetHealthSystem) (Utilities|Struct|MakeHealthData 3e+02 3e+02 0.0 0.0 0.0 0.0 0.0 false)))
    (:then_1
      (Default|Initialize _mei_cryofreeze_skill_bpc _self "L SHIFT")
      (Utilities|Array|Add (Variables|Default|GetSkills) _mei_cryofreeze_skill_bpc))
    (:then_2
      (Default|Initialize _mei_icewall_skill_bpc _self "E")
      (Utilities|Array|Add (Variables|Default|GetSkills) _mei_icewall_skill_bpc))))

(fn ConstructionScript
  (|CallParentFunction))