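; Mei's icicle projectile, which damages what it strikes through its Sphere collision hit event.
; Targets with a HealthSystem component take damage, flagged as a headshot when the hit bone is Head.
; Headshots also charge the owning character's Ultimate, and the icicle destroys itself after damaging, except on headshots without a valid owner.
; Otherwise, Mei's ice wall receives the struck mesh component as damage, without destroying the icicle.
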(event OnComponentHit(Sphere)
  (params (HitComponent :type Primitive%20Component%20Object%20Reference) (OtherActor :type Actor%20Object%20Reference) (OtherComp :type Primitive%20Component%20Object%20Reference) (NormalImpulse :type Vector :default "0, 0, 0") (Hit :type Hit%20Result%20Structure%20%28by%20ref%29))
  (bind (_bblockinghit _binitialoverlap _time _distance _location _impactpoint _normal _impactnormal _physmat _hitactor _hitcomponent _hitbonename) (Collision|BreakHitResult Hit))
  (bind _owningcharacter (Variables|Default|GetOwningCharacter))
  (bind _returnvalue (Actor|GetComponentbyClass _hitactor "/Game/_Project/CommonSystems/HealthSystem/HealthSystem.HealthSystem_C"))
  (bind _asmei_ice_wall_bp (Utilities|Casting|CastToMei_IceWall_BP _hitactor))
  (bind _returnvalue_2 (== _hitbonename "Head"))
  ;[0.15 0.15 0.15 0.5] Fix headshot checking
  (Utilities|IsValid _returnvalue
    (:Is%20Valid
      (Default|TakeDamage _returnvalue _returnvalue_2 (Variables|Default|GetDamage))
      (if _returnvalue_2
        (Utilities|IsValid _owningcharacter
          (:Is%20Valid
            (Default|AddCharge (Variables|/Game/_Project/Characters/BaseCharacter_BP.BaseCharacter_BP_C|GetUltimate _owningcharacter) 2.5))))
      (Actor|DestroyActor))
    (:Is%20Not%20Valid
      (Utilities|IsValid _asmei_ice_wall_bp
        (:Is%20Valid
          (Default|ReceiveDamage _asmei_ice_wall_bp (.AsStatic%20Mesh%20Component (Utilities|Casting|CastToStaticMeshComponent _hitcomponent))))))))

(fn ConstructionScript)