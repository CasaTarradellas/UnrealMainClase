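; Pharah's ultimate ability, which fires a barrage of bullets for 2.5 seconds once Fire passes its state check, then calls Finish.
; While active, Tick feeds slight upward movement input to the owning character.
; A Delay inside Tick throttles spawning of PharahBulletUlt_BP to roughly every 0.1 seconds.
; Bullets spawn at the character's Arrow1 transform, randomly scattered along world Y and Z.
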(event EventTick
  (params (DeltaSeconds :type Float%20%28single-precision%29))
  (bind _owningcharacter (Variables|Default|GetOwningCharacter))
  (bind _aspharah_bp (Utilities|Casting|CastToPharah_BP _owningcharacter))
  (bind _arrow1 (Variables|/Game/_Project/Characters/Pharah/Pharah_BP.Pharah_BP_C|GetArrow1 _aspharah_bp))
  (bind _returnvalue (Transformation|GetWorldTransform _arrow1))
  (if (Variables|Default|GetActive)
    (Pawn|Input|AddMovementInput (Variables|Default|GetOwningCharacter) "0.000000,0.000000,0.250000" 1.0 false)
    (Utilities|FlowControl|Delay 0.1)
    (Game|SpawnActorfromClass "/Game/_Project/Characters/Pharah/Ultimate/PharahBulletUlt_BP.PharahBulletUlt_BP_C" (Math|Transform|MakeTransform (Math|Vector|MakeVector (.x (.location _returnvalue)) (+ (.y (.location _returnvalue)) (Math|Random|RandomFloatinRange -1e+02 1e+02)) (+ (.z (.location _returnvalue)) (Math|Random|RandomFloatinRange -1e+02 1e+02))) (.rotation _returnvalue) (.scale _returnvalue)) "Undefined" "MultiplyWithRoot" 0 0)))

(event EventFire
  (|CallParentFunction)
  (if (Utilities|Enum|Equal(Enum) (Variables|Default|GetState) "NewEnumerator2")
    (Variables|Default|SetActive true)
    (Utilities|FlowControl|Delay 2.5)
    (Variables|Default|SetActive false)
    (CallFunction|Finish)))