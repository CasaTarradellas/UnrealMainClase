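; Pharah's horizontal jump skill, which launches the owning character in the direction the camera faces.
; Fire runs the parent skill logic, then proceeds only if the skill's State matches the required value.
; The launch adds camera forward scaled by Power, plus a fixed upward boost, to the current velocity without overriding it.
; The skill calls Finish immediately after the launch.
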(event EventFire
  (bind _owningcharacter (Variables|Default|GetOwningCharacter))
  (|CallParentFunction)
  (if (Utilities|Enum|Equal(Enum) (Variables|Default|GetState) "NewEnumerator1")
    (Character|LaunchCharacter _owningcharacter (+ (* (Math|Vector|GetForwardVector (Variables|/Game/_Project/Characters/BaseCharacter_BP.BaseCharacter_BP_C|GetCamera _owningcharacter)) (Variables|Default|GetPower)) "0.000000,0.000000,350.000000") false false)
    (CallFunction|Finish)))