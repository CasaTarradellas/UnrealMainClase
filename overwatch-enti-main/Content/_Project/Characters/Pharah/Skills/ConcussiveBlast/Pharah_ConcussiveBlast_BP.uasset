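; Pharah's Concussive Blast skill Blueprint, which launches the blast projectile when fired.
; Fire runs the parent logic, then, if the skill is in the required state, spawns the bullet actor at the Arrow1 transform on Pharah.
; It then adds ultimate charge to the owner, sets the bullet's sphere not to ignore the owner when moving, and finishes the skill.
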(event EventFire
  (|CallParentFunction)
  (if (Utilities|Enum|Equal(Enum) (Variables|Default|GetState) "NewEnumerator1")
    (bind _returnvalue (Game|SpawnActorfromClass "/Game/_Project/Characters/Pharah/Skills/ConcussiveBlast/PharahConcBl_Bullet_BP.PharahConcBl_Bullet_BP_C" (Transformation|GetWorldTransform (Variables|/Game/_Project/Characters/Pharah/Pharah_BP.Pharah_BP_C|GetArrow1 (.AsPharah%20BP (Utilities|Casting|CastToPharah_BP (Variables|Default|GetOwningCharacter))))) "Undefined" "MultiplyWithRoot" 0 0))
    (Default|AddCharge (Variables|/Game/_Project/Characters/BaseCharacter_BP.BaseCharacter_BP_C|GetUltimate (Variables|Default|GetOwningCharacter)) 5e+01)
    (Collision|IgnoreActorwhenMoving (Variables|/Game/_Project/Characters/Pharah/Skills/ConcussiveBlast/PharahConcBl_Bullet_BP.PharahConcBl_Bullet_BP_C|GetSphere _returnvalue) (Variables|Default|GetOwningCharacter) false)
    (CallFunction|Finish)))