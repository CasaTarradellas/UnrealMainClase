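; Pharah's vertical jump skill, a Blueprint ability that boosts the character straight up.
; Its Fire event calls the parent skill logic, then, if the skill is in a specific state, launches the owning character upward without overriding existing velocity.
; It also adds a fixed amount to Pharah's Fuel through a cast to Pharah_BP, then finishes the skill.
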(event EventFire
  (bind _owningcharacter (Variables|Default|GetOwningCharacter))
  (bind _aspharah_bp (Utilities|Casting|CastToPharah_BP _owningcharacter))
  (|CallParentFunction)
  (if (Utilities|Enum|Equal(Enum) (Variables|Default|GetState) "NewEnumerator1")
    (Character|LaunchCharacter _owningcharacter "0.000000,0.000000,1000.000000" false false)
    (Variables|/Game/_Project/Characters/Pharah/Pharah_BP.Pharah_BP_C|SetFuel _aspharah_bp (+ (Variables|/Game/_Project/Characters/Pharah/Pharah_BP.Pharah_BP_C|GetFuel _aspharah_bp) 5e+01))
    (CallFunction|Finish)))