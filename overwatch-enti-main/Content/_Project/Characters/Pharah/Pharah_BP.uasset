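; Pharah hero character Blueprint that sets up health, three skills bound to inputs, an ultimate and a fuel-based hover jetpack.
; BeginPlay initializes each skill component with its control label and registers it in Skills, and input actions fire them.
; Holding Space with enough fuel switches movement to Flying; Tick then drains fuel while nudging upward, or refills it when not flying.
; Tick also prints fuel and destroys the actor at zero health.
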(event Input|EnhancedActionEvents|EnhancedInputActionSkill_0
  (params (ActionValue :type Boolean) (ElapsedSeconds :type Float%20%28double-precision%29) (TriggeredSeconds :type Float%20%28double-precision%29) (InputAction :type Input%20Action%20Object%20Reference :default "/Game/_Project/CommonSystems/Input/Skill_0.Skill_0"))
  (Default|Fire (Variables|Default|GetPharah_VerticalJump_BP)))

(event Input|EnhancedActionEvents|EnhancedInputActionSkill_1
  (params (ActionValue :type Boolean) (ElapsedSeconds :type Float%20%28double-precision%29) (TriggeredSeconds :type Float%20%28double-precision%29) (InputAction :type Input%20Action%20Object%20Reference :default "/Game/_Project/CommonSystems/Input/Skill_1.Skill_1"))
  (Default|Fire (Variables|Default|GetPharah_ConcussiveBlast_BP)))

(event Input|EnhancedActionEvents|EnhancedInputActionSecondaryFire
  (params (ActionValue :type Boolean) (ElapsedSeconds :type Float%20%28double-precision%29) (TriggeredSeconds :type Float%20%28double-precision%29) (InputAction :type Input%20Action%20Object%20Reference :default "/Game/_Project/CommonSystems/Input/SecondaryFire.SecondaryFire"))
  (Default|Fire (Variables|Default|GetPharah_HorizontalJump_Skill_BP)))

(event Input|EnhancedActionEvents|EnhancedInputActionUltimate
  (params (ActionValue :type Boolean) (ElapsedSeconds :type Float%20%28double-precision%29) (TriggeredSeconds :type Float%20%28double-precision%29) (InputAction :type Input%20Action%20Object%20Reference :default "/Game/_Project/CommonSystems/Input/Ultimate.Ultimate"))
  (Default|Fire (Variables|Default|GetUltimate)))

(event EventBeginPlay
  (bind _pharah_horizontaljump_skill_bp (Variables|Default|GetPharah_HorizontalJump_Skill_BP))
  (bind _pharah_concussiveblast_bp (Variables|Default|GetPharah_ConcussiveBlast_BP))
  (bind _pharah_verticaljump_bp (Variables|Default|GetPharah_VerticalJump_BP))
  (|CallParentFunction)
  (Utilities|FlowControl|Sequence
    (:then_0
      (CallFunction|InitializeHealth (Utilities|Struct|MakeHealthData 225.0 225.0 0.0 0.0 0.0 0.0 0.0 false)))
    (:then_1
      (Default|Initialize _pharah_horizontaljump_skill_bp self "RIGHT CLICK")
      (Utilities|Array|Add (Variables|Default|GetSkills) _pharah_horizontaljump_skill_bp))
    (:then_2
      (Default|Initialize _pharah_concussiveblast_bp self "E")
      (Utilities|Array|Add (Variables|Default|GetSkills) _pharah_concussiveblast_bp))
    (:then_3
      (Default|Initialize _pharah_verticaljump_bp self "RIGHT SHIFT")
      (Utilities|Array|Add (Variables|Default|GetSkills) _pharah_verticaljump_bp))))

(event EventTick
  (params (DeltaSeconds :type Float%20%28single-precision%29))
  (bind _returnvalue (* DeltaSeconds 15.0))
  (|CallParentFunction DeltaSeconds)
  (Utilities|FlowControl|Sequence
    (:then_0
      (if (Variables|Default|GetFlying)
        (if (> (Variables|Default|GetFuel) 0.1)
          (Variables|Default|SetFuel (- (Variables|Default|GetFuel) _returnvalue))
          (Pawn|Input|AddMovementInput "0.000000,0.000000,0.250000" 1.0 false)
          (else
            (Pawn|Components|CharacterMovement|SetMovementMode (Variables|Character|GetCharacterMovement) "MOVE_Falling" 0)
            (Variables|Default|SetFlying false)))
        (elif (< (Variables|Default|GetFuel) (Variables|Default|GetMaxFuel))
          (Variables|Default|SetFuel (+ _returnvalue (Variables|Default|GetFuel))))))
    (:then_1
      (Development|PrintText (Utilities|Text|ToText(Float) (Variables|Default|GetFuel) "HalfToEven") true true "(R=0.000000,G=0.660000,B=1.000000,A=1.000000)" 0.01))
    (:then_2
      (if (<= (.currenthealth (Default|GetHealthData (Variables|Default|GetHealthSystem))) 0.0)
        (Actor|DestroyActor)))))

(event Input|KeyboardEvents|SpaceBar
  (params (Key :type Key%20Structure :default "None"))
  (:Pressed
    (if (> (Variables|Default|GetFuel) 2e+01)
      (Pawn|Components|CharacterMovement|SetMovementMode (Variables|Character|GetCharacterMovement) "MOVE_Flying" 0)
      (Variables|Default|SetFlying true)
      (else
        (if (Class|NavMovementComponent|IsFlying (Variables|Character|GetCharacterMovement)) :!label _label
          (Pawn|Components|CharacterMovement|SetMovementMode (Variables|Character|GetCharacterMovement) "MOVE_Falling" 0)
          (else
            (Pawn|Components|CharacterMovement|SetMovementMode (Variables|Character|GetCharacterMovement) "MOVE_Walking" 0)))
        (Variables|Default|SetFlying false))))
  (:Released
    (goto _label)))

(fn ConstructionScript
  (|CallParentFunction))