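; Pharah's weapon Blueprint, a child weapon that fires projectile bullets and handles reload.
; Fire spawns a PharahBullet_BP at the character's arrow, adds ultimate charge, then runs parent fire logic, animation, cooldown and recoil.
; Tick mirrors the ultimate's active state to block firing while it runs.
; Reload picks a long or short time based on an empty magazine and drives the character's animation Blueprint.
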(event EventTick
  (params (DeltaSeconds :type Float%20%28single-precision%29))
  (|CallParentFunction DeltaSeconds)
  (if (Variables|/Game/_Project/Characters/Pharah/Ultimate/Pharah_Ultimate_BP.Pharah_Ultimate_BP_C|GetActive (.AsPharah%20Ultimate%20BP (Utilities|Casting|CastToPharah_Ultimate_BP (Variables|/Game/_Project/Characters/BaseCharacter_BP.BaseCharacter_BP_C|GetUltimate (Variables|Default|GetOwningCharacter)))))
    (Variables|Default|SetUltActive true)
    (elif (Variables|Default|GetUltActive)
      (Variables|Default|SetUltActive false))))

(event EventFire
  (if (not (Variables|Default|GetUltActive))
    (Utilities|FlowControl|Sequence
      (:then_0
        (bind _returnvalue (Game|SpawnActorfromClass "/Game/_Project/Characters/Pharah/Weapon/PharahBullet_BP.PharahBullet_BP_C" (Transformation|GetWorldTransform (Variables|/Game/_Project/Characters/Pharah/Pharah_BP.Pharah_BP_C|GetArrow1 (.AsPharah%20BP (Utilities|Casting|CastToPharah_BP (Variables|Default|GetOwningCharacter))))) "Undefined" "MultiplyWithRoot" 0 0))
        (Default|AddCharge (Variables|/Game/_Project/Characters/BaseCharacter_BP.BaseCharacter_BP_C|GetUltimate (Variables|Default|GetOwningCharacter)) 5e+01)
        (Collision|IgnoreActorwhenMoving (Variables|/Game/_Project/Characters/Pharah/Weapon/PharahBullet_BP.PharahBullet_BP_C|GetSphere _returnvalue) (Variables|Default|GetOwningCharacter) false))
      (:then_1
        (|CallParentFunction))
      (:then_2
        (Default|Fire (Variables|Default|GetAnimator))
        (CallFunction|EnterFireCooldown))
      (:then_3
        (CallFunction|AddRecoil 0.1 0.0)))))

(event EventInitialize
  (params (WeaponUI :type Weapon%20UI%20Object%20Reference) (OwningCharacter :type Base%20Character%20BP%20Object%20Reference))
  (|CallParentFunction WeaponUI OwningCharacter)
  (Variables|Default|SetAnimator (.AsRecruit%20Animation%20BP (Utilities|Casting|CastToRecruit_AnimationBP (Components|SkeletalMesh|GetAnimInstance (Variables|/Script/Engine.Character|GetMesh OwningCharacter))))))

(event EventReload
  (bind _currentammo (Variables|Default|GetCurrentAmmo))
  (bind _returnvalue (== _currentammo 0))
  (Utilities|FlowControl|Sequence
    (:then_0
      (Variables|Default|SetReloadTime (Math|Float|SelectFloat (Variables|Default|GetLong%20Reload%20Time) (Variables|Default|GetShort%20Reload%20Time) _returnvalue))
      (Default|DoReload (Variables|Default|GetAnimator) _returnvalue))
    (:then_1
      (|CallParentFunction))))