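; D.Va's mecha ultimate, which turns the mech into an exploding mecha and ejects the pilot.
; When fired in the required state, it spawns the exploding mecha at the character's transform, passing on the flying velocity saved at activation.
; It then plays the eject sound, spawns an on-foot D.Va at an offset, possesses her and destroys the original character.
; The exploding mecha's owner is reassigned to the new D.Va.
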(event EventBeginPlay)

(event EventTick
  (params (DeltaSeconds :type Float%20%28single-precision%29)))

(event EventFire
  (bind _owningcharacter (Variables|Default|GetOwningCharacter))
  (bind _owningcharacter_2 (Variables|Default|GetOwningCharacter))
  (bind _returnvalue (Transformation|GetActorTransform _owningcharacter_2))
  (|CallParentFunction)
  (if (Utilities|Enum|Equal(Enum) (Variables|Default|GetState) "NewEnumerator2")
    (bind _returnvalue_2 (Game|SpawnActorfromClass "/Game/_Project/Characters/DVa/Mecha/Ultimate/Exploding_Mecha_BP.Exploding_Mecha_BP_C" (Transformation|GetActorTransform _owningcharacter) "AlwaysSpawn" "MultiplyWithRoot" _owningcharacter (Variables|Default|GetFlyingVelocityOnActivate) _owningcharacter))
    (bind _babydvaref (CallFunction|SpawnBabyDVa (Math|Transform|MakeTransform (.location _returnvalue) (.rotation _returnvalue) (.scale _returnvalue))))
    (Actor|SetOwner _returnvalue_2 _babydvaref)))

(fn SpawnBabyDVa
  (params (InitTransform :type Transform))
  (Audio|PlaySoundatLocation "/Engine/EditorSounds/GamePreview/EjectFromPlayer.EjectFromPlayer" (.location InitTransform) "0, 0, 0" 1.0 1.0 0.0 0 0 0 0)
  (bind _returnvalue (Game|SpawnActorfromClass "/Game/_Project/Characters/DVa/DVa/DVa_BP.DVa_BP_C" (Math|Transform|MakeTransform (+ (.location InitTransform) (Variables|Default|GetExtractionImpulseDir)) (.rotation InitTransform) (.scale InitTransform)) "Undefined" "MultiplyWithRoot" 0 0))
  (Pawn|Possess (Pawn|GetController (Variables|Default|GetOwningCharacter)) _returnvalue)
  (Actor|DestroyActor (Variables|Default|GetOwningCharacter))
  (return _returnvalue))