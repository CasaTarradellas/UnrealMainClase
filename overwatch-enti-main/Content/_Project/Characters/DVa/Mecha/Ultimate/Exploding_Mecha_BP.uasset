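; Exploding mecha actor for D.Va's ultimate, which drifts on the velocity inherited from the mecha until its fuse runs out on Tick.
; It then overlaps pawns within the RadialForce radius, ignoring its owner, and damages their HealthSystem by distance falloff, capped by Min at 20% of ExplosionDamage.
; Finally, it spawns explosion effects and sound, adds charge to the owner's Ultimate and destroys itself.
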(event EventBeginPlay)

(event Collision|EventActorBeginOverlap
  (params (OtherActor :type Actor%20Object%20Reference)))

(event EventTick
  (params (DeltaSeconds :type Float%20%28single-precision%29))
  (bind _radialforce (Variables|Default|GetRadialForce))
  (bind _sphere (Variables|Default|GetSphere))
  (bind _returnvalue (Transformation|GetWorldLocation _sphere))
  (bind _radius (Variables|/Script/Engine.RadialForceComponent|GetRadius _radialforce))
  (if (>= (Variables|Default|GetcurrentTimeExploding) (Variables|Default|GettimeToExplode))
    (bind _outactors (Collision|SphereOverlapActors (Transformation|GetWorldLocation (Variables|Default|GetSphere)) _radius (Utilities|Array|MakeArray "ObjectTypeQuery3") 0 (Utilities|Array|MakeArray (Components|GetOwner))))
    (for _array_element _outactors
      (Utilities|IsValid (Actor|GetComponentbyClass _array_element "/Game/_Project/CommonSystems/HealthSystem/HealthSystem.HealthSystem_C")
        (:Is%20Valid
          (Default|TakeDamage (Actor|GetComponentbyClass _array_element "/Game/_Project/CommonSystems/HealthSystem/HealthSystem.HealthSystem_C") false (* (Variables|Default|GetexplosionDamage) (Math|Float|Min(Float) (- 1.0 (/ (Math|Vector|Distance(Vector) (Transformation|GetActorLocation _array_element) (Transformation|GetWorldLocation (Variables|Default|GetSphere))) _radius)) 0.2))))))
    (Utilities|FlowControl|DoOnce false
      (:Completed
        (Niagara|SpawnSystematLocation "/Game/MuzzleFlash/MuzzleFlash/Niagara/NS_MuzzleFlash.NS_MuzzleFlash" _returnvalue "0, 0, 0" "6.000000,6.000000,6.000000" true true "AutoRelease")
        (Audio|PlaySoundatLocation "/Game/_Project/StarterContent/Audio/Explosion01.Explosion01" _returnvalue "0, 0, 0" 1.0 1.0 0.0 0 0 0 0)
        (Default|AddCharge (Variables|/Game/_Project/Characters/BaseCharacter_BP.BaseCharacter_BP_C|GetUltimate (.AsBase%20Character%20BP (Utilities|Casting|CastToBaseCharacter_BP (Components|GetOwner self)))) 1e+02)
        (Actor|DestroyActor)))
    (else
      (Variables|Default|SetcurrentTimeExploding (+ DeltaSeconds (Variables|Default|GetcurrentTimeExploding)))
      (Transformation|AddActorWorldOffset (* (Variables|Default|GetinheritanceVelocityFromMecha) DeltaSeconds) true))))

(fn ConstructionScript)