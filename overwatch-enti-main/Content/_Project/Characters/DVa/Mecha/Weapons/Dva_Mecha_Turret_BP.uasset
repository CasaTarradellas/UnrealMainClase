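; D.Va mech turret weapon, a child weapon Blueprint that fires a spread of hitscan traces from the owner's camera.
; Each trace takes a random direction within the current spread cone and damages any hit HealthSystem, with headshot detection and clamped distance falloff.
; Hits add ultimate charge, and each shot runs the parent fire logic, fire cooldown and sound.
; The muzzle flash spawn is unconnected and never runs.
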(event EventBeginPlay)

(event EventTick
  (params (DeltaSeconds :type Float%20%28single-precision%29)))

(event EventFire
  (bind _owningcharacter (Variables|Default|GetOwningCharacter))
  (bind _camera (Variables|/Game/_Project/Characters/BaseCharacter_BP.BaseCharacter_BP_C|GetCamera _owningcharacter))
  (bind _returnvalue (Transformation|GetWorldLocation _camera))
  (Utilities|FlowControl|Sequence
    (:then_0
      (for _index (range 0 (Variables|Default|GetbulletsNum))
        (bind (_outhit _returnvalue_2) (Collision|LineTraceByChannel _returnvalue (+ _returnvalue (* (Math|Random|RandomUnitVectorinConeinDegrees (Math|Vector|GetForwardVector _camera) (Variables|Default|GetCurrentSpread)) (Variables|Default|GetFireDistance))) "TraceTypeQuery1" false 0 "None"))
        (if _returnvalue_2
          (Utilities|FlowControl|Sequence
            (:then_0
              (Utilities|IsValid (Actor|GetComponentbyClass (.HitActor (Collision|BreakHitResult _outhit)) "/Game/_Project/CommonSystems/HealthSystem/HealthSystem.HealthSystem_C")
                (:Is%20Valid
                  (Audio|SpawnSoundatLocation "/Engine/VREditor/Sounds/UI/Drop_Item_From_ContentBrowser.Drop_Item_From_ContentBrowser" _returnvalue "0, 0, 0" 2.0 1.0 0.0 0 0)
                  (Default|TakeDamage (Actor|GetComponentbyClass (.HitActor (Collision|BreakHitResult _outhit)) "/Game/_Project/CommonSystems/HealthSystem/HealthSystem.HealthSystem_C") (== (.HitBoneName (Collision|BreakHitResult _outhit)) "Head") (* (Variables|Default|GetDamage) (Math|Float|Max(Float) (- 1.0 (/ (.Distance (Collision|BreakHitResult _outhit)) (Variables|Default|GetFireDistance))) 0.2)))
                  (Default|AddCharge (Variables|/Game/_Project/Characters/BaseCharacter_BP.BaseCharacter_BP_C|GetUltimate (Variables|Default|GetOwningCharacter)) (Math|Float|SelectFloat (Variables|Default|GetultimateChargePerHeadshot_0) (Variables|Default|GetultimateChargePerHit_0) (== (.HitBoneName (Collision|BreakHitResult _outhit)) "Head"))))))))))
    (:then_1
      (|CallParentFunction))
    (:then_2
      (CallFunction|EnterFireCooldown))
    (:then_3
      (Audio|PlaySoundatLocation "/Game/StarterContent/Audio/Explosion02.Explosion02" (Transformation|GetActorLocation (Variables|Default|GetOwningCharacter)) "0, 0, 0" 1.0 1.0 0.0 0 0 0 0))))

(event EventInitialize
  (params (WeaponUI :type Weapon%20UI%20Object%20Reference) (OwningCharacter :type Base%20Character%20BP%20Object%20Reference))
  (|CallParentFunction WeaponUI OwningCharacter))