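; D.Va's mecha character Blueprint, a playable hero with armor-heavy health, built on a parent character class.
; On possession it initializes health and registers Boosters, Rockets Launcher and Barrier skills, each triggered by its own input.
; Holding the barrier disables the current weapon, and shooting changes walk speed each tick.
; The ultimate cancels boosters in a given state and inherits their velocity, while death spawns Baby D.Va through the ultimate.
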(event Input|EnhancedActionEvents|EnhancedInputActionUltimate
  (params (ActionValue :type Boolean) (ElapsedSeconds :type Float%20%28double-precision%29) (TriggeredSeconds :type Float%20%28double-precision%29) (InputAction :type Input%20Action%20Object%20Reference :default "/Game/_Project/CommonSystems/Input/Ultimate.Ultimate"))
  (bind _dva_boosters_skill_bp (Variables|Default|GetDVa_Boosters_Skill_BP))
  (bind _ultimate (Variables|Default|GetUltimate))
  (Utilities|FlowControl|Sequence
    (:then_0
      (if (Utilities|Enum|Equal(Enum) (Variables|/Game/_Project/CommonSystems/Character_Skills/Character_Skill_BP.Character_Skill_BP_C|GetState _dva_boosters_skill_bp) "NewEnumerator1")
        (Variables|/Game/_Project/Characters/DVa/Mecha/Ultimate/DVa_Mecha_Ultimate_BP.DVa_Mecha_Ultimate_BP_C|SetFlyingVelocityOnActivate (.AsDVa%20Mecha%20Ultimate%20BP (Utilities|Casting|CastToDVa_Mecha_Ultimate_BP _ultimate)) (Transformation|GetVelocity))
        (Default|Cancel _dva_boosters_skill_bp)))
    (:then_1
      (Default|Fire _ultimate))))

(event Input|EnhancedActionEvents|EnhancedInputActionSkill_0
  (params (ActionValue :type Boolean) (ElapsedSeconds :type Float%20%28double-precision%29) (TriggeredSeconds :type Float%20%28double-precision%29) (InputAction :type Input%20Action%20Object%20Reference :default "/Game/_Project/CommonSystems/Input/Skill_0.Skill_0"))
  (:Started
    (Default|Fire (Variables|Default|GetDVa_Boosters_Skill_BP))))

(event Input|EnhancedActionEvents|EnhancedInputActionSecondaryFire
  (params (ActionValue :type Boolean) (ElapsedSeconds :type Float%20%28double-precision%29) (TriggeredSeconds :type Float%20%28double-precision%29) (InputAction :type Input%20Action%20Object%20Reference :default "/Game/_Project/CommonSystems/Input/SecondaryFire.SecondaryFire"))
  (bind _dva_barrier_skill_bp (Variables|Default|GetDVa_Barrier_Skill_BP))
  (bind _weapons (Variables|Default|GetWeapons))
  (bind _currentweaponindex (Variables|Default|GetCurrentWeaponIndex))
  (bind _output (Utilities|Array|Get(acopy) _weapons _currentweaponindex))
  (:Started
    (Default|Fire _dva_barrier_skill_bp)
    (Default|SetDisabled _output true))
  (:Canceled
    (Default|CancelBarrier _dva_barrier_skill_bp :!label _label)
    (Default|SetDisabled _output false))
  (:Completed
    (goto _label)))

(event Input|EnhancedActionEvents|EnhancedInputActionSkill_1
  (params (ActionValue :type Boolean) (ElapsedSeconds :type Float%20%28double-precision%29) (TriggeredSeconds :type Float%20%28double-precision%29) (InputAction :type Input%20Action%20Object%20Reference :default "/Game/_Project/CommonSystems/Input/Skill_1.Skill_1"))
  (:Started
    (Default|Fire (Variables|Default|GetDVa_RocketsLauncher_Skill_BP))))

(event EventBeginPlay
  (|CallParentFunction))

(event Collision|EventActorBeginOverlap
  (params (OtherActor :type Actor%20Object%20Reference)))

(event EventTick
  (params (DeltaSeconds :type Float%20%28single-precision%29))
  (|CallParentFunction DeltaSeconds)
  (Variables|/Script/Engine.CharacterMovementComponent|SetMaxWalkSpeed (Variables|Character|GetCharacterMovement) (select (Variables|/Game/_Project/CommonSystems/Weapon/BaseWeapon.BaseWeapon_C|GetWantsToShoot (Utilities|Array|Get(acopy) (Variables|Default|GetWeapons) (Variables|Default|GetCurrentWeaponIndex))) (Variables|Default|GetshootingMoveSpeed) (Variables|Default|GetmoveSpeed))))

(event EventDie
  (Default|SpawnBabyDVa (.AsDVa%20Mecha%20Ultimate%20BP (Utilities|Casting|CastToDVa_Mecha_Ultimate_BP (Variables|Default|GetUltimate))) (Transformation|GetActorTransform))
  (|CallParentFunction))

(event EventPossessed
  (params (NewController :type Controller%20Object%20Reference))
  (bind _self self)
  (bind _skills (Variables|Default|GetSkills))
  (bind _dva_boosters_skill_bp (Variables|Default|GetDVa_Boosters_Skill_BP))
  (bind _dva_rocketslauncher_skill_bp (Variables|Default|GetDVa_RocketsLauncher_Skill_BP))
  (bind _dva_barrier_skill_bp (Variables|Default|GetDVa_Barrier_Skill_BP))
  (|CallParentFunction NewController)
  (Utilities|FlowControl|Sequence
    (:then_0
      (Default|Initialize (Variables|Default|GetHealthSystem) (Utilities|Struct|MakeHealthData 1e+02 1e+02 4e+02 4e+02 0.0 0.0 0.0 false)))
    (:then_1
      (Default|Initialize _dva_boosters_skill_bp _self "L SHIFT")
      (Utilities|Array|Add _skills _dva_boosters_skill_bp))
    (:then_2
      (Default|Initialize _dva_rocketslauncher_skill_bp _self "E")
      (Utilities|Array|Add _skills _dva_rocketslauncher_skill_bp))
    (:then_3
      (Default|Initialize _dva_barrier_skill_bp _self "R CLICK")
      (Utilities|Array|Add _skills _dva_barrier_skill_bp))))

(fn ConstructionScript
  (|CallParentFunction))