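; D.Va mecha Boosters skill that flies the character along the camera's forward vector for a limited duration.
; Fire switches movement to Flying with move input ignored; Update relaunches the character every tick while active.
; A timer or second Fire cancels, restoring Falling and clearing the hit list.
; Actor-hit events knock other characters away with a sound, once per character per boost.
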(event Custom|Cancel
  (if (Utilities|Enum|Equal(Enum) (Variables|Default|GetState) "NewEnumerator1")
    (CallFunction|Finish)
    (CallFunction|DisableFlying)
    (Utilities|Array|Clear (Variables|Default|GethitCharactersOnBoost))))

(event Custom|EnableFlying
  (bind _owningcharacter (Variables|Default|GetOwningCharacter))
  (Pawn|Components|CharacterMovement|SetMovementMode (Variables|/Script/Engine.Character|GetCharacterMovement _owningcharacter) "MOVE_Flying" 0)
  (Input|SetIgnoreMoveInput (Pawn|GetController _owningcharacter) true))

(event Custom|DisableFlying
  (bind _owningcharacter (Variables|Default|GetOwningCharacter))
  (bind _charactermovement (Variables|/Script/Engine.Character|GetCharacterMovement _owningcharacter))
  (Pawn|Components|CharacterMovement|SetMovementMode _charactermovement "MOVE_Falling" 0)
  (Input|SetIgnoreMoveInput (Pawn|GetController _owningcharacter) false)
  (Pawn|Components|CharacterMovement|ClearAccumulatedForces _charactermovement))

(event Custom|PushOnHitCharacter
  (params (SelfActor :type Actor%20Object%20Reference) (OtherActor :type Actor%20Object%20Reference) (NormalImpulse :type Vector) (Hit :type Hit%20Result%20Structure%20%28by%20ref%29))
  (bind _returnvalue (Transformation|GetActorLocation SelfActor))
  (bind _ascharacter (Utilities|Casting|CastToCharacter OtherActor))
  (if (Utilities|Enum|Equal(Enum) (Variables|Default|GetState) "NewEnumerator1")
    (Utilities|IsValid _ascharacter
      (:Is%20Valid
        (if (not (Utilities|Array|ContainsItem (Variables|Default|GethitCharactersOnBoost) _ascharacter))
          (Character|LaunchCharacter _ascharacter (* (Math|Vector|Normalize (+ (- (Transformation|GetActorLocation _ascharacter) _returnvalue) "0.000000,0.000000,10.000000")) (Variables|Default|GetpushForce)) true true)
          (Utilities|Array|Add (Variables|Default|GethitCharactersOnBoost) _ascharacter)
          (Audio|PlaySoundatLocation "/Engine/VREditor/Sounds/UI/Foliage_Placed.Foliage_Placed" _returnvalue "0, 0, 0" 1.0 1.0 0.0 0 0 0 0))))))

(event EventFire
  (bind _state (Variables|Default|GetState))
  (bind _returnvalue (Utilities|Enum|Equal(Enum) _state "NewEnumerator1"))
  (if _returnvalue
    (CallFunction|Cancel)
    (else
      (|CallParentFunction)
      (if _returnvalue
        (Utilities|FlowControl|Sequence
          (:then_0
            (CallFunction|EnableFlying)
            (Utilities|Time|SetTimerbyEvent (delegate Custom|Cancel) (Variables|Default|GetboostDuration) false true))
          (:then_1
            (Default|SetActive (Variables|Default|GetUI) true)))))))

(event EventUpdate
  (params (DeltaTime :type Float%20%28double-precision%29))
  (bind _owningcharacter (Variables|Default|GetOwningCharacter))
  (|CallParentFunction DeltaTime)
  (if (Utilities|Enum|Equal(Enum) (Variables|Default|GetState) "NewEnumerator1")
    (Character|LaunchCharacter _owningcharacter (* (Math|Vector|GetForwardVector (Variables|/Game/_Project/Characters/BaseCharacter_BP.BaseCharacter_BP_C|GetCamera _owningcharacter)) 1.5e+03) true true)))

(event EventInitialize
  (params (OwningCharacter :type Base%20Character%20BP%20Object%20Reference) (Control%20Text :type String))
  (|CallParentFunction OwningCharacter Control%20Text)
  (Collision|BindEventtoOnActorHit (Variables|Default|GetOwningCharacter) (delegate Custom|PushOnHitCharacter)))