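; D.Va mech rocket launcher skill that fires a timed volley of rockets toward the camera's aim point.
; While in its firing state, Update spawns a rocket at each interval from alternating left and right points, playing a sound, then finishes once the count is reached.
; Each shot re-traces from the camera, ignoring projectile barriers and launched rockets, so the volley follows live aim.
; Fire activates the skill's UI.
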(event EventFire
  (|CallParentFunction)
  (if (Utilities|Enum|Equal(Enum) (Variables|Default|GetState) "NewEnumerator1")
    (Default|SetActive (Variables|Default|GetUI) true)))

(event EventUpdate
  (params (DeltaTime :type Float%20%28double-precision%29))
  (bind _rocketdistance (Variables|Default|GetrocketDistance))
  (bind _rocketslaunched (Variables|Default|GetrocketsLaunched))
  (bind _actors_to_ignore (Variables|Default|GetActors%20to%20Ignore))
  (bind _owningcharacter (Variables|Default|GetOwningCharacter))
  (bind _camera (Variables|/Game/_Project/Characters/BaseCharacter_BP.BaseCharacter_BP_C|GetCamera _owningcharacter))
  (bind _returnvalue (Math|Vector|GetForwardVector _camera))
  (bind _returnvalue_2 (Transformation|GetWorldLocation _camera))
  (bind _returnvalue_3 (* _returnvalue _rocketdistance))
  (bind _returnvalue_4 (+ _returnvalue_2 _returnvalue_3))
  (|CallParentFunction DeltaTime)
  (if (and (>= (Variables|Default|GetcurrentWaitTimeBetweenRockets) (Variables|Default|GettimeBetweenRockets)) (Utilities|Enum|Equal(Enum) (Variables|Default|GetState) "NewEnumerator1"))
    (if (> (Variables|Default|GetrocketsNum) (Utilities|Array|Length _rocketslaunched))
      (bind _outactors (Actor|GetAllActorsOfClass "/Game/_Project/Characters/DVa/Mecha/Skills/ProjectileBarrier/ProjectileBarrier.ProjectileBarrier_C"))
      (Utilities|Array|AppendArray _actors_to_ignore _outactors)
      (Utilities|Array|AppendArray _actors_to_ignore _rocketslaunched)
      (bind (_outhit _returnvalue_5) (Collision|LineTraceByChannel _returnvalue_2 _returnvalue_4 "TraceTypeQuery1" false _actors_to_ignore "None"))
      (if _returnvalue_5
        (Variables|Default|SetTargetLocation (.Location (Collision|BreakHitResult _outhit)))
        (else
          (Variables|Default|SetTargetLocation _returnvalue_4)))
      (bind _returnvalue_6 (Game|SpawnActorfromClass "/Game/_Project/Characters/DVa/Mecha/Skills/RocketsLauncher/Rocket.Rocket_C" (Math|Transform|MakeTransform (Math|Transform|TransformLocation (Transformation|GetActorTransform (Variables|Default|GetOwningCharacter)) (select (Variables|Default|GetIsLastFromRight) (Variables|Default|GetspawnPointLeft) (Variables|Default|GetspawnPointRight))) (Math|Rotator|FindLookatRotation (Math|Transform|TransformLocation (Transformation|GetActorTransform (Variables|Default|GetOwningCharacter)) (select (Variables|Default|GetIsLastFromRight) (Variables|Default|GetspawnPointLeft) (Variables|Default|GetspawnPointRight))) (Variables|Default|GetTargetLocation)) "1.000000,1.000000,1.000000") "Undefined" "MultiplyWithRoot" (Variables|Default|GetOwningCharacter) 0))
      (Variables|Default|SetIsLastFromRight (not (Variables|Default|GetIsLastFromRight)))
      (Variables|/Game/_Project/Characters/DVa/Mecha/Skills/RocketsLauncher/Rocket.Rocket_C|SetowningCharacter _returnvalue_6 (Variables|Default|GetOwningCharacter))
      (Utilities|Array|Add (Variables|Default|GetrocketsLaunched) _returnvalue_6)
      (Audio|PlaySoundatLocation "/Game/_Project/StarterContent/Audio/Explosion01.Explosion01" (Transformation|GetActorLocation (Variables|Default|GetOwningCharacter)) "0, 0, 0" 0.7 1.0 0.0 0 0 0 0)
      (Variables|Default|SetcurrentWaitTimeBetweenRockets 0.0)
      (else
        (CallFunction|Finish)
        (Utilities|Array|Clear (Variables|Default|GetrocketsLaunched))))
    (else
      (Variables|Default|SetcurrentWaitTimeBetweenRockets (+ (Variables|Default|GetcurrentWaitTimeBetweenRockets) DeltaTime)))))