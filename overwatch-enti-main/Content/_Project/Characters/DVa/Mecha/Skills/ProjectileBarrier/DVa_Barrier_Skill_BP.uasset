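; D.Va mecha skill that projects a barrier in front of the player's camera, limited by an energy pool.
; Firing requires a minimum energy, calls the parent skill logic, then spawns the barrier and passes it the camera.
; Update drains energy per call while active, ignoring delta time, and regenerates it otherwise.
; When energy runs out, the barrier is destroyed and the skill finishes.
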(event Custom|CancelBarrier
  (bind _spawnedbarrier (Variables|Default|GetSpawnedBarrier))
  (Utilities|IsValid _spawnedbarrier
    (:Is%20Valid
      (Actor|DestroyActor _spawnedbarrier)
      (CallFunction|Finish))))

(event EventBeginPlay)

(event EventTick
  (params (DeltaSeconds :type Float%20%28single-precision%29)))

(event EventUpdate
  (params (DeltaTime :type Float%20%28double-precision%29))
  (|CallParentFunction DeltaTime)
  (if (Utilities|Enum|Equal(Enum) (Variables|Default|GetState) "NewEnumerator1")
    (Variables|Default|SetcurrentEnergy (- (Variables|Default|GetcurrentEnergy) 2.0))
    (if (<= (Variables|Default|GetcurrentEnergy) 0.0)
      (CallFunction|CancelBarrier))
    (elif (< (Variables|Default|GetcurrentEnergy) (Variables|Default|GetmaxBarrierEnergy))
      (Variables|Default|SetcurrentEnergy (+ (Variables|Default|GetcurrentEnergy) 1.5)))))

(event EventFire
  (bind _owningcharacter (Variables|Default|GetOwningCharacter))
  (bind _camera (Variables|/Game/_Project/Characters/BaseCharacter_BP.BaseCharacter_BP_C|GetCamera _owningcharacter))
  (if (>= (Variables|Default|GetcurrentEnergy) 2e+01)
    (|CallParentFunction)
    (if (Utilities|Enum|Equal(Enum) (Variables|Default|GetState) "NewEnumerator1")
      (Default|SetActive (Variables|Default|GetUI) true)
      (bind _returnvalue (Game|SpawnActorfromClass "/Game/_Project/Characters/DVa/Mecha/Skills/ProjectileBarrier/ProjectileBarrier.ProjectileBarrier_C" (Math|Transform|MakeTransform (+ (* (Math|Vector|GetForwardVector _camera) (Variables|Default|GetspawnDistanceFromPlayer)) (Transformation|GetWorldLocation _camera)) "0, 0, 0" "1.000000,1.000000,1.000000") "Undefined" "OverrideRootScale" _owningcharacter _owningcharacter))
      (bind _output_get (Variables|Default|SetSpawnedBarrier _returnvalue))
      (Variables|/Game/_Project/Characters/DVa/Mecha/Skills/ProjectileBarrier/ProjectileBarrier.ProjectileBarrier_C|Setcamera _output_get (Variables|/Game/_Project/Characters/BaseCharacter_BP.BaseCharacter_BP_C|GetCamera (Variables|Default|GetOwningCharacter))))))

(event EventInitialize
  (params (OwningCharacter :type Base%20Character%20BP%20Object%20Reference) (Control%20Text :type String))
  (|CallParentFunction OwningCharacter Control%20Text)
  (Variables|Default|SetcurrentEnergy (Variables|Default|GetmaxBarrierEnergy)))