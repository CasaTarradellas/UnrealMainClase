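; D.Va's ultimate ability, which replaces the owning character with her mecha.
; Fire runs the parent logic, then calls SpawnMecha at the owner's transform if State matches a specific enum value.
; SpawnMecha spawns DVa_Mecha_BP with a location offset, hands it the owner's controller, destroys the old character and plays a sound at the spawn point.
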(event Custom|SpawnMecha
  (params (InitTransform :type Transform))
  (bind _spawnoffset (Variables|Default|GetspawnOffset))
  (bind _owningcharacter (Variables|Default|GetOwningCharacter))
  (bind _returnvalue (+ (.location InitTransform) _spawnoffset))
  (Utilities|FlowControl|Sequence
    (:then_0
      (bind _returnvalue_2 (Game|SpawnActorfromClass "/Game/_Project/Characters/DVa/Mecha/DVa_Mecha_BP.DVa_Mecha_BP_C" (Math|Transform|MakeTransform _returnvalue (.rotation InitTransform) (.scale InitTransform)) "Undefined" "MultiplyWithRoot" 0 0))
      (Pawn|Possess (Pawn|GetController _owningcharacter) _returnvalue_2)
      (Actor|DestroyActor _owningcharacter))
    (:then_1
      (Audio|PlaySoundatLocation "/Engine/EditorSounds/GamePreview/EjectFromPlayer.EjectFromPlayer" _returnvalue "0, 0, 0" 1.0 1.0 0.0 0 0 0 0))))

(event EventBeginPlay)

(event EventTick
  (params (DeltaSeconds :type Float%20%28single-precision%29)))

(event EventFire
  (|CallParentFunction)
  (if (Utilities|Enum|Equal(Enum) (Variables|Default|GetState) "NewEnumerator2")
    (CallFunction|SpawnMecha (Transformation|GetActorTransform (Variables|Default|GetOwningCharacter)))))