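; D.Va's weapon projectile, which deals damage on impact and charges the owner's ultimate.
; On hit it passes Damage to the target's HealthSystem component, flagging a headshot when the hit bone is named "Head".
; Those hits add ultimate charge to a BaseCharacter_BP owner, using separate amounts for headshots and regular hits.
; The projectile destroys itself after any hit.
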(event EventBeginPlay)

(event Collision|EventActorBeginOverlap
  (params (OtherActor :type Actor%20Object%20Reference)))

(event EventTick
  (params (DeltaSeconds :type Float%20%28single-precision%29)))

(event Collision|EventHit
  (params (MyComp :type Primitive%20Component%20Object%20Reference) (Other :type Actor%20Object%20Reference) (OtherComp :type Primitive%20Component%20Object%20Reference) (bSelfMoved :type Boolean) (HitLocation :type Vector :default "0, 0, 0") (HitNormal :type Vector :default "0, 0, 0") (NormalImpulse :type Vector :default "0, 0, 0") (Hit :type Hit%20Result%20Structure%20%28by%20ref%29))
  (bind _returnvalue (Actor|GetComponentbyClass Other "/Game/_Project/CommonSystems/HealthSystem/HealthSystem.HealthSystem_C"))
  (bind _returnvalue_2 (Components|GetOwner))
  (bind _returnvalue_3 (== (.hitbonename Hit) "Head"))
  (bind _asbase_character_bp (Utilities|Casting|CastToBaseCharacter_BP _returnvalue_2))
  (Utilities|IsValid _returnvalue
    (:Is%20Valid
      (Default|TakeDamage _returnvalue _returnvalue_3 (Variables|Default|Getdamage))
      (Utilities|IsValid _asbase_character_bp
        (:Is%20Valid
          (Default|AddCharge (Variables|/Game/_Project/Characters/BaseCharacter_BP.BaseCharacter_BP_C|GetUltimate _asbase_character_bp) (select _returnvalue_3 (Variables|Default|GetultimateChargePerHeadshot) (Variables|Default|GetultimateChargePerHit))))
        (:Is%20Not%20Valid
          _)))
    (:Is%20Not%20Valid
      _))
  (Actor|DestroyActor))

(fn ConstructionScript)