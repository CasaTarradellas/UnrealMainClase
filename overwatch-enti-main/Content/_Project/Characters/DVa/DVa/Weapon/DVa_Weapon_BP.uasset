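; DVa_Weapon_BP is D.Va's weapon Blueprint, which fires projectiles from the owning character's camera.
; Fire spawns a DVa_Weapon_Projectile_BP just ahead of the camera along its view direction, with the character as owner and instigator.
; It then runs the parent Fire, plays a sound at the spawn point and enters the fire cooldown.
; Initialize and BeginPlay only pass through to the parent class.
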(event EventBeginPlay
  (|CallParentFunction))

(event EventFire
  (bind _owningcharacter (Variables|Default|GetOwningCharacter))
  (bind _owningcharacter_2 (Variables|Default|GetOwningCharacter))
  (bind _camera (Variables|/Game/_Project/Characters/BaseCharacter_BP.BaseCharacter_BP_C|GetCamera _owningcharacter_2))
  (bind _returnvalue (Transformation|GetWorldLocation _camera))
  (bind _returnvalue_2 (Math|Vector|GetForwardVector _camera))
  (bind _returnvalue_3 (* _returnvalue_2 1e+02))
  (bind _returnvalue_4 (+ _returnvalue_3 _returnvalue))
  (Utilities|String|LogString "PIUM")
  (Utilities|FlowControl|Sequence
    (:then_0
      (Game|SpawnActorfromClass "/Game/_Project/Characters/DVa/DVa/Weapon/DVa_Weapon_Projectile_BP.DVa_Weapon_Projectile_BP_C" (Math|Transform|MakeTransform _returnvalue_4 (Transformation|GetWorldRotation _camera) "1.000000,1.000000,1.000000") "Undefined" "MultiplyWithRoot" _owningcharacter _owningcharacter))
    (:then_1
      (|CallParentFunction))
    (:then_2
      (Audio|PlaySoundatLocation "/Engine/VREditor/Sounds/UI/Teleport_Committed.Teleport_Committed" _returnvalue_4 "0, 0, 0" 1.0 1.0 0.0 0 0 0 0))
    (:then_3
      (CallFunction|EnterFireCooldown))))

(event EventInitialize
  (params (WeaponUI :type Weapon%20UI%20Object%20Reference) (OwningCharacter :type Base%20Character%20BP%20Object%20Reference))
  (|CallParentFunction WeaponUI OwningCharacter))