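; Base character Blueprint for Ana, a playable hero with a zoomable secondary fire, a grenade skill and a stun skill.
; On BeginPlay it initializes layered health, armor and shields, then registers both skill components, which input events fire.
; Secondary fire narrows camera FOV and lowers look sensitivity.
; Jumping cancels zoom and blocks it until a short timer after jump release clears the flag.
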(event Custom|ZoomCoolDown
  (Variables|Default|SetJumping false))

(event Input|EnhancedActionEvents|EnhancedInputActionSecondaryFire
  (params (ActionValue :type Boolean) (ElapsedSeconds :type Float%20%28double-precision%29) (TriggeredSeconds :type Float%20%28double-precision%29) (InputAction :type Input%20Action%20Object%20Reference :default "/Game/_Project/CommonSystems/Input/SecondaryFire.SecondaryFire"))
  (:Triggered
    (if (and ActionValue (not (Variables|Default|GetJumping))) :!label _label
      (Camera|SetFieldOfView (Variables|Default|GetCamera) 4e+01)
      (Variables|Default|SetCurrentSens 0.5)))
  (:Ongoing
    (goto _label))
  (:Completed
    (Camera|SetFieldOfView (Variables|Default|GetCamera) 9e+01)
    (Variables|Default|SetCurrentSens 1.0)))

(event Input|EnhancedActionEvents|EnhancedInputActionLook
  (params (ActionValue :type Vector%202D%20Structure) (ElapsedSeconds :type Float%20%28double-precision%29) (TriggeredSeconds :type Float%20%28double-precision%29) (InputAction :type Input%20Action%20Object%20Reference :default "/Game/_Project/CommonSystems/Input/Look.Look"))
  (bind (_x _y) (Math|Vector2D|BreakVector2D ActionValue))
  (bind _currentsens (Variables|Default|GetCurrentSens))
  (Pawn|Input|AddControllerYawInput (* _x _currentsens))
  (Pawn|Input|AddControllerPitchInput (* _y _currentsens)))

(event Input|EnhancedActionEvents|EnhancedInputActionJump
  (params (ActionValue :type Boolean) (ElapsedSeconds :type Float%20%28double-precision%29) (TriggeredSeconds :type Float%20%28double-precision%29) (InputAction :type Input%20Action%20Object%20Reference :default "/Game/_Project/CommonSystems/Input/Jump.Jump"))
  (:Triggered
    (Variables|Default|SetJumping true)
    (Camera|SetFieldOfView (Variables|Default|GetCamera) 9e+01)
    (Variables|Default|SetCurrentSens 1.0))
  (:Completed
    (Utilities|Time|SetTimerbyEvent (delegate Custom|ZoomCoolDown) 1.0)))

(event Input|EnhancedActionEvents|EnhancedInputActionSkill_0
  (params (ActionValue :type Boolean) (ElapsedSeconds :type Float%20%28double-precision%29) (TriggeredSeconds :type Float%20%28double-precision%29) (InputAction :type Input%20Action%20Object%20Reference :default "/Game/_Project/CommonSystems/Input/Skill_0.Skill_0"))
  (bind _ana_granade_skill_bp (Variables|Default|GetAna_Granade_Skill_BP))
  (:Started
    (Variables|/Game/_Project/Characters/Ana/Ana_Granade_Skill_BP.Ana_Granade_Skill_BP_C|SetSpawnPos _ana_granade_skill_bp (Transformation|GetWorldTransform (Variables|Default|GetGranadeSpawnPos)))
    (Default|Fire _ana_granade_skill_bp)))

(event Input|EnhancedActionEvents|EnhancedInputActionSkill_1
  (params (ActionValue :type Boolean) (ElapsedSeconds :type Float%20%28double-precision%29) (TriggeredSeconds :type Float%20%28double-precision%29) (InputAction :type Input%20Action%20Object%20Reference :default "/Game/_Project/CommonSystems/Input/Skill_1.Skill_1"))
  ;[0.15 0.15 0.15 0.5] Stun
  (Default|Fire (Variables|Default|GetAna_Stun_Skill_BP)))

(event Input|EnhancedActionEvents|EnhancedInputActionIA_Crouch
  (params (ActionValue :type Boolean) (ElapsedSeconds :type Float%20%28double-precision%29) (TriggeredSeconds :type Float%20%28double-precision%29) (InputAction :type Input%20Action%20Object%20Reference :default "/Game/_Project/Characters/Ana/IA_Crouch.IA_Crouch"))
  (:Triggered
    (Character|Crouch))
  (:Completed
    (Character|UnCrouch)))

(event EventBeginPlay
  (bind _ana_granade_skill_bp (Variables|Default|GetAna_Granade_Skill_BP))
  (bind _ana_stun_skill_bp (Variables|Default|GetAna_Stun_Skill_BP))
  (|CallParentFunction)
  (Utilities|FlowControl|Sequence
    (:then_0
      (Default|Initialize (Variables|Default|GetHealthSystem) (Utilities|Struct|MakeHealthData 5e+02 5e+02 5e+01 5e+01 5e+01 5e+01 5e+01 false)))
    (:then_1
      (Default|Initialize _ana_granade_skill_bp self "E")
      (Utilities|Array|Add (Variables|Default|GetSkills) _ana_granade_skill_bp))
    (:then_2
      (Default|Initialize _ana_stun_skill_bp self)
      (Utilities|Array|Add (Variables|Default|GetSkills) _ana_stun_skill_bp))))

(fn ConstructionScript
  (|CallParentFunction))