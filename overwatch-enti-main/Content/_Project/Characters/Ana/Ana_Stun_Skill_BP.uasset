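; Ana's stun skill, which puts an enemy to sleep by disabling its input and tipping it over.
; Fire line-traces from the camera for an Enemy-tagged actor, then adds Ultimate charge or sets OverCharge, depending on Ultimate state.
; A timer restores input and rotation, but one overcharge branch skips the tip-over, timer and Finish.
; The node saving OriginalRotation is unconnected, so the original rotation is never captured.
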(event Custom|SleepTime
  (bind _originalrotation (Variables|Default|GetOriginalRotation))
  (Input|EnableInput (.HitActor (Collision|BreakHitResult (stale EventFire _outhit))) (.As玩家控制器 (Utilities|Casting|CastToPlayerController (Pawn|GetController (.As角色 (Utilities|Casting|CastToCharacter (.HitActor (Collision|BreakHitResult (stale EventFire _outhit)))))))))
  (Transformation|SetActorRotation (.HitActor (Collision|BreakHitResult (stale EventFire _outhit))) (Math|Rotator|MakeRotator (.roll _originalrotation) (.pitch _originalrotation) 1.8e+02))
  (Development|PrintString "changebackrotation"))

(event EventFire
  (bind _owningcharacter (Variables|Default|GetOwningCharacter))
  (bind _owningcharacter_2 (Variables|Default|GetOwningCharacter))
  (bind _asana_base_bp (Utilities|Casting|CastToAna_base_BP _owningcharacter_2))
  (bind _camera (Variables|/Game/_Project/Characters/BaseCharacter_BP.BaseCharacter_BP_C|GetCamera _owningcharacter))
  (bind _returnvalue (Transformation|GetWorldLocation _camera))
  (|CallParentFunction)
  (if (Utilities|Enum|Equal(Enum) (Variables|Default|GetState) "NewEnumerator1")
    (bind (_outhit _returnvalue_2) (Collision|LineTraceByChannel _returnvalue (+ _returnvalue (* (Math|Vector|GetForwardVector _camera) (Variables|Default|GetHitDistance))) "TraceTypeQuery1" false 0 "ForDuration"))
    (if _returnvalue_2
      (if (Actor|ActorHasTag (.HitActor (Collision|BreakHitResult _outhit)) "Enemy")
        (Input|DisableInput (.HitActor (Collision|BreakHitResult _outhit)) (.As玩家控制器 (Utilities|Casting|CastToPlayerController (Pawn|GetController (.As角色 (Utilities|Casting|CastToCharacter (.HitActor (Collision|BreakHitResult _outhit))))))))
        (if (Utilities|Enum|Equal(Enum) (Variables|/Game/_Project/CommonSystems/Character_Ultimate/Ultimate_BP.Ultimate_BP_C|GetState (Variables|/Game/_Project/Characters/BaseCharacter_BP.BaseCharacter_BP_C|GetUltimate (Variables|Default|GetOwningCharacter))) "NewEnumerator0")
          (Default|AddCharge (Variables|/Game/_Project/Characters/BaseCharacter_BP.BaseCharacter_BP_C|GetUltimate (Variables|Default|GetOwningCharacter)) 5e+01)
          (Transformation|SetActorRotation (.HitActor (Collision|BreakHitResult _outhit)) (Math|Rotator|MakeRotator 1.8e+02 (+ (.pitch (Transformation|GetActorRotation (.HitActor (Collision|BreakHitResult _outhit)))) 9e+01) 0.0) :!label _label)
          (Utilities|Time|SetTimerbyEvent (delegate Custom|SleepTime) (Variables|Default|GetSleepTimer))
          (CallFunction|Finish)
          (elif (>= (Variables|/Game/_Project/Characters/Ana/Ana_base_BP.Ana_base_BP_C|GetMaxOverCharge _asana_base_bp) (+ (Variables|/Game/_Project/Characters/Ana/Ana_base_BP.Ana_base_BP_C|GetOverCharge _asana_base_bp) 5.0))
            (Variables|/Game/_Project/Characters/Ana/Ana_base_BP.Ana_base_BP_C|SetOverCharge _asana_base_bp (Variables|/Game/_Project/Characters/Ana/Ana_base_BP.Ana_base_BP_C|GetMaxOverCharge _asana_base_bp))
            (Development|PrintString "Overcharge ultimate")
            (else
              (Variables|/Game/_Project/Characters/Ana/Ana_base_BP.Ana_base_BP_C|SetOverCharge (.AsAna%20Base%20BP (Utilities|Casting|CastToAna_base_BP (Variables|Default|GetOwningCharacter))) 5.0)
              (Development|PrintString "Overcharge ultimate")
              (goto _label))))))))