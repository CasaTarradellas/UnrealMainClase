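; Ana's weapon Blueprint, a hitscan gun that damages enemies and heals allies over time.
; Fire traces from the camera, checks the hit actor's HealthSystem and Enemy or Ally tag, then plays the animation and starts cooldown.
; Looping timers apply damage or healing from the stored trace hit until a retriggerable delay clears them.
; Enemy hits charge the ultimate, with a headshot rate, or build OverCharge by ultimate state; heal ticks also feed OverCharge.
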(event Custom|DamageOverTime
  (Default|TakeDamage (Actor|GetComponentbyClass (.HitActor (Collision|BreakHitResult (stale EventFire _outhit))) "/Game/_Project/CommonSystems/HealthSystem/HealthSystem.HealthSystem_C") (== (.HitBoneName (Collision|BreakHitResult (stale EventFire _outhit))) "Head") (Variables|Default|GetDamage)))

(event Custom|HealOverTime
  (bind _owningcharacter (Variables|Default|GetOwningCharacter))
  (bind _asana_base_bp (Utilities|Casting|CastToAna_base_BP _owningcharacter))
  (Default|AddHealthType (Actor|GetComponentbyClass (.HitActor (Collision|BreakHitResult (stale EventFire _outhit))) "/Game/_Project/CommonSystems/HealthSystem/HealthSystem.HealthSystem_C") "NewEnumerator0" 15.0)
  (if (Utilities|Enum|Equal(Enum) (Variables|/Game/_Project/CommonSystems/Character_Ultimate/Ultimate_BP.Ultimate_BP_C|GetState (Variables|/Game/_Project/Characters/BaseCharacter_BP.BaseCharacter_BP_C|GetUltimate (Variables|Default|GetOwningCharacter))) "NewEnumerator0")
    (Default|AddCharge (Variables|/Game/_Project/Characters/BaseCharacter_BP.BaseCharacter_BP_C|GetUltimate (Variables|Default|GetOwningCharacter)) 0.0)
    (elif (>= (Variables|/Game/_Project/Characters/Ana/Ana_base_BP.Ana_base_BP_C|GetMaxOverCharge _asana_base_bp) (+ (Variables|/Game/_Project/Characters/Ana/Ana_base_BP.Ana_base_BP_C|GetOverCharge _asana_base_bp) 5.0))
      (Variables|/Game/_Project/Characters/Ana/Ana_base_BP.Ana_base_BP_C|SetOverCharge _asana_base_bp (Variables|/Game/_Project/Characters/Ana/Ana_base_BP.Ana_base_BP_C|GetMaxOverCharge _asana_base_bp))
      (Development|PrintString "Full Overcharge")
      (else
        (Variables|/Game/_Project/Characters/Ana/Ana_base_BP.Ana_base_BP_C|SetOverCharge (.AsAna%20Base%20BP (Utilities|Casting|CastToAna_base_BP (Variables|Default|GetOwningCharacter))) (+ (Variables|/Game/_Project/Characters/Ana/Ana_base_BP.Ana_base_BP_C|GetOverCharge (.AsAna%20Base%20BP (Utilities|Casting|CastToAna_base_BP (Variables|Default|GetOwningCharacter)))) 5.0))
        (Development|PrintString "Overcharge ultimate"))))
  (Development|PrintString (Utilities|String|ToString(Float) (.currenthealth (Default|GetHealthData (Actor|GetComponentbyClass (.HitActor (Collision|BreakHitResult (stale EventFire _outhit))) "/Game/_Project/CommonSystems/HealthSystem/HealthSystem.HealthSystem_C"))))))

(event EventFire
  (bind _owningcharacter (Variables|Default|GetOwningCharacter))
  (bind _owningcharacter_2 (Variables|Default|GetOwningCharacter))
  (bind _asana_base_bp (Utilities|Casting|CastToAna_base_BP _owningcharacter_2))
  (bind _camera (Variables|/Game/_Project/Characters/BaseCharacter_BP.BaseCharacter_BP_C|GetCamera _owningcharacter))
  (bind _returnvalue (Transformation|GetWorldLocation _camera))
  (|CallParentFunction)
  (Utilities|FlowControl|Sequence
    (:then_0
      (Development|PrintString "Shooting"))
    (:then_1
      (bind (_outhit _returnvalue_2) (Collision|LineTraceByChannel _returnvalue (+ _returnvalue (* (Math|Vector|GetForwardVector _camera) (Variables|Default|GetFireDistance))) "TraceTypeQuery1" false 0 "ForDuration" false))
      (if _returnvalue_2
        (Utilities|IsValid (Actor|GetComponentbyClass (.HitActor (Collision|BreakHitResult _outhit)) "/Game/_Project/CommonSystems/HealthSystem/HealthSystem.HealthSystem_C")
          (:Is%20Valid
            (if (Actor|ActorHasTag (.HitActor (Collision|BreakHitResult _outhit)) "Enemy")
              (Development|PrintString "hitting enemy")
              (if (Utilities|Enum|Equal(Enum) (Variables|/Game/_Project/CommonSystems/Character_Ultimate/Ultimate_BP.Ultimate_BP_C|GetState (Variables|/Game/_Project/Characters/BaseCharacter_BP.BaseCharacter_BP_C|GetUltimate (Variables|Default|GetOwningCharacter))) "NewEnumerator0")
                (Default|AddCharge (Variables|/Game/_Project/Characters/BaseCharacter_BP.BaseCharacter_BP_C|GetUltimate (Variables|Default|GetOwningCharacter)) (Math|Float|SelectFloat (Variables|Default|GetChargePerHeadshot) (Variables|Default|GetNormalCharge) (== (.HitBoneName (Collision|BreakHitResult _outhit)) "Head")))
                (elif (>= (+ (Variables|/Game/_Project/Characters/Ana/Ana_base_BP.Ana_base_BP_C|GetOverCharge _asana_base_bp) 5.0) (Variables|/Game/_Project/Characters/Ana/Ana_base_BP.Ana_base_BP_C|GetMaxOverCharge _asana_base_bp))
                  (Variables|/Game/_Project/Characters/Ana/Ana_base_BP.Ana_base_BP_C|SetOverCharge _asana_base_bp (Variables|/Game/_Project/Characters/Ana/Ana_base_BP.Ana_base_BP_C|GetMaxOverCharge _asana_base_bp))
                  (Development|PrintString "Full Overcharge")
                  (else
                    (Variables|/Game/_Project/Characters/Ana/Ana_base_BP.Ana_base_BP_C|SetOverCharge _asana_base_bp (+ (Variables|/Game/_Project/Characters/Ana/Ana_base_BP.Ana_base_BP_C|GetOverCharge _asana_base_bp) 5.0))
                    (Development|PrintString "Overcharge ultimate"))))
              (bind _returnvalue_3 (Utilities|Time|SetTimerbyEvent (delegate Custom|DamageOverTime) 0.3 true))
              (bind _output_get (Variables|Default|SetTimer _returnvalue_3))
              (Utilities|FlowControl|RetriggerableDelay 1.0)
              (Utilities|Time|ClearandInvalidateTimerbyHandle _output_get)
              (elif (Actor|ActorHasTag (.HitActor (Collision|BreakHitResult _outhit)) "Ally")
                (Development|PrintString "healling ally")
                (bind _returnvalue_4 (Utilities|Time|SetTimerbyEvent (delegate Custom|HealOverTime) 0.3 true))
                (bind _output_get_2 (Variables|Default|SetTimer _returnvalue_4))
                (Utilities|FlowControl|RetriggerableDelay 1.0)
                (Utilities|Time|ClearandInvalidateTimerbyHandle _output_get_2)))))))
    (:then_2
      (Default|Fire (Variables|Default|Getanimator))
      (CallFunction|EnterFireCooldown))))

(event EventInitialize
  (params (WeaponUI :type Weapon%20UI%20Object%20Reference) (OwningCharacter :type Base%20Character%20BP%20Object%20Reference))
  (|CallParentFunction WeaponUI OwningCharacter)
  (Variables|Default|Setanimator (.AsRecruit%20Animation%20BP (Utilities|Casting|CastToRecruit_AnimationBP (Components|SkeletalMesh|GetAnimInstance (Variables|/Script/Engine.Character|GetMesh OwningCharacter))))))