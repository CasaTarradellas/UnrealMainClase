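; Ana's grenade projectile, which damages enemies and heals allies in an area when it goes off.
; It destroys itself on impact, and its Destroyed event runs a pawn sphere overlap sized by HitDetector and spawns an explosion effect.
; Actor tags choose between damage and healing with overheal through each target's HealthSystem.
; Each affected target feeds the owner's ultimate, adding charge or setting Ana's OverCharge depending on the ultimate's state.
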(event OnComponentHit(Granade)
  (params (HitComponent :type Primitive%20Component%20Object%20Reference) (OtherActor :type Actor%20Object%20Reference) (OtherComp :type Primitive%20Component%20Object%20Reference) (NormalImpulse :type Vector :default "0, 0, 0") (Hit :type Hit%20Result%20Structure%20%28by%20ref%29))
  (Actor|DestroyActor))

(event EventDestroyed
  (bind _owningcharacter (Variables|Default|GetOwningCharacter))
  (bind _asana_base_bp (Utilities|Casting|CastToAna_base_BP _owningcharacter))
  (Utilities|FlowControl|Sequence
    (:then_0
      (bind (_outactors _returnvalue) (Collision|SphereOverlapActors (Transformation|GetActorLocation) (Components|Sphere|GetScaledSphereRadius (Variables|Default|GetHitDetector)) (Utilities|Array|MakeArray "ObjectTypeQuery3") 0))
      (if _returnvalue
        (for _array_element _outactors
          (Utilities|IsValid (Actor|GetComponentbyClass _array_element "/Game/_Project/CommonSystems/HealthSystem/HealthSystem.HealthSystem_C")
            (:Is%20Valid
              (if (Actor|ActorHasTag (Components|GetOwner (Actor|GetComponentbyClass _array_element "/Game/_Project/CommonSystems/HealthSystem/HealthSystem.HealthSystem_C")) "Enemy")
                (Development|PrintString "granade hit Enemy")
                (Default|TakeDamage (Actor|GetComponentbyClass _array_element "/Game/_Project/CommonSystems/HealthSystem/HealthSystem.HealthSystem_C") false 5e+01)
                (Utilities|IsValid (Variables|Default|GetOwningCharacter)
                  (:Is%20Valid
                    (if (Utilities|Enum|Equal(Enum) (Variables|/Game/_Project/CommonSystems/Character_Ultimate/Ultimate_BP.Ultimate_BP_C|GetState (Variables|/Game/_Project/Characters/BaseCharacter_BP.BaseCharacter_BP_C|GetUltimate (Variables|Default|GetOwningCharacter))) "NewEnumerator0")
                      (Default|AddCharge (Variables|/Game/_Project/Characters/BaseCharacter_BP.BaseCharacter_BP_C|GetUltimate (Variables|Default|GetOwningCharacter)) 2e+01)
                      (else
                        (Variables|/Game/_Project/Characters/Ana/Ana_base_BP.Ana_base_BP_C|SetOverCharge (.AsAna%20Base%20BP (Utilities|Casting|CastToAna_base_BP (Variables|Default|GetOwningCharacter))) 5.0)
                        (Development|PrintString "Overcharge ultimate")))))
                (elif (Actor|ActorHasTag (Components|GetOwner (Actor|GetComponentbyClass _array_element "/Game/_Project/CommonSystems/HealthSystem/HealthSystem.HealthSystem_C")) "Ally")
                  (Development|PrintString "Granade heal ally")
                  (Default|AddHealthType (Actor|GetComponentbyClass _array_element "/Game/_Project/CommonSystems/HealthSystem/HealthSystem.HealthSystem_C") "NewEnumerator0" 5e+01)
                  (Variables|/Game/_Project/CommonSystems/HealthSystem/HealthSystem.HealthSystem_C|SetOverHealOn (Actor|GetComponentbyClass _array_element "/Game/_Project/CommonSystems/HealthSystem/HealthSystem.HealthSystem_C") true)
                  (Utilities|IsValid (Variables|Default|GetOwningCharacter)
                    (:Is%20Valid
                      (Development|PrintString (Utilities|String|ToString(Float) (.currenthealth (Default|GetHealthData (Actor|GetComponentbyClass _array_element "/Game/_Project/CommonSystems/HealthSystem/HealthSystem.HealthSystem_C")))))
                      (if (Utilities|Enum|Equal(Enum) (Variables|/Game/_Project/CommonSystems/Character_Ultimate/Ultimate_BP.Ultimate_BP_C|GetState (Variables|/Game/_Project/Characters/BaseCharacter_BP.BaseCharacter_BP_C|GetUltimate (Variables|Default|GetOwningCharacter))) "NewEnumerator0")
                        (Default|AddCharge (Variables|/Game/_Project/Characters/BaseCharacter_BP.BaseCharacter_BP_C|GetUltimate (Variables|Default|GetOwningCharacter)) 2e+01)
                        (elif (>= (Variables|/Game/_Project/Characters/Ana/Ana_base_BP.Ana_base_BP_C|GetMaxOverCharge _asana_base_bp) (+ (Variables|/Game/_Project/Characters/Ana/Ana_base_BP.Ana_base_BP_C|GetOverCharge _asana_base_bp) 5.0))
                          (Variables|/Game/_Project/Characters/Ana/Ana_base_BP.Ana_base_BP_C|SetOverCharge _asana_base_bp (Variables|/Game/_Project/Characters/Ana/Ana_base_BP.Ana_base_BP_C|GetMaxOverCharge _asana_base_bp))
                          (Development|PrintString "Overcharge ultimate")
                          (else
                            (Variables|/Game/_Project/Characters/Ana/Ana_base_BP.Ana_base_BP_C|SetOverCharge (.AsAna%20Base%20BP (Utilities|Casting|CastToAna_base_BP (Variables|Default|GetOwningCharacter))) 5.0)
                            (Development|PrintString "Overcharge ultimate")))))))))))))
    (:then_1
      (Effects|SpawnEmitteratLocation "/Game/StarterContent/Particles/P_Explosion.P_Explosion" (Transformation|GetActorLocation) "0, 0, 0" "5.000000,5.000000,5.000000"))
    (:then_2
      (Actor|DestroyActor))))

(fn ConstructionScript)