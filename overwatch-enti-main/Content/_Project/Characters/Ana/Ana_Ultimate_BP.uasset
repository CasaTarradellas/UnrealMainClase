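; Ana's ultimate ability, which boosts the health of allies in a narrow cone in front of her when fired in the required state.
; Fire calls the parent, gathers nearby pawns with a sphere overlap, then filters them by a 2D forward dot product and the Ally tag.
; Each match, cast to Dummy, gets health through its HealthSystem; the ability then finishes and updates the ultimate UI using current charge plus Ana's OverCharge.
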(event EventFire
  (|CallParentFunction)
  (if (Utilities|Enum|Equal(Enum) "NewEnumerator2" (Variables|Default|GetState))
    (bind _outactors (Collision|SphereOverlapActors "0, 0, 0" 5e+02 (Utilities|Array|MakeArray "ObjectTypeQuery3") 0))
    (bind _output_get (Variables|Default|SetPotentialTarget _outactors))
    (for _array_element _output_get
      (if (Math|Float|InRange(Float) (Math|Vector|DotProduct (Class|KismetMathLibrary|VectorNormal2D (- (Transformation|GetActorLocation _array_element) (Transformation|GetActorLocation (Variables|Default|GetOwningCharacter))) 0.0001) (Transformation|GetActorForwardVector (Variables|Default|GetOwningCharacter))) 0.9 1.0)
        (if (Actor|ActorHasTag _array_element "Ally")
          (Default|AddHealthType (Variables|/Game/_Project/Characters/Dummy/Dummy.Dummy_C|GetHealthSystem (.AsDummy (Utilities|Casting|CastToDummy _array_element))) "NewEnumerator0" 5e+01)
          (Development|PrintString (Utilities|String|ToString(Float) (.currenthealth (Default|GetHealthData (Variables|/Game/_Project/Characters/Dummy/Dummy.Dummy_C|GetHealthSystem (.AsDummy (Utilities|Casting|CastToDummy _array_element)))))))
          (CallFunction|Finish)
          (Default|SetUltimateAmount (Variables|Default|GetUltimateUI) (+ (Variables|Default|GetCurrentCharge) (Variables|/Game/_Project/Characters/Ana/Ana_base_BP.Ana_base_BP_C|GetOverCharge (.AsAna%20Base%20BP (Utilities|Casting|CastToAna_base_BP (Variables|Default|GetOwningCharacter)))))))))))