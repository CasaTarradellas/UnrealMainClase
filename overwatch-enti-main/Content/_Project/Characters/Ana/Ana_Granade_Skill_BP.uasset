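; Ana's grenade skill Blueprint, which throws a grenade actor when fired.
; Fire calls the parent logic, then, in one specific skill state, spawns Ana_Granade_BP at the spawn position.
; The grenade component ignores the owning character when moving, the skill finishes, and the owner reference is passed to the spawned grenade.
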(event EventFire
  (|CallParentFunction)
  (if (Utilities|Enum|Equal(Enum) (Variables|Default|GetState) "NewEnumerator1")
    (bind _returnvalue (Game|SpawnActorfromClass "/Game/_Project/Characters/Ana/Ana_Granade_BP.Ana_Granade_BP_C" (Variables|Default|GetSpawnPos) "Undefined" "MultiplyWithRoot" 0 0))
    (Utilities|FlowControl|Sequence
      (:then_0
        (Collision|IgnoreActorwhenMoving (Variables|/Game/_Project/Characters/Ana/Ana_Granade_BP.Ana_Granade_BP_C|GetGranade _returnvalue) (Variables|Default|GetOwningCharacter) true)
        (CallFunction|Finish))
      (:then_1
        (Variables|/Game/_Project/Characters/Ana/Ana_Granade_BP.Ana_Granade_BP_C|SetOwningCharacter _returnvalue (Variables|Default|GetOwningCharacter))))))