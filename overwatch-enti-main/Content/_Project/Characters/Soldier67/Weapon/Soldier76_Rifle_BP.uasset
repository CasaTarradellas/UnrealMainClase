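; Soldier 76's hitscan rifle, a child weapon Blueprint adding firing, recoil and reload animation.
; Normal shots trace from the camera within a spread cone, damaging HealthSystem components, pushing physics bodies and charging the ultimate on hits.
; In one ultimate state (presumably active), Fire auto-aims at the character best aligned with the camera by dot product, grants no charge, and Reload switches to the short time.
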(event EventFire
  (bind _owningcharacter (Variables|Default|GetOwningCharacter))
  (bind _assoldier_76_bp (Utilities|Casting|CastToSoldier76_BP _owningcharacter))
  (bind _camera (Variables|/Game/_Project/Characters/BaseCharacter_BP.BaseCharacter_BP_C|GetCamera _assoldier_76_bp))
  (Utilities|FlowControl|Sequence
    (:then_0
      (if (not (Utilities|Enum|Equal(Enum) (Variables|/Game/_Project/CommonSystems/Character_Ultimate/Ultimate_BP.Ultimate_BP_C|GetState (Variables|/Game/_Project/Characters/BaseCharacter_BP.BaseCharacter_BP_C|GetUltimate (Variables|Default|GetOwningCharacter))) "NewEnumerator2"))
        (CallFunction|Shoot)
        (else
          (bind _outactors (Actor|GetAllActorsOfClass "/Script/Engine.Character"))
          (for _array_element _outactors
            (if (!= _array_element (Variables|Default|GetOwningCharacter))
              (if (> (Variables|Default|GetClosest) (Math|Vector|DotProduct (Math|Vector|GetForwardVector _camera) (Math|Vector|Normalize (- (Transformation|GetWorldLocation _camera) (Transformation|GetWorldLocation (Variables|/Script/Engine.Character|GetMesh _array_element))))))
                (Variables|Default|SetClosestCharacter _array_element)
                (Variables|Default|SetClosest (Math|Vector|DotProduct (Math|Vector|GetForwardVector _camera) (Math|Vector|Normalize (- (Transformation|GetWorldLocation _camera) (Transformation|GetWorldLocation (Variables|/Script/Engine.Character|GetMesh _array_element)))))))))
          (Utilities|IsValid (Variables|Default|GetClosestCharacter)
            (:Is%20Valid
              (bind (_outhit _returnvalue) (Collision|LineTraceByChannel (Transformation|GetWorldLocation (Variables|/Game/_Project/Characters/BaseCharacter_BP.BaseCharacter_BP_C|GetCamera (.AsSoldier%2076%20BP (Utilities|Casting|CastToSoldier76_BP (Variables|Default|GetOwningCharacter))))) (+ (Transformation|GetWorldLocation (Variables|/Script/Engine.Character|GetMesh (Variables|Default|GetClosestCharacter))) "0.000000,0.000000,125.000000") "TraceTypeQuery1" false 0 "ForDuration"))
              (if _returnvalue
                (Utilities|FlowControl|Sequence
                  (:then_0
                    (Utilities|IsValid (Actor|GetComponentbyClass (.HitActor (Collision|BreakHitResult _outhit)) "/Game/_Project/CommonSystems/HealthSystem/HealthSystem.HealthSystem_C")
                      (:Is%20Valid
                        (Default|TakeDamage (Actor|GetComponentbyClass (.HitActor (Collision|BreakHitResult _outhit)) "/Game/_Project/CommonSystems/HealthSystem/HealthSystem.HealthSystem_C") (== (.HitBoneName (Collision|BreakHitResult _outhit)) "Head") (Variables|Default|GetDamage)))))
                  (:then_1
                    (Utilities|IsValid (.HitComponent (Collision|BreakHitResult _outhit))
                      (:Is%20Valid
                        (if (Physics|IsSimulatingPhysics (.HitComponent (Collision|BreakHitResult _outhit)) "None")
                          (Physics|AddImpulseatLocation (.HitComponent (Collision|BreakHitResult _outhit)) "0, 0, 0" (.ImpactPoint (Collision|BreakHitResult _outhit)) "None"))))))))
            (:Is%20Not%20Valid
              (CallFunction|Shoot))))))
    (:then_1
      (|CallParentFunction))
    (:then_2
      (Default|Fire (Variables|Default|GetAnimator))
      (CallFunction|EnterFireCooldown))
    (:then_3
      (CallFunction|AddRecoil 0.1 (Math|Random|RandomFloatinRange -0.03 0.03)))))

(event EventInitialize
  (params (WeaponUI :type Weapon%20UI%20Object%20Reference) (OwningCharacter :type Base%20Character%20BP%20Object%20Reference))
  (|CallParentFunction WeaponUI OwningCharacter)
  (Variables|Default|SetAnimator (.AsRecruit%20Animation%20BP (Utilities|Casting|CastToRecruit_AnimationBP (Components|SkeletalMesh|GetAnimInstance (Variables|/Script/Engine.Character|GetMesh OwningCharacter))))))

(event EventReload
  (bind _owningcharacter (Variables|Default|GetOwningCharacter))
  (bind _ultimate (Variables|/Game/_Project/Characters/BaseCharacter_BP.BaseCharacter_BP_C|GetUltimate _owningcharacter))
  (bind _state (Variables|/Game/_Project/CommonSystems/Character_Ultimate/Ultimate_BP.Ultimate_BP_C|GetState _ultimate))
  (bind _returnvalue (Utilities|Enum|Equal(Enum) _state "NewEnumerator2"))
  (bind _returnvalue_2 (not _returnvalue))
  (Utilities|FlowControl|Sequence
    (:then_0
      (Variables|Default|SetReloadTime (Math|Float|SelectFloat (Variables|Default|GetLong%20Reload%20Time) (Variables|Default|GetShort%20Reload%20Time) _returnvalue_2))
      (Default|DoReload (Variables|Default|GetAnimator) _returnvalue_2))
    (:then_1
      (|CallParentFunction))))

(fn Shoot
  (bind _currentspread (Variables|Default|GetCurrentSpread))
  (bind _owningcharacter (Variables|Default|GetOwningCharacter))
  (bind _firedistance (Variables|Default|GetFireDistance))
  (bind _assoldier_76_bp (Utilities|Casting|CastToSoldier76_BP _owningcharacter))
  (bind _camera (Variables|/Game/_Project/Characters/BaseCharacter_BP.BaseCharacter_BP_C|GetCamera _assoldier_76_bp))
  (bind _returnvalue (Transformation|GetWorldLocation _camera))
  (bind _returnvalue_2 (Math|Vector|GetForwardVector _camera))
  (bind _returnvalue_3 (Math|Random|RandomUnitVectorinConeinDegrees _returnvalue_2 _currentspread))
  (bind _returnvalue_4 (* _returnvalue_3 _firedistance))
  (bind _returnvalue_5 (+ _returnvalue _returnvalue_4))
  (bind (_outhit _returnvalue_6) (Collision|LineTraceByChannel _returnvalue _returnvalue_5 "TraceTypeQuery1" false 0 "ForDuration"))
  (if _returnvalue_6
    (Utilities|FlowControl|Sequence
      (:then_0
        (Utilities|IsValid (Actor|GetComponentbyClass (.HitActor (Collision|BreakHitResult _outhit)) "/Game/_Project/CommonSystems/HealthSystem/HealthSystem.HealthSystem_C")
          (:Is%20Valid
            (Default|TakeDamage (Actor|GetComponentbyClass (.HitActor (Collision|BreakHitResult _outhit)) "/Game/_Project/CommonSystems/HealthSystem/HealthSystem.HealthSystem_C") (== (.HitBoneName (Collision|BreakHitResult _outhit)) "Head") (Variables|Default|GetDamage))
            (Default|AddCharge (Variables|/Game/_Project/Characters/BaseCharacter_BP.BaseCharacter_BP_C|GetUltimate (Variables|Default|GetOwningCharacter)) (Math|Float|SelectFloat (Variables|Default|GetUltimate%20Charge%20Per%20Headshot) (Variables|Default|GetUltimate%20Charge%20Per%20Hit) false)))))
      (:then_1
        (Utilities|IsValid (.HitComponent (Collision|BreakHitResult _outhit))
          (:Is%20Valid
            (if (Physics|IsSimulatingPhysics (.HitComponent (Collision|BreakHitResult _outhit)) "None")
              (Physics|AddImpulseatLocation (.HitComponent (Collision|BreakHitResult _outhit)) _returnvalue_5 (.ImpactPoint (Collision|BreakHitResult _outhit)) "None"))))))))