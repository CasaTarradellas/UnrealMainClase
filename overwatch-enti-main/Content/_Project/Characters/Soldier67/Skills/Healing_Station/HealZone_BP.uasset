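; HealZone_BP is the healing area of Soldier67's Healing Station skill, restoring health to whatever stands inside its capsule.
; Capsule overlap events add and remove the HealthSystem components of overlapping actors in the ActorsInside collection, with no team or owner filtering.
; Each Tick gives every tracked component Amount scaled by DeltaSeconds through AddHealthType, using a fixed health type, so healing is a per-second rate.
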(event OnComponentBeginOverlap(Capsule)
  (params (OverlappedComponent :type Primitive%20Component%20Object%20Reference) (OtherActor :type Actor%20Object%20Reference) (OtherComp :type Primitive%20Component%20Object%20Reference) (OtherBodyIndex :type Integer) (bFromSweep :type Boolean) (SweepResult :type Hit%20Result%20Structure%20%28by%20ref%29))
  (bind _returnvalue (Actor|GetComponentbyClass OtherActor "/Game/_Project/CommonSystems/HealthSystem/HealthSystem.HealthSystem_C"))
  (Utilities|IsValid _returnvalue
    (:Is%20Valid
      (Utilities|Set|Add (Variables|Default|GetActorsInside) _returnvalue))))

(event OnComponentEndOverlap(Capsule)
  (params (OverlappedComponent :type Primitive%20Component%20Object%20Reference) (OtherActor :type Actor%20Object%20Reference) (OtherComp :type Primitive%20Component%20Object%20Reference) (OtherBodyIndex :type Integer))
  (bind _returnvalue (Actor|GetComponentbyClass OtherActor "/Game/_Project/CommonSystems/HealthSystem/HealthSystem.HealthSystem_C"))
  (Utilities|IsValid _returnvalue
    (:Is%20Valid
      (Utilities|Set|Remove (Variables|Default|GetActorsInside) _returnvalue))))

(event EventTick
  (params (DeltaSeconds :type Float%20%28single-precision%29))
  (bind _result (Utilities|Set|ToArray (Variables|Default|GetActorsInside)))
  (for _array_element _result
    (Default|AddHealthType _array_element "NewEnumerator0" (* DeltaSeconds (Variables|Default|GetAmount)))))

(fn ConstructionScript)