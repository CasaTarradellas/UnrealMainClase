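; Soldier 76 hero character Blueprint that initializes health and three skill components: sprint, heal station and missile.
; Input actions drive each skill and the ultimate, registering skills with their key labels at BeginPlay.
; Holding sprint disables the other two skills until it is released.
; The heal station fires only when grounded, while it and the missile get spawn points from scene components before firing.
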(event Input|EnhancedActionEvents|EnhancedInputActionSkill_0
  (params (ActionValue :type Boolean) (ElapsedSeconds :type Float%20%28double-precision%29) (TriggeredSeconds :type Float%20%28double-precision%29) (InputAction :type Input%20Action%20Object%20Reference :default "/Game/_Project/CommonSystems/Input/Skill_0.Skill_0"))
  (bind _soldier_healstation_skill_bpc (Variables|Default|GetSoldier_HealStation_Skill_BPC))
  (bind _soldier_sprint_skill_bpc (Variables|Default|GetSoldier_Sprint_Skill_BPC))
  (bind _soldier_missile_skill_bpc (Variables|Default|GetSoldier_Missile_Skill_BPC))
  (:Triggered
    (Default|Fire _soldier_sprint_skill_bpc :!label _label)
    (Default|SetEnabled _soldier_healstation_skill_bpc false)
    (Default|SetEnabled _soldier_missile_skill_bpc false))
  (:Started
    (goto _label))
  (:Canceled
    (Default|Finish _soldier_sprint_skill_bpc :!label _label_2)
    (Default|SetEnabled _soldier_healstation_skill_bpc true)
    (Default|SetEnabled _soldier_missile_skill_bpc true))
  (:Completed
    (goto _label_2)))

(event Input|EnhancedActionEvents|EnhancedInputActionSkill_1
  (params (ActionValue :type Boolean) (ElapsedSeconds :type Float%20%28double-precision%29) (TriggeredSeconds :type Float%20%28double-precision%29) (InputAction :type Input%20Action%20Object%20Reference :default "/Game/_Project/CommonSystems/Input/Skill_1.Skill_1"))
  (bind _soldier_healstation_skill_bpc (Variables|Default|GetSoldier_HealStation_Skill_BPC))
  (if (not (AI|Components|NavMovement|IsFalling (Variables|Character|GetCharacterMovement)))
    (Variables|/Game/_Project/Characters/Soldier67/Skills/Healing_Station/Soldier_HealStation_Skill_BPC.Soldier_HealStation_Skill_BPC_C|SetSpawnPoint _soldier_healstation_skill_bpc (Math|Transform|MakeTransform (Transformation|GetWorldLocation (Variables|Default|GetHealthZone_Spawn))))
    (Default|Fire _soldier_healstation_skill_bpc)))

(event Input|EnhancedActionEvents|EnhancedInputActionSkill_2
  (params (ActionValue :type Boolean) (ElapsedSeconds :type Float%20%28double-precision%29) (TriggeredSeconds :type Float%20%28double-precision%29) (InputAction :type Input%20Action%20Object%20Reference :default "/Game/_Project/CommonSystems/Input/Skill_2.Skill_2"))
  (bind _soldier_missile_skill_bpc (Variables|Default|GetSoldier_Missile_Skill_BPC))
  (Variables|/Game/_Project/Characters/Soldier67/Skills/Missile/Soldier_Missile_Skill_BPC.Soldier_Missile_Skill_BPC_C|SetSpawnPoint _soldier_missile_skill_bpc (Transformation|GetWorldTransform (Variables|Default|GetMissile_Spawn)))
  (Default|Fire _soldier_missile_skill_bpc))

(event Input|EnhancedActionEvents|EnhancedInputActionUltimate
  (params (ActionValue :type Boolean) (ElapsedSeconds :type Float%20%28double-precision%29) (TriggeredSeconds :type Float%20%28double-precision%29) (InputAction :type Input%20Action%20Object%20Reference :default "/Game/_Project/CommonSystems/Input/Ultimate.Ultimate"))
  (Default|Fire (Variables|Default|GetUltimate)))

(event EventBeginPlay
  (bind _soldier_sprint_skill_bpc (Variables|Default|GetSoldier_Sprint_Skill_BPC))
  (bind _soldier_healstation_skill_bpc (Variables|Default|GetSoldier_HealStation_Skill_BPC))
  (bind _soldier_missile_skill_bpc (Variables|Default|GetSoldier_Missile_Skill_BPC))
  (|CallParentFunction)
  (Utilities|FlowControl|Sequence
    (:then_0
      (CallFunction|InitializeHealth (Utilities|Struct|MakeHealthData 5e+01 2.5e+02 0.0 0.0 0.0 0.0 0.0 false)))
    (:then_1
      (Default|Initialize _soldier_sprint_skill_bpc self "L SHIFT")
      (Utilities|Array|Add (Variables|Default|GetSkills) _soldier_sprint_skill_bpc))
    (:then_2
      (Default|Initialize _soldier_healstation_skill_bpc self "E")
      (Utilities|Array|Add (Variables|Default|GetSkills) _soldier_healstation_skill_bpc))
    (:then_3
      (Default|Initialize _soldier_missile_skill_bpc self "C")
      (Utilities|Array|Add (Variables|Default|GetSkills) _soldier_missile_skill_bpc))))

(fn ConstructionScript
  (|CallParentFunction))