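; Tracer's Pulse Bomb actor, an explosive that detonates on a timer started at BeginPlay.
; On explosion it destroys itself, spawns a scaled-up particle effect and sphere-overlaps Pawns within the explosion radius.
; Each overlapped Pawn with a HealthSystem component takes flat, non-headshot damage, with no owner or team filtering.
; A camera-forward launch impulse on the Sphere is present but disconnected, so it never runs.
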(event Custom|Explode
  (Actor|DestroyActor)
  (Effects|SpawnEmitteratLocation "/Game/_Project/StarterContent/Particles/P_Explosion.P_Explosion" (Transformation|GetActorLocation) "0, 0, 0" "5.000000,5.000000,5.000000")
  (bind (_outactors _returnvalue) (Collision|SphereOverlapActors (Transformation|GetActorLocation) (Variables|Default|GetExplosionRadius) (Utilities|Array|MakeArray "ObjectTypeQuery3") 0))
  (if _returnvalue
    (for _array_element _outactors
      (Utilities|IsValid (Actor|GetComponentbyClass _array_element "/Game/_Project/CommonSystems/HealthSystem/HealthSystem.HealthSystem_C")
        (:Is%20Valid
          (Default|TakeDamage (Actor|GetComponentbyClass _array_element "/Game/_Project/CommonSystems/HealthSystem/HealthSystem.HealthSystem_C") false (Variables|Default|GetDamage)))))))

(event EventBeginPlay
  (Utilities|Time|SetTimerbyEvent (delegate Custom|Explode) (Variables|Default|GetTimeToExplode)))

(fn ConstructionScript)