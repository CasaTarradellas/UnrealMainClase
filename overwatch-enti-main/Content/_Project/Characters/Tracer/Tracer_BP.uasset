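; Tracer hero character Blueprint that sets up health, armor and shield and wires input to her abilities.
; On BeginPlay it initializes Blink and Recall skill components with key labels and registers them in the Skills array.
; Skill inputs fire those components, while Ultimate passes a spawn point transform to the ultimate component before firing it.
; Tick polls the health system and reloads the current level when health runs out.
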(event Input|EnhancedActionEvents|EnhancedInputActionSkill_0
  (params (ActionValue :type Boolean) (ElapsedSeconds :type Float%20%28double-precision%29) (TriggeredSeconds :type Float%20%28double-precision%29) (InputAction :type Input%20Action%20Object%20Reference :default "/Game/_Project/CommonSystems/Input/Skill_0.Skill_0"))
  (Default|Fire (Variables|Default|GetTracer_Blink_Skill_BPC)))

(event Input|EnhancedActionEvents|EnhancedInputActionSkill_1
  (params (ActionValue :type Boolean) (ElapsedSeconds :type Float%20%28double-precision%29) (TriggeredSeconds :type Float%20%28double-precision%29) (InputAction :type Input%20Action%20Object%20Reference :default "/Game/_Project/CommonSystems/Input/Skill_1.Skill_1"))
  (Default|Fire (Variables|Default|GetTracer_Recall_Skill_BPC)))

(event Input|EnhancedActionEvents|EnhancedInputActionUltimate
  (params (ActionValue :type Boolean) (ElapsedSeconds :type Float%20%28double-precision%29) (TriggeredSeconds :type Float%20%28double-precision%29) (InputAction :type Input%20Action%20Object%20Reference :default "/Game/_Project/CommonSystems/Input/Ultimate.Ultimate"))
  (bind _ultimate (Variables|Default|GetUltimate))
  (Variables|/Game/_Project/Characters/Tracer/Tracer_Ultimate_BPC.Tracer_Ultimate_BPC_C|SetspawnPoint (.AsTracer%20Ultimate%20BPC (Utilities|Casting|CastToTracer_Ultimate_BPC _ultimate)) (Transformation|GetWorldTransform (Variables|Default|GetUltimateSpawnPoint)))
  (Default|Fire _ultimate))

(event EventBeginPlay
  (bind _tracer_blink_skill_bpc (Variables|Default|GetTracer_Blink_Skill_BPC))
  (bind _tracer_recall_skill_bpc (Variables|Default|GetTracer_Recall_Skill_BPC))
  (|CallParentFunction)
  (Utilities|FlowControl|Sequence
    (:then_0
      (CallFunction|InitializeHealth (Utilities|Struct|MakeHealthData 125.0 125.0 5e+01 5e+01 5e+01 5e+01 0.0 false)))
    (:then_1
      (Default|Initialize _tracer_blink_skill_bpc self "L SHIFT")
      (Utilities|Array|Add (Variables|Default|GetSkills) _tracer_blink_skill_bpc))
    (:then_2
      (Default|Initialize _tracer_recall_skill_bpc self "E")
      (Utilities|Array|Add (Variables|Default|GetSkills) _tracer_recall_skill_bpc))))

(event EventTick
  (params (DeltaSeconds :type Float%20%28single-precision%29))
  (|CallParentFunction DeltaSeconds)
  (if (<= (.currenthealth (Default|GetHealthData (Variables|Default|GetHealthSystem))) 0.0)
    (bind _returnvalue (Game|GetCurrentLevelName true))
    (Game|OpenLevel(byName) (Utilities|String|StringToName _returnvalue))))

(fn ConstructionScript
  (|CallParentFunction))