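; Soldier character Blueprint that sets up health, armor and shield values and registers two skill components: Cura and Sprint.
; Skill_3 fires Sprint on Started and on every Triggered, and disables Cura until the input completes or cancels, which finishes Sprint.
; Skill_4 passes the HealthSpawnPoint world transform to Cura as its spawn point, then fires it.
; The CuraSpawn function is an empty stub.
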(event Input|EnhancedActionEvents|EnhancedInputActionSkill_4
  (params (ActionValue :type Boolean) (ElapsedSeconds :type Float%20%28double-precision%29) (TriggeredSeconds :type Float%20%28double-precision%29) (InputAction :type Input%20Action%20Object%20Reference :default "/Game/_Project/CommonSystems/Input/Skill_4.Skill_4"))
  (bind _cura_soldier_bp_cool (Variables|Default|GetCura_Soldier_BP_Cool))
  (:Started
    (Variables|/Game/_Project/Characters/Soldier/Skills/Cura/Cura_Soldier_BP_Cool.Cura_Soldier_BP_Cool_C|SetSpawn%20Point _cura_soldier_bp_cool (Transformation|GetWorldTransform (Variables|Default|GetHealthSpawnPoint)))
    (Default|Fire _cura_soldier_bp_cool)))

(event Input|EnhancedActionEvents|EnhancedInputActionSkill_3
  (params (ActionValue :type Boolean) (ElapsedSeconds :type Float%20%28double-precision%29) (TriggeredSeconds :type Float%20%28double-precision%29) (InputAction :type Input%20Action%20Object%20Reference :default "/Game/_Project/CommonSystems/Input/Skill_3.Skill_3"))
  (bind _cura_soldier_bp_cool (Variables|Default|GetCura_Soldier_BP_Cool))
  (bind _soldier_sprint_skill_bpc (Variables|Default|GetSoldier_Sprint_Skill_BPC))
  (:Triggered
    (Default|Fire _soldier_sprint_skill_bpc :!label _label)
    (Default|SetEnabled _cura_soldier_bp_cool false))
  (:Started
    (goto _label))
  (:Canceled
    (Default|Finish _soldier_sprint_skill_bpc :!label _label_2)
    (Default|SetEnabled _cura_soldier_bp_cool true))
  (:Completed
    (goto _label_2)))

(event EventBeginPlay
  (bind _soldier_sprint_skill_bpc (Variables|Default|GetSoldier_Sprint_Skill_BPC))
  (bind _cura_soldier_bp_cool (Variables|Default|GetCura_Soldier_BP_Cool))
  (|CallParentFunction)
  (Utilities|FlowControl|Sequence
    (:then_0
      (CallFunction|InitializeHealth (Utilities|Struct|MakeHealthData 1e+02 2.5e+02 5e+01 5e+01 5e+01 5e+01 0.0 false)))
    (:then_1
      (Default|Initialize _cura_soldier_bp_cool self "E")
      (Utilities|Array|Add (Variables|Default|GetSkills) _cura_soldier_bp_cool))
    (:then_2
      (Default|Initialize _soldier_sprint_skill_bpc self "L SHIFT")
      (Utilities|Array|Add (Variables|Default|GetSkills) _soldier_sprint_skill_bpc))))

(event EventTick
  (params (DeltaSeconds :type Float%20%28single-precision%29))
  (|CallParentFunction DeltaSeconds))

(fn ConstructionScript
  (|CallParentFunction))

(fn CuraSpawn)