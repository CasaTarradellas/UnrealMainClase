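; Soldier skill Blueprint that launches a rocket when fired.
; It extends the parent Fire event and, if the skill is in the required state, spawns a rocket actor at SpawnPoint.
; The rocket's Sphere ignores the owning character during movement, then the skill calls Finish and passes the owner reference to the rocket.
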(event EventFire
  (|CallParentFunction)
  (if (Utilities|Enum|Equal(Enum) (Variables|Default|GetState) "NewEnumerator1")
    (bind _returnvalue (Game|SpawnActorfromClass "/Game/_Project/Characters/Soldier/Skills/RocketLaunch/RocketLaunch.RocketLaunch_C" (Variables|Default|GetSpawn%20Point) "Undefined" "MultiplyWithRoot" 0 0))
    (Utilities|FlowControl|Sequence
      (:then_0
        (Collision|IgnoreActorwhenMoving (Variables|/Game/_Project/Characters/Soldier/Skills/RocketLaunch/RocketLaunch.RocketLaunch_C|GetSphere _returnvalue) (Variables|Default|GetOwningCharacter) true)
        (CallFunction|Finish))
      (:then_1
        (Variables|/Game/_Project/Characters/Soldier/Skills/RocketLaunch/RocketLaunch.RocketLaunch_C|SetOwningCharacter _returnvalue (Variables|Default|GetOwningCharacter))))))