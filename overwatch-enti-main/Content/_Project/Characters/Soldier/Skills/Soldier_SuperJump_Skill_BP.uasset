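; Soldier super jump skill that launches the owning character straight up when fired.
; Fire calls the parent logic, then applies a vertical launch if the skill state matches and no jump is pending, flags the jump and calls Finish.
; Update clears the flag and calls Finish again once the character is no longer falling, allowing another jump.
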(event EventBeginPlay)

(event EventTick
  (params (DeltaSeconds :type Float%20%28single-precision%29)))

(event EventFire
  (|CallParentFunction)
  (if (and (Utilities|Enum|Equal(Enum) (Variables|Default|GetState) "NewEnumerator1") (not (Variables|Default|GethasJumped)))
    (Character|LaunchCharacter (Variables|Default|GetOwningCharacter) "0.000000,0.000000,1000.000000" false false)
    (Variables|Default|SethasJumped true)
    (CallFunction|Finish)))

(event EventUpdate
  (params (DeltaTime :type Float%20%28double-precision%29))
  (|CallParentFunction DeltaTime)
  (if (and (not (AI|Components|NavMovement|IsFalling (Variables|/Script/Engine.Character|GetCharacterMovement (Variables|Default|GetOwningCharacter)))) (Variables|Default|GethasJumped))
    (Variables|Default|SethasJumped false)
    (CallFunction|Finish)))