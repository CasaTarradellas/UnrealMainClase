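; Playable Symmetra hero character that sets up health and shield, registers Turret and Shield skill components, and fires them or the Ultimate from input actions.
; Capsule overlaps track whether a Portal_BP is in reach.
; While one is, the second skill input teleports instead of firing the shield.
; Teleport loops over all portals, moving the character slightly ahead of each one except the portal in reach, so the last one wins.
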(event OnComponentBeginOverlap(CapsuleComponent)
  (params (OverlappedComponent :type Primitive%20Component%20Object%20Reference) (OtherActor :type Actor%20Object%20Reference) (OtherComp :type Primitive%20Component%20Object%20Reference) (OtherBodyIndex :type Integer) (bFromSweep :type Boolean) (SweepResult :type Hit%20Result%20Structure%20%28by%20ref%29))
  (bind _asportal_bp (Utilities|Casting|CastToPortal_BP OtherActor))
  (Variables|Default|SetInUltimateReach true)
  (Variables|Default|SetPortalInReach _asportal_bp))

(event OnComponentEndOverlap(CapsuleComponent)
  (params (OverlappedComponent :type Primitive%20Component%20Object%20Reference) (OtherActor :type Actor%20Object%20Reference) (OtherComp :type Primitive%20Component%20Object%20Reference) (OtherBodyIndex :type Integer))
  (Utilities|Casting|CastToPortal_BP OtherActor)
  (Variables|Default|SetInUltimateReach false)
  (Variables|Default|SetPortalInReach 0))

(event Custom|Teleport
  (bind _outactors (Actor|GetAllActorsOfClass "/Game/_Project/Characters/Symmetra/Ultimate/Portal_BP.Portal_BP_C"))
  (for _array_element _outactors
    (if (!= _array_element (Variables|Default|GetPortalInReach))
      (Transformation|SetActorLocation (+ (Transformation|GetActorLocation _array_element) (* (Transformation|GetActorForwardVector) 1e+02)) false false))))

(event Input|EnhancedActionEvents|EnhancedInputActionSkill_1
  (params (ActionValue :type Boolean) (ElapsedSeconds :type Float%20%28double-precision%29) (TriggeredSeconds :type Float%20%28double-precision%29) (InputAction :type Input%20Action%20Object%20Reference :default "/Game/_Project/CommonSystems/Input/Skill_1.Skill_1"))
  (:Started
    (if (Variables|Default|GetInUltimateReach)
      (CallFunction|Teleport)
      (else
        (Default|Fire (Variables|Default|GetSymmetraShieldSkill_BPC))))))

(event Input|EnhancedActionEvents|EnhancedInputActionUltimate
  (params (ActionValue :type Boolean) (ElapsedSeconds :type Float%20%28double-precision%29) (TriggeredSeconds :type Float%20%28double-precision%29) (InputAction :type Input%20Action%20Object%20Reference :default "/Game/_Project/CommonSystems/Input/Ultimate.Ultimate"))
  (:Started
    (Default|Fire (Variables|Default|GetUltimate))))

(event Input|EnhancedActionEvents|EnhancedInputActionSkill_0
  (params (ActionValue :type Boolean) (ElapsedSeconds :type Float%20%28double-precision%29) (TriggeredSeconds :type Float%20%28double-precision%29) (InputAction :type Input%20Action%20Object%20Reference :default "/Game/_Project/CommonSystems/Input/Skill_0.Skill_0"))
  (:Started
    (Default|Fire (Variables|Default|GetTurretSkill_BPC))))

(event EventBeginPlay
  (bind _symmetrashieldskill_bpc (Variables|Default|GetSymmetraShieldSkill_BPC))
  (bind _turretskill_bpc (Variables|Default|GetTurretSkill_BPC))
  (|CallParentFunction)
  (Utilities|FlowControl|Sequence
    (:then_0
      (CallFunction|InitializeHealth (Utilities|Struct|MakeHealthData 1e+02 1e+02 0.0 0.0 1e+02 1e+02 0.0 false)))
    (:then_1
      (Default|Initialize _turretskill_bpc self "LEFT_SHIFT")
      (Utilities|Array|Add (Variables|Default|GetSkills) _turretskill_bpc))
    (:then_2
      (Default|Initialize _symmetrashieldskill_bpc self "E")
      (Utilities|Array|Add (Variables|Default|GetSkills) _symmetrashieldskill_bpc))))

(fn ConstructionScript
  (|CallParentFunction))