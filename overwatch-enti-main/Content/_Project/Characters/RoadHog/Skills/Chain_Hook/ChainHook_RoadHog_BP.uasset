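; Roadhog's Chain Hook skill, which throws a hook actor from the character's hook start point.
; Fire checks the skill state and a one-throw guard, then disables the first weapon and Take a Breather, shows the UI and halves walk speed.
; It spawns Hook_Roadhog_BP, passing the character and itself to it.
; Finish re-enables the weapon and skill, restores the saved speed and clears the guard.
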(event EventFire
  (bind _owningcharacter (Variables|Default|GetOwningCharacter))
  (bind _asroad_hog_bp (Utilities|Casting|CastToRoadHog_BP _owningcharacter))
  (bind _charactermovement (Variables|/Script/Engine.Character|GetCharacterMovement _asroad_hog_bp))
  (|CallParentFunction)
  (if (and (Utilities|Enum|Equal(Enum) (Variables|Default|GetState) "NewEnumerator1") (not (Variables|Default|GetalreadyThrown)))
    (Utilities|FlowControl|Sequence
      (:then_0
        (Default|SetDisabled (Utilities|Array|Get(acopy) (Variables|/Game/_Project/Characters/BaseCharacter_BP.BaseCharacter_BP_C|GetWeapons (Variables|Default|GetOwningCharacter))) true)
        (Default|SetActive (Variables|Default|GetUI) true)
        (Default|SetEnabled (Variables|/Game/_Project/Characters/RoadHog/RoadHog_BP.RoadHog_BP_C|GetTakeABreather_Roadhog_BP (.AsRoad%20Hog%20BP (Utilities|Casting|CastToRoadHog_BP (Variables|Default|GetOwningCharacter)))) false)
        (Variables|Default|SetOldSpeed (Variables|/Script/Engine.CharacterMovementComponent|GetMaxWalkSpeed _charactermovement))
        (Variables|/Script/Engine.CharacterMovementComponent|SetMaxWalkSpeed _charactermovement (/ (Variables|/Script/Engine.CharacterMovementComponent|GetMaxWalkSpeed _charactermovement) 2.0)))
      (:then_1
        (bind _returnvalue (Game|SpawnActorfromClass "/Game/_Project/Characters/RoadHog/Skills/Chain_Hook/Hook_Roadhog_BP.Hook_Roadhog_BP_C" (Transformation|GetWorldTransform (Variables|/Game/_Project/Characters/RoadHog/RoadHog_BP.RoadHog_BP_C|Gethook%20start/end (.AsRoad%20Hog%20BP (Utilities|Casting|CastToRoadHog_BP (Variables|Default|GetOwningCharacter))))) "AlwaysSpawn" "MultiplyWithRoot" 0 0))
        (Utilities|IsValid _returnvalue
          (:Is%20Valid
            (Utilities|FlowControl|Sequence
              (:then_0
                (Default|Initialize _returnvalue (.AsRoad%20Hog%20BP (Utilities|Casting|CastToRoadHog_BP (Variables|Default|GetOwningCharacter))) self))
              (:then_1
                (Variables|Default|SetalreadyThrown true)))))))))

(event EventFinish
  (|CallParentFunction)
  (Default|SetDisabled (Utilities|Array|Get(acopy) (Variables|/Game/_Project/Characters/BaseCharacter_BP.BaseCharacter_BP_C|GetWeapons (Variables|Default|GetOwningCharacter))) false)
  (Default|SetEnabled (Variables|/Game/_Project/Characters/RoadHog/RoadHog_BP.RoadHog_BP_C|GetTakeABreather_Roadhog_BP (.AsRoad%20Hog%20BP (Utilities|Casting|CastToRoadHog_BP (Variables|Default|GetOwningCharacter)))) true)
  (Variables|Default|SetalreadyThrown false)
  (Variables|/Script/Engine.CharacterMovementComponent|SetMaxWalkSpeed (Variables|/Script/Engine.Character|GetCharacterMovement (.AsRoad%20Hog%20BP (Utilities|Casting|CastToRoadHog_BP (Variables|Default|GetOwningCharacter)))) (Variables|Default|GetOldSpeed)))