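; Roadhog's Chain Hook projectile, which catches a character and drags it back to the owner, trailed by a cable.
; On overlap it stops, attaches to the victim and disables their movement and input.
; After a brief delay, Tick interpolates the victim to the owner's hook point, then re-enables only input and destroys the hook.
; A hook reaching max range without a hit self-destructs; destruction always calls Finish on the skill.
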(event OnComponentBeginOverlap(hook)
  (params (OverlappedComponent :type Primitive%20Component%20Object%20Reference) (OtherActor :type Actor%20Object%20Reference) (OtherComp :type Primitive%20Component%20Object%20Reference) (OtherBodyIndex :type Integer) (bFromSweep :type Boolean) (SweepResult :type Hit%20Result%20Structure%20%28by%20ref%29))
  (bind _hitactor (Collision|BreakHitResult SweepResult))
  (if (not (Variables|Default|GetalreadyHit))
    (Utilities|FlowControl|Sequence
      (:then_0
        (if (!= _hitactor (Variables|Default|GetowningCharacter))
          (bind _ascharacter (Utilities|Casting|CastToCharacter _hitactor))
          (Utilities|IsValid _ascharacter
            (:Is%20Valid
              (Pawn|Components|CharacterMovement|DisableMovement (Variables|/Script/Engine.Character|GetCharacterMovement _ascharacter))
              (Input|DisableInput _ascharacter 0)
              (bind _output_get (Variables|Default|SetcharacterHooked _ascharacter))
              (Components|Activation|Deactivate (Variables|Default|GetProjectileMovement))
              (Transformation|AttachActorToActor self _output_get "None" "SnapToTarget" "KeepRelative" "KeepRelative" true)))
          (else
            (Utilities|IsValid _hitactor
              (:Is%20Valid
                (Actor|DestroyActor))))))
      (:then_1
        (Variables|Default|SetalreadyHit true))
      (:then_2
        (Utilities|FlowControl|Delay 0.2)
        (Variables|Default|Setpull true)))))

(event Custom|Initialize
  (params (owningCharacter :type Road%20Hog%20BP%20Object%20Reference) (skillRef :type Chain%20Hook%20Road%20Hog%20BP%20Object%20Reference))
  (Utilities|FlowControl|Sequence
    (:then_0
      (bind _output_get (Variables|Default|SetowningCharacter owningCharacter))
      (Variables|Default|SetskillRef skillRef)
      (Variables|Default|SetStartLocation (.location (Transformation|GetActorTransform))))
    (:then_1
      (Class|CableComponent|SetAttachEndto (Variables|Default|GetCable) _output_get "None" "None"))))

(event EventTick
  (params (DeltaSeconds :type Float%20%28single-precision%29))
  (bind _cable (Variables|Default|GetCable))
  (|CallParentFunction DeltaSeconds)
  (Utilities|FlowControl|Sequence
    (:then_0
      (if (Variables|Default|GetalreadyHit)
        (if (Variables|Default|Getpull)
          (Transformation|SetActorLocation (Variables|Default|GetcharacterHooked) (Math|Interpolation|VInterpTo (Transformation|GetActorLocation (Variables|Default|GetcharacterHooked)) (Transformation|GetWorldLocation (Variables|/Game/_Project/Characters/RoadHog/RoadHog_BP.RoadHog_BP_C|Gethook%20start/end (Variables|Default|GetowningCharacter))) DeltaSeconds (Variables|Default|Getvel)) true false)
          (if (<= (Math|Vector|Distance(Vector) (Transformation|GetActorLocation (Variables|Default|GetcharacterHooked)) (Transformation|GetWorldLocation (Variables|/Game/_Project/Characters/RoadHog/RoadHog_BP.RoadHog_BP_C|Gethook%20start/end (Variables|Default|GetowningCharacter)))) 1e+01)
            (Input|EnableInput (Variables|Default|GetcharacterHooked) 0)
            (Actor|DestroyActor)))
        (elif (>= (Math|Vector|Distance(Vector) (Variables|Default|GetStartLocation) (.location (Transformation|GetActorTransform))) (Variables|Default|Getdistance))
          (Actor|DestroyActor))))
    (:then_1
      (Utilities|IsValid _cable
        (:Is%20Valid
          (Variables|/Script/CableComponent.CableComponent|SetCableLength _cable (Math|Vector|Distance(Vector) (Transformation|GetActorLocation) (Transformation|GetWorldLocation (Variables|/Game/_Project/Characters/RoadHog/RoadHog_BP.RoadHog_BP_C|Gethook%20start/end (Variables|Default|GetowningCharacter))))))))))

(event EventDestroyed
  (Default|Finish (Variables|Default|GetskillRef)))

(fn ConstructionScript)