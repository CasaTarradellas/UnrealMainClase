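; Roadhog's Take a Breather skill, a self-heal ability that heals its owner over time.
; Fire disables the first weapon and Chain Hook, halves walk speed, activates the UI and starts healing after a short delay.
; Update adds health scaled by delta time until the heal timer expires, then schedules Finish.
; Finish restores weapon, hook and speed, and resets the timer and re-press guard.
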(event EventFire
  (bind _owningcharacter (Variables|Default|GetOwningCharacter))
  (bind _asroad_hog_bp (Utilities|Casting|CastToRoadHog_BP _owningcharacter))
  (bind _charactermovement (Variables|/Script/Engine.Character|GetCharacterMovement _asroad_hog_bp))
  (|CallParentFunction)
  (if (and (Utilities|Enum|Equal(Enum) (Variables|Default|GetState) "NewEnumerator1") (not (Variables|Default|GetalreadyPressed)))
    (Utilities|FlowControl|Sequence
      (:then_0
        (Default|SetDisabled (Utilities|Array|Get(acopy) (Variables|/Game/_Project/Characters/BaseCharacter_BP.BaseCharacter_BP_C|GetWeapons (Variables|Default|GetOwningCharacter))) true)
        (Default|SetActive (Variables|Default|GetUI) true)
        (Default|SetEnabled (Variables|/Game/_Project/Characters/RoadHog/RoadHog_BP.RoadHog_BP_C|GetChainHook_RoadHog_BP (.AsRoad%20Hog%20BP (Utilities|Casting|CastToRoadHog_BP (Variables|Default|GetOwningCharacter)))) false)
        (bind _output_get (Variables|Default|SetOldSpeed (Variables|/Script/Engine.CharacterMovementComponent|GetMaxWalkSpeed _charactermovement)))
        (Variables|/Script/Engine.CharacterMovementComponent|SetMaxWalkSpeed _charactermovement (/ _output_get 2.0)))
      (:then_1
        (Variables|Default|SetalreadyPressed true))
      (:then_2
        (Utilities|FlowControl|Delay 0.5)
        (Variables|Default|Sethealing true)))))

(event EventFinish
  (|CallParentFunction)
  (Default|SetDisabled (Utilities|Array|Get(acopy) (Variables|/Game/_Project/Characters/BaseCharacter_BP.BaseCharacter_BP_C|GetWeapons (Variables|Default|GetOwningCharacter))) false)
  (Variables|Default|SethealTime 2.0)
  (Default|SetEnabled (Variables|/Game/_Project/Characters/RoadHog/RoadHog_BP.RoadHog_BP_C|GetChainHook_RoadHog_BP (.AsRoad%20Hog%20BP (Utilities|Casting|CastToRoadHog_BP (Variables|Default|GetOwningCharacter)))) true)
  (Variables|/Script/Engine.CharacterMovementComponent|SetMaxWalkSpeed (Variables|/Script/Engine.Character|GetCharacterMovement (.AsRoad%20Hog%20BP (Utilities|Casting|CastToRoadHog_BP (Variables|Default|GetOwningCharacter)))) (Variables|Default|GetOldSpeed))
  (Variables|Default|SetalreadyPressed false))

(event EventUpdate
  (params (DeltaTime :type Float%20%28double-precision%29))
  (|CallParentFunction DeltaTime)
  (if (Variables|Default|Gethealing)
    (Utilities|FlowControl|Sequence
      (:then_0
        (Default|AddHealthType (Variables|/Game/_Project/Characters/BaseCharacter_BP.BaseCharacter_BP_C|GetHealthSystem (Variables|Default|GetOwningCharacter)) "NewEnumerator0" (* (Variables|Default|GethealPerSecond) DeltaTime))
        (Variables|Default|SethealTime (- (Variables|Default|GethealTime) DeltaTime)))
      (:then_1
        (if (<= (Variables|Default|GethealTime) 0.0)
          (Variables|Default|Sethealing false)
          (Utilities|Time|SetTimerbyEvent (delegate EventFinish) 0.5))))))