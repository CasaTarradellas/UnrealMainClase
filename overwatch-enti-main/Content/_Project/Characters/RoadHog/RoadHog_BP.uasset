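; RoadHog_BP is the Roadhog character Blueprint, setting up health, two skills and secondary weapon fire.
; BeginPlay initializes health, then initializes Take a Breather and Chain Hook with owner and key labels and adds both to Skills.
; Enhanced Input actions fire each skill, or flag secondary fire and start or stop the current weapon.
; On death, it reloads the current level.
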(event OnDeath(HealthSystem)
  (bind _returnvalue (Game|GetCurrentLevelName true))
  (Game|OpenLevel(byName) (Utilities|String|StringToName _returnvalue)))

(event Input|EnhancedActionEvents|EnhancedInputActionSecondaryFire
  (params (ActionValue :type Boolean) (ElapsedSeconds :type Float%20%28double-precision%29) (TriggeredSeconds :type Float%20%28double-precision%29) (InputAction :type Input%20Action%20Object%20Reference :default "/Game/_Project/CommonSystems/Input/SecondaryFire.SecondaryFire"))
  (bind _weapons (Variables|Default|GetWeapons))
  (bind _currentweaponindex (Variables|Default|GetCurrentWeaponIndex))
  (bind _output (Utilities|Array|Get(acopy) _weapons _currentweaponindex))
  ;[0.15 0.15 0.15 0.5] Seconday Shoot of weapon
  (:Triggered
    (Variables|Default|SetisSecondaryFire true :!label _label)
    (Default|StartFireWeapon _output))
  (:Started
    (goto _label))
  (:Canceled
    (Variables|Default|SetisSecondaryFire false :!label _label_2)
    (Default|StopFireWeapon _output))
  (:Completed
    (goto _label_2)))

(event Input|EnhancedActionEvents|EnhancedInputActionSkill_1
  (params (ActionValue :type Boolean) (ElapsedSeconds :type Float%20%28double-precision%29) (TriggeredSeconds :type Float%20%28double-precision%29) (InputAction :type Input%20Action%20Object%20Reference :default "/Game/_Project/CommonSystems/Input/Skill_1.Skill_1"))
  (:Triggered
    (Default|Fire (Variables|Default|GetTakeABreather_Roadhog_BP) :!label _label))
  (:Started
    (goto _label)))

(event Input|EnhancedActionEvents|EnhancedInputActionSkill_0
  (params (ActionValue :type Boolean) (ElapsedSeconds :type Float%20%28double-precision%29) (TriggeredSeconds :type Float%20%28double-precision%29) (InputAction :type Input%20Action%20Object%20Reference :default "/Game/_Project/CommonSystems/Input/Skill_0.Skill_0"))
  (:Triggered
    (Default|Fire (Variables|Default|GetChainHook_RoadHog_BP) :!label _label))
  (:Started
    (goto _label)))

(event EventBeginPlay
  (bind _takeabreather_roadhog_bp (Variables|Default|GetTakeABreather_Roadhog_BP))
  (bind _chainhook_roadhog_bp (Variables|Default|GetChainHook_RoadHog_BP))
  (|CallParentFunction)
  (Utilities|FlowControl|Sequence
    (:then_0
      (CallFunction|InitializeHealth (Utilities|Struct|MakeHealthData 3e+02 6.5e+02 0.0 0.0 0.0 0.0 0.0 false)))
    (:then_1
      (Default|Initialize _takeabreather_roadhog_bp self "E")
      (Utilities|Array|Add (Variables|Default|GetSkills) _takeabreather_roadhog_bp))
    (:then_2
      (Default|Initialize _chainhook_roadhog_bp self "LEFT SHIFT")
      (Utilities|Array|Add (Variables|Default|GetSkills) _chainhook_roadhog_bp))))

(fn ConstructionScript
  (|CallParentFunction))