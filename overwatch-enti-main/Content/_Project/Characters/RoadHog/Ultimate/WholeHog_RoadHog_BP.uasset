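; Whole Hog ultimate for RoadHog, temporarily turning the Scrap Gun into a rapid-fire weapon with effectively unlimited ammo.
; Fire, gated by State and a one-cast flag, disables Take A Breather and Chain Hook and slows walking.
; After a brief delay, it saves and overrides gun stats, sets the WholeHog flag and clears charge.
; Chained timers restore the gun in Finishing, then speed and abilities in Finish.
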(event Custom|Finishing
  (bind _oldmaxamo (Variables|Default|GetoldMaxAmo))
  (bind _owningcharacter (Variables|Default|GetOwningCharacter))
  (bind _asroad_hog_bp (Utilities|Casting|CastToRoadHog_BP _owningcharacter))
  (bind _weapons (Variables|/Game/_Project/Characters/BaseCharacter_BP.BaseCharacter_BP_C|GetWeapons _asroad_hog_bp))
  (bind _output (Utilities|Array|Get(acopy) _weapons))
  (bind _asscrap_gun_roadhog_bp (Utilities|Casting|CastToScrapGun_Roadhog_BP _output))
  (Utilities|Time|SetTimerbyEvent (delegate EventFinish) 1.0)
  (Variables|/Game/_Project/Characters/RoadHog/Weapon/ScrapGun_Roadhog_BP.ScrapGun_Roadhog_BP_C|SetwholeHog _asscrap_gun_roadhog_bp false)
  (Variables|/Game/_Project/CommonSystems/Weapon/BaseWeapon.BaseWeapon_C|SetCurrentAmmo _asscrap_gun_roadhog_bp _oldmaxamo)
  (Variables|/Game/_Project/CommonSystems/Weapon/BaseWeapon.BaseWeapon_C|SetMaxAmmo _asscrap_gun_roadhog_bp _oldmaxamo)
  (Variables|/Game/_Project/CommonSystems/Weapon/BaseWeapon.BaseWeapon_C|SetFireCooldown _asscrap_gun_roadhog_bp (Variables|Default|GetoldFireRate)))

(event EventFinish
  (|CallParentFunction)
  (Variables|/Script/Engine.CharacterMovementComponent|SetMaxWalkSpeed (Variables|/Script/Engine.Character|GetCharacterMovement (.AsRoad%20Hog%20BP (Utilities|Casting|CastToRoadHog_BP (Variables|Default|GetOwningCharacter)))) (Variables|Default|GetOldSpeed))
  (Default|SetEnabled (Variables|/Game/_Project/Characters/RoadHog/RoadHog_BP.RoadHog_BP_C|GetTakeABreather_Roadhog_BP (.AsRoad%20Hog%20BP (Utilities|Casting|CastToRoadHog_BP (Variables|Default|GetOwningCharacter)))) true)
  (Default|SetEnabled (Variables|/Game/_Project/Characters/RoadHog/RoadHog_BP.RoadHog_BP_C|GetChainHook_RoadHog_BP (.AsRoad%20Hog%20BP (Utilities|Casting|CastToRoadHog_BP (Variables|Default|GetOwningCharacter)))) true))

(event EventFire
  (bind _owningcharacter (Variables|Default|GetOwningCharacter))
  (bind _owningcharacter_2 (Variables|Default|GetOwningCharacter))
  (bind _asroad_hog_bp (Utilities|Casting|CastToRoadHog_BP _owningcharacter_2))
  (bind _asroad_hog_bp_2 (Utilities|Casting|CastToRoadHog_BP _owningcharacter))
  (bind _weapons (Variables|/Game/_Project/Characters/BaseCharacter_BP.BaseCharacter_BP_C|GetWeapons _asroad_hog_bp))
  (bind _charactermovement (Variables|/Script/Engine.Character|GetCharacterMovement _asroad_hog_bp_2))
  (bind _output (Utilities|Array|Get(acopy) _weapons))
  (bind _asscrap_gun_roadhog_bp (Utilities|Casting|CastToScrapGun_Roadhog_BP _output))
  (|CallParentFunction)
  (if (and (Utilities|Enum|Equal(Enum) (Variables|Default|GetState) "NewEnumerator2") (not (Variables|Default|GetalreadyCast)))
    (Variables|Default|SetalreadyCast true)
    (Utilities|FlowControl|Sequence
      (:then_0
        (Default|SetEnabled (Variables|/Game/_Project/Characters/RoadHog/RoadHog_BP.RoadHog_BP_C|GetTakeABreather_Roadhog_BP (.AsRoad%20Hog%20BP (Utilities|Casting|CastToRoadHog_BP (Variables|Default|GetOwningCharacter)))) false)
        (Default|SetEnabled (Variables|/Game/_Project/Characters/RoadHog/RoadHog_BP.RoadHog_BP_C|GetChainHook_RoadHog_BP (.AsRoad%20Hog%20BP (Utilities|Casting|CastToRoadHog_BP (Variables|Default|GetOwningCharacter)))) false)
        (bind _output_get (Variables|Default|SetOldSpeed (Variables|/Script/Engine.CharacterMovementComponent|GetMaxWalkSpeed _charactermovement)))
        (Variables|/Script/Engine.CharacterMovementComponent|SetMaxWalkSpeed _charactermovement (/ _output_get 1.333333)))
      (:then_1
        (Utilities|FlowControl|Delay 0.5)
        (Variables|Default|SetoldFireRate (Variables|/Game/_Project/CommonSystems/Weapon/BaseWeapon.BaseWeapon_C|GetFireCooldown _asscrap_gun_roadhog_bp))
        (Variables|/Game/_Project/CommonSystems/Weapon/BaseWeapon.BaseWeapon_C|SetFireCooldown _asscrap_gun_roadhog_bp (Variables|Default|GetFireRate))
        (Variables|Default|SetoldMaxAmo (Variables|/Game/_Project/CommonSystems/Weapon/BaseWeapon.BaseWeapon_C|GetMaxAmmo _asscrap_gun_roadhog_bp))
        (Variables|/Game/_Project/CommonSystems/Weapon/BaseWeapon.BaseWeapon_C|SetCurrentAmmo _asscrap_gun_roadhog_bp 999999999)
        (Variables|/Game/_Project/CommonSystems/Weapon/BaseWeapon.BaseWeapon_C|SetMaxAmmo _asscrap_gun_roadhog_bp 999999999)
        (Variables|/Game/_Project/Characters/RoadHog/Weapon/ScrapGun_Roadhog_BP.ScrapGun_Roadhog_BP_C|SetwholeHog _asscrap_gun_roadhog_bp true)
        (Utilities|Time|SetTimerbyEvent (delegate Custom|Finishing) 7.5)
        (Variables|Default|SetCurrentCharge 0.0)))))