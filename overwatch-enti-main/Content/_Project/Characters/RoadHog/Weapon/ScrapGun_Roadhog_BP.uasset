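; Roadhog's Scrap Gun weapon, firing spread hitscan shots, a secondary-fire projectile, or Whole Hog blasts.
; Fire picks the mode from the WholeHog and secondary-fire flags, then runs parent logic, animation, cooldown and recoil.
; Shoot line-traces randomly spread pellets, applies distance-falloff damage with headshot detection, adds ultimate charge and returns unique hit characters.
; Whole Hog uses its own shot stats and launches those characters forward and up relative to the camera.
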(event EventFire
  (bind _owningcharacter (Variables|Default|GetOwningCharacter))
  (bind _owningcharacter_2 (Variables|Default|GetOwningCharacter))
  (bind _maxspread (Variables|Default|GetMaxSpread))
  (bind _owningcharacter_3 (Variables|Default|GetOwningCharacter))
  (bind _owningcharacter_4 (Variables|Default|GetOwningCharacter))
  (bind _camera (Variables|/Game/_Project/Characters/BaseCharacter_BP.BaseCharacter_BP_C|GetCamera _owningcharacter))
  (bind _camera_2 (Variables|/Game/_Project/Characters/BaseCharacter_BP.BaseCharacter_BP_C|GetCamera _owningcharacter_3))
  (bind _camera_3 (Variables|/Game/_Project/Characters/BaseCharacter_BP.BaseCharacter_BP_C|GetCamera _owningcharacter_4))
  (Utilities|FlowControl|Sequence
    (:then_0
      (if (Variables|Default|GetwholeHog)
        (if (not (Variables|/Game/_Project/Characters/RoadHog/RoadHog_BP.RoadHog_BP_C|GetisSecondaryFire (.AsRoad%20Hog%20BP (Utilities|Casting|CastToRoadHog_BP (Variables|Default|GetOwningCharacter)))))
          (bind _hitcharacters (CallFunction|Shoot (Variables|Default|GetwholeHogTotalBullets) (Variables|Default|GetwholeHogSpredX) (Variables|Default|GetwholeHogSpredY) (Variables|Default|GetwholeHogDamage) (Math|Vector|GetForwardVector _camera_3) (Transformation|GetWorldLocation _camera_3) 0.0))
          (for _array_element _hitcharacters
            (Character|LaunchCharacter _array_element (* (+ (Math|Vector|GetForwardVector _camera) (Math|Vector|GetUpVector _camera)) 5e+02) true true)))
        (elif (Variables|/Game/_Project/Characters/RoadHog/RoadHog_BP.RoadHog_BP_C|GetisSecondaryFire (.AsRoad%20Hog%20BP (Utilities|Casting|CastToRoadHog_BP (Variables|Default|GetOwningCharacter))))
          (bind _returnvalue (Game|SpawnActorfromClass "/Game/_Project/Characters/RoadHog/Weapon/RoadHog_Proyectile_BP.RoadHog_Proyectile_BP_C" (Transformation|GetWorldTransform (Variables|/Game/_Project/Characters/RoadHog/RoadHog_BP.RoadHog_BP_C|Getproyectile%20spawn (.AsRoad%20Hog%20BP (Utilities|Casting|CastToRoadHog_BP (Variables|Default|GetOwningCharacter))))) "Undefined" "MultiplyWithRoot" _owningcharacter_2 _owningcharacter_2))
          (Variables|/Game/_Project/Characters/RoadHog/Weapon/RoadHog_Proyectile_BP.RoadHog_Proyectile_BP_C|SetowningCharacter _returnvalue (.AsRoad%20Hog%20BP (Utilities|Casting|CastToRoadHog_BP (Variables|Default|GetOwningCharacter))))
          (Collision|IgnoreActorwhenMoving (Variables|/Game/_Project/Characters/RoadHog/Weapon/RoadHog_Proyectile_BP.RoadHog_Proyectile_BP_C|GetSphere _returnvalue) (Variables|Default|GetOwningCharacter) false)
          (else
            (CallFunction|Shoot (Variables|Default|GetTotalBullets) _maxspread _maxspread (Variables|Default|GetDamage) (Math|Vector|GetForwardVector _camera_2) (Transformation|GetWorldLocation _camera_2) (Variables|Default|GetUltimateChargePerHit))))))
    (:then_1
      (|CallParentFunction))
    (:then_2
      (Default|Fire (Variables|Default|GetAnimator))
      (CallFunction|EnterFireCooldown))
    (:then_3
      (CallFunction|AddRecoil 0.2 0.0))))

(event EventInitialize
  (params (WeaponUI :type Weapon%20UI%20Object%20Reference) (OwningCharacter :type Base%20Character%20BP%20Object%20Reference))
  (|CallParentFunction WeaponUI OwningCharacter)
  (Variables|Default|SetAnimator (.AsRecruit%20Animation%20BP (Utilities|Casting|CastToRecruit_AnimationBP (Components|SkeletalMesh|GetAnimInstance (Variables|/Script/Engine.Character|GetMesh OwningCharacter))))))

(event EventReload
  (Utilities|FlowControl|Sequence
    (:then_0
      (Variables|Default|SetReloadTime (Variables|Default|GetReloadTime))
      (Default|DoReload (Variables|Default|GetAnimator) false))
    (:then_1
      (|CallParentFunction))))

(fn Shoot
  (params (Bullets :type Integer) (spreadX :type Float%20%28double-precision%29) (spreadY :type Float%20%28double-precision%29) (Damage :type Float%20%28double-precision%29) (forward :type Vector) (Start%20Location :type Vector) (UltimateChargePerHit :type Float%20%28double-precision%29) (ActorsToIgnore :type Array%20of%20Actor%20Object%20References))
  (bind _alreadyhitcharacters (LocalVariables|GetalreadyHitCharacters))
  (Utilities|Array|Clear (LocalVariables|GetalreadyHitCharacters))
  (for _index (range 0 Bullets)
    (bind (_outhit _returnvalue) (Collision|LineTraceByChannel Start%20Location (+ Start%20Location (* (Math|Vector|RotateVector forward (Math|Rotator|MakeRotator 0.0 (Math|Random|RandomFloatinRange (* spreadY -1.0) spreadY) (Math|Random|RandomFloatinRange (* spreadX -1.0) spreadX))) (Variables|Default|GetFireDistance))) "TraceTypeQuery1" false ActorsToIgnore "ForDuration" true "(R=1.000000,G=0.000000,B=0.000000,A=1.000000)" "(R=0.000000,G=1.000000,B=0.000000,A=1.000000)" 0.5))
    (Utilities|FlowControl|Sequence
      (:then_0
        (if _returnvalue
          (Utilities|IsValid (Actor|GetComponentbyClass (.HitActor (Collision|BreakHitResult _outhit)) "/Game/_Project/CommonSystems/HealthSystem/HealthSystem.HealthSystem_C")
            (:Is%20Valid
              (Default|TakeDamage (Actor|GetComponentbyClass (.HitActor (Collision|BreakHitResult _outhit)) "/Game/_Project/CommonSystems/HealthSystem/HealthSystem.HealthSystem_C") (== (.HitBoneName (Collision|BreakHitResult _outhit)) "Head") (* Damage (Math|Float|Max(Float) (- 1.0 (/ (.Distance (Collision|BreakHitResult _outhit)) (Variables|Default|GetFireDistance))) 0.2)))
              (Default|AddCharge (Variables|/Game/_Project/Characters/BaseCharacter_BP.BaseCharacter_BP_C|GetUltimate (Variables|Default|GetOwningCharacter)) UltimateChargePerHit)
              (if (not (Utilities|Array|ContainsItem _alreadyhitcharacters (.AsCharacter (Utilities|Casting|CastToCharacter (.HitActor (Collision|BreakHitResult _outhit))))))
                (Utilities|Array|Add _alreadyhitcharacters (.AsCharacter (Utilities|Casting|CastToCharacter (.HitActor (Collision|BreakHitResult _outhit))))))))))
      (:then_1
        (Effects|SpawnEmitteratLocation "/Game/StarterContent/Particles/P_Explosion.P_Explosion" (.Location (Collision|BreakHitResult _outhit)) "0, 0, 0" "0.200000,0.200000,0.200000"))))
  (return (LocalVariables|GetalreadyHitCharacters)))