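; RoadHog weapon projectile that explodes on impact, or bursts into a shotgun-style pellet spread if destroyed before hitting anything.
; A sphere hit on anything but the owner destroys it, applying HealthSystem damage with headshot detection.
; Otherwise, Destroyed fires debug-drawn line traces in a random forward cone, with pellet damage falling off over distance to a minimum fraction.
; Both damage paths add charge to the owner's Ultimate.
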(event OnComponentHit(Sphere)
  (params (HitComponent :type Primitive%20Component%20Object%20Reference) (OtherActor :type Actor%20Object%20Reference) (OtherComp :type Primitive%20Component%20Object%20Reference) (NormalImpulse :type Vector :default "0, 0, 0") (Hit :type Hit%20Result%20Structure%20%28by%20ref%29))
  (bind (_bblockinghit _binitialoverlap _time _distance _location _impactpoint _normal _impactnormal _physmat _hitactor _hitcomponent _hitbonename) (Collision|BreakHitResult Hit))
  (Utilities|FlowControl|Sequence
    (:then_0
      (if (not (== _hitactor (Variables|Default|GetowningCharacter)))
        (Variables|Default|SethitSomething true)
        (Utilities|FlowControl|Sequence
          (:then_0
            (Utilities|IsValid _hitactor
              (:Is%20Valid
                (Default|TakeDamage (Actor|GetComponentbyClass _hitactor "/Game/_Project/CommonSystems/HealthSystem/HealthSystem.HealthSystem_C") (== _hitbonename "Head") (Variables|Default|GetdamageProyectile))
                (Default|AddCharge (Variables|/Game/_Project/Characters/BaseCharacter_BP.BaseCharacter_BP_C|GetUltimate (Variables|Default|GetowningCharacter)) (Variables|Default|GetUltimate%20Charge%20Per%20proyectile)))))
          (:then_1
            (Actor|DestroyActor)))))
    (:then_1
      (Effects|SpawnEmitteratLocation "/Game/_Project/StarterContent/Particles/P_Explosion.P_Explosion" _location "0, 0, 0" "0.500000,0.500000,0.500000"))))

(event EventDestroyed
  (bind _sphere (Variables|Default|GetSphere))
  (bind _returnvalue (Transformation|GetWorldLocation _sphere))
  (if (not (Variables|Default|GethitSomething))
    (for _index (range 0 (Variables|Default|GetTotalBullets))
      (bind (_outhit _returnvalue_2) (Collision|LineTraceByChannel _returnvalue (+ _returnvalue (* (Math|Random|RandomUnitVectorinConeinDegrees (Math|Vector|GetForwardVector _sphere) (Variables|Default|GetMaxSpread)) (Variables|Default|GetFireDistance))) "TraceTypeQuery1" false 0 "ForDuration" true "(R=1.000000,G=0.000000,B=0.000000,A=1.000000)" "(R=0.000000,G=1.000000,B=0.000000,A=1.000000)" 0.5))
      (Utilities|FlowControl|Sequence
        (:then_0
          (if _returnvalue_2
            (Utilities|IsValid (Actor|GetComponentbyClass (.HitActor (Collision|BreakHitResult _outhit)) "/Game/_Project/CommonSystems/HealthSystem/HealthSystem.HealthSystem_C")
              (:Is%20Valid
                (Default|TakeDamage (Actor|GetComponentbyClass (.HitActor (Collision|BreakHitResult _outhit)) "/Game/_Project/CommonSystems/HealthSystem/HealthSystem.HealthSystem_C") (== (.HitBoneName (Collision|BreakHitResult _outhit)) "Head") (* (Variables|Default|GetdamagePellet) (Math|Float|Max(Float) (- 1.0 (/ (.Distance (Collision|BreakHitResult _outhit)) (Variables|Default|GetFireDistance))) 0.2)))
                (Default|AddCharge (Variables|/Game/_Project/Characters/BaseCharacter_BP.BaseCharacter_BP_C|GetUltimate (Variables|Default|GetOwningCharacter)) (Variables|Default|GetUltimate%20Charge%20Per%20hit))))))
        (:then_1
          (Effects|SpawnEmitteratLocation "/Game/StarterContent/Particles/P_Explosion.P_Explosion" (.Location (Collision|BreakHitResult _outhit)) "0, 0, 0" "0.200000,0.200000,0.200000"))))))

(fn ConstructionScript)