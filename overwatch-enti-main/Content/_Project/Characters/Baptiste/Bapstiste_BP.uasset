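; Playable Baptiste hero character for an Overwatch-style game, with health, skills, an ultimate and a grounded high jump.
; Skill components handle Regenerating Field and Immortality Camp, spawning from character transforms; Camp disables Field until released.
; Secondary fire spawns one grenade at a time from a reloadable shot counter.
; Tick polls health; death disables input, hides the mesh and requests respawn from the GameMode.
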(event Custom|Die
  (bind _returnvalue (Pawn|GetController))
  (bind _asplayer_controller (Utilities|Casting|CastToPlayerController _returnvalue))
  (Input|DisableInput _asplayer_controller)
  (Components|Movement|StopMovementImmediately (Variables|Character|GetCharacterMovement))
  (Rendering|SetVisibility (Variables|Character|GetMesh) false false)
  (Default|RespawnPlayer (.AsOverwatch%20Game%20Mode (Utilities|Casting|CastToOverwatchGameMode (Game|GetGameMode))) self (Variables|Default|GetUI) _asplayer_controller))

(event Input|EnhancedActionEvents|EnhancedInputActionSkill_0
  (params (ActionValue :type Boolean) (ElapsedSeconds :type Float%20%28double-precision%29) (TriggeredSeconds :type Float%20%28double-precision%29) (InputAction :type Input%20Action%20Object%20Reference :default "/Game/_Project/CommonSystems/Input/Skill_0.Skill_0"))
  (bind _baptiste_inmortalcamp_skill_bpc (Variables|Default|GetBaptiste_InmortalCamp_Skill_BPC))
  (bind _baptiste_regeneratingfield_skill_bpc (Variables|Default|GetBaptiste_RegeneratingField_Skill_BPC))
  (:Triggered
    (Variables|/Game/_Project/Characters/Baptiste/Skills/InmortalCamp/Baptiste_InmortalCamp_Skill_BPC.Baptiste_InmortalCamp_Skill_BPC_C|SetSpawnPos _baptiste_inmortalcamp_skill_bpc (Transformation|GetWorldTransform (Variables|Default|GetArrow1)) :!label _label)
    (Default|Fire _baptiste_inmortalcamp_skill_bpc)
    (Default|SetEnabled _baptiste_regeneratingfield_skill_bpc false))
  (:Started
    (goto _label))
  (:Canceled
    (Default|Finish _baptiste_inmortalcamp_skill_bpc :!label _label_2)
    (Default|SetEnabled _baptiste_regeneratingfield_skill_bpc true))
  (:Completed
    (goto _label_2)))

(event Input|EnhancedActionEvents|EnhancedInputActionSkill_1
  (params (ActionValue :type Boolean) (ElapsedSeconds :type Float%20%28double-precision%29) (TriggeredSeconds :type Float%20%28double-precision%29) (InputAction :type Input%20Action%20Object%20Reference :default "/Game/_Project/CommonSystems/Input/Skill_1.Skill_1"))
  (bind _baptiste_regeneratingfield_skill_bpc (Variables|Default|GetBaptiste_RegeneratingField_Skill_BPC))
  (:Triggered
    (Variables|/Game/_Project/Characters/Baptiste/Skills/RegeneratingField/Baptiste_RegeneratingField_Skill_BPC.Baptiste_RegeneratingField_Skill_BPC_C|SetSpawnPosRege _baptiste_regeneratingfield_skill_bpc (Transformation|GetWorldTransform (Variables|Default|GetGenerateCaMPpOS)))
    (Default|Fire _baptiste_regeneratingfield_skill_bpc))
  (:Canceled
    (Default|Finish _baptiste_regeneratingfield_skill_bpc :!label _label))
  (:Completed
    (goto _label)))

(event Input|EnhancedActionEvents|EnhancedInputActionUltimate
  (params (ActionValue :type Boolean) (ElapsedSeconds :type Float%20%28double-precision%29) (TriggeredSeconds :type Float%20%28double-precision%29) (InputAction :type Input%20Action%20Object%20Reference :default "/Game/_Project/CommonSystems/Input/Ultimate.Ultimate"))
  (:Started
    (Default|Fire (Variables|Default|GetBaptiste_Ultimate))))

(event Input|EnhancedActionEvents|EnhancedInputActionSkill_4
  (params (ActionValue :type Boolean) (ElapsedSeconds :type Float%20%28double-precision%29) (TriggeredSeconds :type Float%20%28double-precision%29) (InputAction :type Input%20Action%20Object%20Reference :default "/Game/_Project/CommonSystems/Input/Skill_4.Skill_4"))
  (:Started
    (Development|PrintString "reload")
    (bind _output_get (Variables|Default|Setdisparos 10))
    (Development|PrintString "Disparos:")
    (Development|PrintString (Utilities|String|ToString(Integer) _output_get))))

(event Input|EnhancedActionEvents|EnhancedInputActionSecondaryFire
  (params (ActionValue :type Boolean) (ElapsedSeconds :type Float%20%28double-precision%29) (TriggeredSeconds :type Float%20%28double-precision%29) (InputAction :type Input%20Action%20Object%20Reference :default "/Game/_Project/CommonSystems/Input/SecondaryFire.SecondaryFire"))
  (:Started
    (if (> (Variables|Default|Getdisparos) 0)
      (Utilities|IsValid (Variables|Default|GetbaptisteGrenade)
        (:Is%20Not%20Valid
          (bind _returnvalue (Game|SpawnActorfromClass "/Game/_Project/Characters/Baptiste/Weapon/Baptiste_Grenade_BP.Baptiste_Grenade_BP_C" (Transformation|GetWorldTransform (Variables|Default|GetArrow1)) "Undefined" "MultiplyWithRoot" 0 0))
          (Variables|Default|SetbaptisteGrenade _returnvalue)
          (Variables|Default|Setdisparos (- (Variables|Default|Getdisparos) 1))
          (if (== (Variables|Default|Getdisparos) 0)
            (Development|PrintString "NO QUEDAN BALAS")))))))

(event Input|EnhancedActionEvents|EnhancedInputActionSkill_5
  (params (ActionValue :type Boolean) (ElapsedSeconds :type Float%20%28double-precision%29) (TriggeredSeconds :type Float%20%28double-precision%29) (InputAction :type Input%20Action%20Object%20Reference :default "/Game/_Project/CommonSystems/Input/Skill_5.Skill_5"))
  (:Triggered
    (if (not (AI|Components|NavMovement|IsFalling (Variables|Character|GetCharacterMovement)))
      (Character|LaunchCharacter "0.000000,0.000000,1000.000000" false false))))

(event EventBeginPlay
  (bind _baptiste_inmortalcamp_skill_bpc (Variables|Default|GetBaptiste_InmortalCamp_Skill_BPC))
  (bind _baptiste_regeneratingfield_skill_bpc (Variables|Default|GetBaptiste_RegeneratingField_Skill_BPC))
  (|CallParentFunction)
  (Utilities|FlowControl|Sequence
    (:then_0
      (CallFunction|InitializeHealth (Utilities|Struct|MakeHealthData 2.5e+02 2.5e+02 0.0 0.0 0.0 0.0 0.0 false)))
    (:then_1
      (Default|Initialize _baptiste_regeneratingfield_skill_bpc self "L SHIFT")
      (Utilities|Array|Add (Variables|Default|GetSkills) _baptiste_regeneratingfield_skill_bpc))
    (:then_2
      (Default|Initialize _baptiste_inmortalcamp_skill_bpc self "E")
      (Utilities|Array|Add (Variables|Default|GetSkills) _baptiste_inmortalcamp_skill_bpc))))

(event EventTick
  (params (DeltaSeconds :type Float%20%28single-precision%29))
  (|CallParentFunction DeltaSeconds)
  (if (<= (.currenthealth (Default|GetHealthData (Variables|Default|GetHealthSystem))) 0.0)
    (CallFunction|Die)))

(fn ConstructionScript
  (|CallParentFunction))