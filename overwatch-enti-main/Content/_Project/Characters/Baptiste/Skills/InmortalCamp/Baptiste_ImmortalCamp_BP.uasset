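; Baptiste's Immortality Field skill: a deployed, destructible device that keeps nearby actors from dying.
; One second after spawning it stops its projectile movement, animates its height on a timeline and starts a fast looping timer.
; The timer tops up HealthSystems tracked by sphere overlaps to a minimum health and sets them invulnerable, with no reset here.
; Tick prints the device's own health and destroys it when that equals LifeToDie.
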(event OnComponentEndOverlap(Sphere)
  (params (OverlappedComponent :type Primitive%20Component%20Object%20Reference) (OtherActor :type Actor%20Object%20Reference) (OtherComp :type Primitive%20Component%20Object%20Reference) (OtherBodyIndex :type Integer))
  (bind _returnvalue (Actor|GetComponentbyClass OtherActor "/Game/_Project/CommonSystems/HealthSystem/HealthSystem.HealthSystem_C"))
  (Utilities|IsValid _returnvalue
    (:Is%20Valid
      (Utilities|Set|Remove (Variables|Default|GetActorInside) _returnvalue))))

(event OnComponentBeginOverlap(Sphere)
  (params (OverlappedComponent :type Primitive%20Component%20Object%20Reference) (OtherActor :type Actor%20Object%20Reference) (OtherComp :type Primitive%20Component%20Object%20Reference) (OtherBodyIndex :type Integer) (bFromSweep :type Boolean) (SweepResult :type Hit%20Result%20Structure%20%28by%20ref%29))
  (bind _returnvalue (Actor|GetComponentbyClass OtherActor "/Game/_Project/CommonSystems/HealthSystem/HealthSystem.HealthSystem_C"))
  (Utilities|IsValid _returnvalue
    (:Is%20Valid
      (Utilities|Set|Add (Variables|Default|GetActorInside) _returnvalue))))

(event Custom|Inmortalty
  (bind _minunminmortallife (Variables|Default|GetminunmInmortalLife))
  (bind _result (Utilities|Set|ToArray (Variables|Default|GetActorInside)))
  (for _array_element _result
    (if (< (.currenthealth (Default|GetHealthData _array_element)) _minunminmortallife)
      (Default|SetInvulnerable _array_element true)
      (Default|AddHealthType _array_element "NewEnumerator0" (- _minunminmortallife (.currenthealth (Default|GetHealthData _array_element))))
      (Development|PrintString "mesHello"))))

(event Custom|Inmmortal
  (Utilities|Time|SetTimerbyEvent (delegate Custom|Inmortalty) 0.1 true))

(event EventTick
  (params (DeltaSeconds :type Float%20%28single-precision%29))
  (bind _healthsystem (Variables|Default|GetHealthSystem))
  (bind _healthdata (Default|GetHealthData _healthsystem))
  (Utilities|FlowControl|Sequence
    (:then_0
      (Development|PrintString "current Data DISCO")
      (Development|PrintString (Utilities|String|ToString(Float) (.currenthealth _healthdata))))
    (:then_1
      (if (== (.currenthealth _healthdata) (Variables|Default|GetlifeToDie))
        (Actor|DestroyActor)))))

(event EventBeginPlay
  (bind _returnvalue (Transformation|GetActorLocation))
  (Default|Initialize (Variables|Default|GetHealthSystem) (Utilities|Struct|MakeHealthData 1e+02 1e+02 0.0 0.0 0.0 0.0 0.0 false))
  (Utilities|FlowControl|Delay 1.0)
  (Utilities|FlowControl|Sequence
    (:then_0
      (Game|Components|ProjectileMovement|StopSimulating (Variables|Default|GetProjectileMovement) (Collision|MakeHitResult false false 0.0 0.0 "0, 0, 0" "0, 0, 0" "0,0,1" "0,0,1" 0 0)))
    (:then_1
      (bind _output_get (Variables|Default|SetcurrentPosZ (.z _returnvalue)))
      (bind _heihgt (Timeline|Timeline Play)
        (:Update
          (Transformation|SetActorLocation (Math|Vector|MakeVector (.x _returnvalue) (.y _returnvalue) (+ _output_get _heihgt)) false false))))
    (:then_2
      (CallFunction|Inmmortal))))

(fn ConstructionScript)