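; Baptiste's Regenerating Field skill actor, which periodically heals characters that enter its box.
; Box begin overlap adds the entering actor's HealthSystem component to the ActorInside set.
; A looping half-second timer started on BeginPlay adds health to every component in that set.
; No end-overlap handler removes entries; the Destroyed event only tries to remove the field's own HealthSystem.
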(event OnComponentBeginOverlap(Box)
  (params (OverlappedComponent :type Primitive%20Component%20Object%20Reference) (OtherActor :type Actor%20Object%20Reference) (OtherComp :type Primitive%20Component%20Object%20Reference) (OtherBodyIndex :type Integer) (bFromSweep :type Boolean) (SweepResult :type Hit%20Result%20Structure%20%28by%20ref%29))
  (bind _returnvalue (Actor|GetComponentbyClass OtherActor "/Game/_Project/CommonSystems/HealthSystem/HealthSystem.HealthSystem_C"))
  (Utilities|IsValid _returnvalue
    (:Is%20Valid
      (Utilities|Set|Add (Variables|Default|GetActorInside) _returnvalue))))

(event Custom|DealHealth
  (bind _result (Utilities|Set|ToArray (Variables|Default|GetActorInside)))
  (for _array_element _result
    (Utilities|IsValid (Variables|Default|GetHealthSystem)
      (:Is%20Valid
        (Default|AddHealthType _array_element "NewEnumerator0" (Variables|Default|GetHealth))))))

(event EventBeginPlay
  (Utilities|Time|SetTimerbyEvent (delegate Custom|DealHealth) 0.5 true))

(event EventDestroyed
  (bind _returnvalue (Actor|GetComponentbyClass "/Game/_Project/CommonSystems/HealthSystem/HealthSystem.HealthSystem_C"))
  (Utilities|IsValid _returnvalue
    (:Is%20Valid
      (Utilities|Set|Remove (Variables|Default|GetActorInside) _returnvalue))))

(fn ConstructionScript)