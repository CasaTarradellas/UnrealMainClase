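; Zenyatta's weapon Blueprint, extending a parent weapon with projectile firing and reloading, built on Recruit grenade and animation classes.
; Initialize caches the owner's Recruit animation Blueprint.
; Fire runs parent logic, spawns a grenade at the owner's transform, offset only along world X by the forward vector, then starts cooldown.
; Reload uses Zenyatta's reload time only on empty ammo, otherwise zero, and tells the animator before calling the parent.
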(event EventFire
  (bind _owningcharacter (Variables|Default|GetOwningCharacter))
  (bind _returnvalue (Transformation|GetActorTransform _owningcharacter))
  (bind (_location _rotation _scale) (Math|Transform|BreakTransform _returnvalue))
  (Utilities|FlowControl|Sequence
    (:then_0
      (|CallParentFunction)
      (Game|SpawnActorfromClass "/Game/_Project/Characters/Recruit/Skills/Grenade/Recruit_Grenade_BP.Recruit_Grenade_BP_C" (Math|Transform|MakeTransform (+ (* (Transformation|GetActorForwardVector _owningcharacter) "50.000000,0.000000,0.000000") _location) _rotation _scale) "AlwaysSpawn" "MultiplyWithRoot" 0 0)
      (CallFunction|EnterFireCooldown))))

(event EventInitialize
  (params (WeaponUI :type Weapon%20UI%20Object%20Reference) (OwningCharacter :type Base%20Character%20BP%20Object%20Reference))
  (|CallParentFunction WeaponUI OwningCharacter)
  (Variables|Default|SetAnimator (.AsRecruit%20Animation%20BP (Utilities|Casting|CastToRecruit_AnimationBP (Components|SkeletalMesh|GetAnimInstance (Variables|/Script/Engine.Character|GetMesh OwningCharacter))))))

(event EventReload
  (bind _currentammo (Variables|Default|GetCurrentAmmo))
  (bind _returnvalue (== _currentammo 0))
  (Utilities|FlowControl|Sequence
    (:then_0
      (Variables|Default|SetReloadTime (Math|Float|SelectFloat (Variables|Default|GetZenReloadTime) 0.0 _returnvalue))
      (Default|DoReload (Variables|Default|GetAnimator) _returnvalue))
    (:then_1
      (|CallParentFunction))))