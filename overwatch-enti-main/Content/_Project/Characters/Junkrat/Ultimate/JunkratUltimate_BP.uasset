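; Junkrat's ultimate ability, which spawns a separate UltimateCharacter_BP pawn and hands player control to it.
; Fire places the pawn at an offset from the owning character, passes it that owner, has player controller 0 possess it, then blocks refiring briefly with a delayed flag reset.
; Update drains charge over time in one specific state, calls Finish once it drops below zero, and feeds the amount to the ultimate UI.
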(event EventUpdate
  (params (DeltaTime :type Float%20%28double-precision%29))
  (if (Utilities|Enum|Equal(Enum) (Variables|Default|GetState) "NewEnumerator2")
    (bind _output_get (Variables|Default|SetCurrentCharge (- (Variables|Default|GetCurrentCharge) (* DeltaTime (Variables|Default|GetDischarge%20Rate)))))
    (if (< _output_get 0.0)
      (Variables|Default|SetCurrentCharge 0.0)
      (CallFunction|Finish))
    (Default|SetUltimateAmount (Variables|Default|GetUltimateUI) (Variables|Default|GetCurrentCharge))))

(event EventFire
  (bind _owningcharacter (Variables|Default|GetOwningCharacter))
  (bind _returnvalue (Transformation|GetActorTransform _owningcharacter))
  (if (not (Variables|Default|GetUltimateActive))
    (Variables|Default|SetUltimateActive true)
    (bind _returnvalue_2 (Game|SpawnActorfromClass "/Game/_Project/Characters/Junkrat/Ultimate/UltimateCharacter_BP.UltimateCharacter_BP_C" (Math|Transform|MakeTransform (+ (* (Transformation|GetActorForwardVector _owningcharacter) "200.000000,1.000000,1.000000") (.location _returnvalue)) (.rotation _returnvalue)) "AlwaysSpawn" "MultiplyWithRoot" 0 0))
    (Variables|/Game/_Project/Characters/Junkrat/Ultimate/UltimateCharacter_BP.UltimateCharacter_BP_C|SetOwningCharacterUlt _returnvalue_2 (Variables|Default|GetOwningCharacter))
    (Pawn|Possess (Game|GetPlayerController 0) _returnvalue_2)
    (Utilities|FlowControl|Delay 1.5)
    (Variables|Default|SetUltimateActive false)))