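; Junkrat's ultimate: a player-steered, self-propelled character that drives forward constantly and explodes after ten seconds or on either mouse click.
; Holding Space climbs surfaces by line-tracing ahead and switching between Flying and Falling movement.
; Detonation fires a radial impulse, calls TakeDamage with zero amount on overlapped pawns' HealthSystems, and spawns an explosion.
; It then hides, destroys itself after a delay and returns possession to the owning character.
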(event Input|EnhancedActionEvents|EnhancedInputActionLook
  (params (ActionValue :type Vector%202D%20Structure) (ElapsedSeconds :type Float%20%28double-precision%29) (TriggeredSeconds :type Float%20%28double-precision%29) (InputAction :type Input%20Action%20Object%20Reference :default "/Game/_Project/CommonSystems/Input/Look.Look"))
  (Pawn|Input|AddControllerYawInput (.x ActionValue)))

(event EventTick
  (params (DeltaSeconds :type Float%20%28single-precision%29))
  (|CallParentFunction DeltaSeconds)
  (Utilities|FlowControl|Sequence
    (:then_0
      (if (Variables|Default|GetSpacebarPressed)
        (bind _returnvalue (Collision|MultiLineTraceByChannel (Transformation|GetActorLocation) (+ (Transformation|GetActorLocation) (* (Transformation|GetActorForwardVector) 1e+02)) "TraceTypeQuery1" false 0 "ForOneFrame"))
        (if _returnvalue
          (Pawn|Components|CharacterMovement|SetMovementMode (Variables|Character|GetCharacterMovement) "MOVE_Flying" 0)
          (Pawn|Input|AddMovementInput "0.000000,0.000000,1.000000" 1.0 false)
          (else
            (Pawn|Components|CharacterMovement|SetMovementMode (Variables|Character|GetCharacterMovement) "MOVE_Falling" 0)))))
    (:then_1
      (Pawn|Input|AddMovementInput (Transformation|GetActorForwardVector) 1.0 false))))

(event EventBeginPlay
  (Utilities|FlowControl|Delay 1e+01)
  (Utilities|FlowControl|Sequence
    (:then_0
      (Class|RadialForceComponent|FireImpulse (Variables|Default|GetRadialForce)))
    (:then_1
      (CallFunction|CheckCollision))
    (:then_2
      (Effects|SpawnEmitteratLocation "/Game/StarterContent/Particles/P_Explosion.P_Explosion" (Transformation|GetActorLocation) "0, 0, 0" "5.000000,5.000000,5.000000"))
    (:then_3
      (Rendering|SetActorHiddenInGame true)
      (Pawn|Components|CharacterMovement|SetMovementMode (Variables|Character|GetCharacterMovement) "MOVE_None" 0)
      (Utilities|FlowControl|Delay 1.5)
      (Actor|DestroyActor)
      (Pawn|Possess (Game|GetPlayerController 0) (Variables|Default|GetOwningCharacterUlt)))))

(event Input|MouseEvents|LeftMouseButton
  (params (Key :type Key%20Structure :default "None"))
  (:Pressed
    (Utilities|FlowControl|Sequence
      (:then_0
        (Class|RadialForceComponent|FireImpulse (Variables|Default|GetRadialForce)))
      (:then_1
        (CallFunction|CheckCollision))
      (:then_2
        (Effects|SpawnEmitteratLocation "/Game/StarterContent/Particles/P_Explosion.P_Explosion" (Transformation|GetActorLocation) "0, 0, 0" "5.000000,5.000000,5.000000"))
      (:then_3
        (Rendering|SetActorHiddenInGame true)
        (Pawn|Components|CharacterMovement|SetMovementMode (Variables|Character|GetCharacterMovement) "MOVE_None" 0)
        (Utilities|FlowControl|Delay 1.5)
        (Actor|DestroyActor)
        (Pawn|Possess (Game|GetPlayerController 0) (Variables|Default|GetOwningCharacterUlt))))))

(event Input|MouseEvents|RightMouseButton
  (params (Key :type Key%20Structure :default "None"))
  (:Pressed
    (Utilities|FlowControl|Sequence
      (:then_0
        (Class|RadialForceComponent|FireImpulse (Variables|Default|GetRadialForce)))
      (:then_1
        (CallFunction|CheckCollision))
      (:then_2
        (Effects|SpawnEmitteratLocation "/Game/StarterContent/Particles/P_Explosion.P_Explosion" (Transformation|GetActorLocation) "0, 0, 0" "5.000000,5.000000,5.000000"))
      (:then_3
        (Rendering|SetActorHiddenInGame true)
        (Pawn|Components|CharacterMovement|SetMovementMode (Variables|Character|GetCharacterMovement) "MOVE_None" 0)
        (Utilities|FlowControl|Delay 1.5)
        (Actor|DestroyActor)
        (Pawn|Possess (Game|GetPlayerController 0) (Variables|Default|GetOwningCharacterUlt))))))

(event Input|KeyboardEvents|SpaceBar
  (params (Key :type Key%20Structure :default "None"))
  (:Pressed
    (Variables|Default|SetSpacebarPressed true))
  (:Released
    (Variables|Default|SetSpacebarPressed false)))

(fn ConstructionScript)

(fn CheckCollision
  (bind (_outactors _returnvalue) (Collision|SphereOverlapActors (Transformation|GetActorLocation) (Variables|/Script/Engine.RadialForceComponent|GetRadius (Variables|Default|GetRadialForce)) (Utilities|Array|MakeArray "ObjectTypeQuery3") 0))
  (if _returnvalue
    (for _array_element _outactors
      (Utilities|IsValid (Actor|GetComponentbyClass _array_element "/Game/_Project/CommonSystems/HealthSystem/HealthSystem.HealthSystem_C")
        (:Is%20Valid
          (Default|TakeDamage (Actor|GetComponentbyClass _array_element "/Game/_Project/CommonSystems/HealthSystem/HealthSystem.HealthSystem_C") false 0.0)
          (Utilities|IsValid 0))))))