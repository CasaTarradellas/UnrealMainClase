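; Junkrat's trap skill actor, which holds a victim in place for a few seconds and then destroys itself.
; When an actor with a HealthSystem component overlaps its box, a short downward trace must hit before the trap fires, and a flag limits it to one victim.
; It snaps the victim to its XY at a fixed world height, disables Character movement, then restores walking after the delay.
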(event OnComponentBeginOverlap(Box)
  (params (OverlappedComponent :type Primitive%20Component%20Object%20Reference) (OtherActor :type Actor%20Object%20Reference) (OtherComp :type Primitive%20Component%20Object%20Reference) (OtherBodyIndex :type Integer) (bFromSweep :type Boolean) (SweepResult :type Hit%20Result%20Structure%20%28by%20ref%29))
  (bind _returnvalue (Transformation|GetActorLocation))
  (Utilities|IsValid (Actor|GetComponentbyClass OtherActor "/Game/_Project/CommonSystems/HealthSystem/HealthSystem.HealthSystem_C")
    (:Is%20Valid
      (bind _returnvalue_2 (Collision|MultiLineTraceByChannel (Transformation|GetActorLocation) (- (Transformation|GetActorLocation) "0.000000,0.000000,25.000000") "TraceTypeQuery1" false 0 "None"))
      (if (and _returnvalue_2 (not (Variables|Default|GetTrappedSomeone)))
        (Transformation|SetActorLocation OtherActor (Math|Vector|MakeVector (.x _returnvalue) (.y _returnvalue) 1e+02) false false)
        (Variables|Default|SetTrappedSomeone true)
        (bind _ascharacter (Utilities|Casting|CastToCharacter OtherActor))
        (Pawn|Components|CharacterMovement|DisableMovement (Variables|/Script/Engine.Character|GetCharacterMovement _ascharacter))
        (Utilities|FlowControl|Delay 3.0)
        (Pawn|Components|CharacterMovement|SetMovementMode (Variables|/Script/Engine.Character|GetCharacterMovement _ascharacter) "MOVE_Walking" 0)
        (Variables|Default|SetTrappedSomeone false)
        (Actor|DestroyActor)))))

(fn ConstructionScript)