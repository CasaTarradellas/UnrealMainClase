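; Junkrat's trap skill, which places a trap at the owning character's location when fired.
; It extends the parent Fire logic and acts only in one specific skill state.
; Each use destroys the previously placed trap, spawns a new Trap_BP oriented to the character's roll and yaw, stores it, and finishes the skill, so the skill keeps one trap at a time.
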(event EventFire
  (bind _owningcharacter (Variables|Default|GetOwningCharacter))
  (bind _returnvalue (Transformation|GetActorRotation _owningcharacter))
  (|CallParentFunction)
  (if (Utilities|Enum|Equal(Enum) (Variables|Default|GetState) "NewEnumerator1")
    (Utilities|IsValid (Variables|Default|GetTrapRef)
      (:Is%20Valid
        (Actor|DestroyActor (Variables|Default|GetTrapRef)))
      (:Is%20Not%20Valid
        _))
    (bind _returnvalue_2 (Game|SpawnActorfromClass "/Game/_Project/Characters/Junkrat/Skills/TrapSkill/Trap_BP.Trap_BP_C" (Math|Transform|MakeTransform (Transformation|GetActorLocation _owningcharacter) (Math|Rotator|MakeRotator (.roll _returnvalue) (.pitch _returnvalue) (.yaw _returnvalue))) "Undefined" "MultiplyWithRoot" 0 0))
    (Transformation|SetActorRotation _returnvalue_2 (Math|Rotator|MakeRotator (.roll _returnvalue) 0.0 (.yaw _returnvalue)))
    (Variables|Default|SetTrapRef _returnvalue_2)
    (CallFunction|Finish)))