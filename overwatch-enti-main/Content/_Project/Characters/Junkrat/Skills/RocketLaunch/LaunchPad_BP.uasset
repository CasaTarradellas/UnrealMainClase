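; Launch pad actor for Junkrat's RocketLaunch skill that explodes to apply a radial impulse, then removes itself.
; Its Explode event fires the RadialForce component, then overlaps Pawns within the same radius and calls TakeDamage with zero damage on any HealthSystem found.
; It finishes by spawning an explosion particle effect and destroying the actor; nothing in this graph triggers Explode.
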(event Custom|Explode
  (Utilities|FlowControl|Sequence
    (:then_0
      (Class|RadialForceComponent|FireImpulse (Variables|Default|GetRadialForce)))
    (:then_1
      (bind (_outactors _returnvalue) (Collision|SphereOverlapActors (Transformation|GetActorLocation) (Variables|/Script/Engine.RadialForceComponent|GetRadius (Variables|Default|GetRadialForce)) (Utilities|Array|MakeArray "ObjectTypeQuery3") 0))
      (if _returnvalue
        (for _array_element _outactors
          (Utilities|IsValid (Actor|GetComponentbyClass _array_element "/Game/_Project/CommonSystems/HealthSystem/HealthSystem.HealthSystem_C")
            (:Is%20Valid
              (Default|TakeDamage (Actor|GetComponentbyClass _array_element "/Game/_Project/CommonSystems/HealthSystem/HealthSystem.HealthSystem_C") false 0.0)
              (Utilities|IsValid 0))))))
    (:then_2
      (Effects|SpawnEmitteratLocation "/Game/StarterContent/Particles/P_Explosion.P_Explosion" (Transformation|GetActorLocation)))
    (:then_3
      (Actor|DestroyActor))))

(fn ConstructionScript)