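; Junkrat's weapon Blueprint, extending a parent weapon class with projectile firing and reloading.
; Fire spawns a bullet actor at the character's arrow component, adds ultimate charge per shot and leaves the owner unignored by the bullet's movement collision.
; It then runs parent fire logic, animation, cooldown and vertical recoil.
; Reload picks a long or short time based on an empty magazine, passing that state to the cached animation Blueprint.
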(event EventFire
  (Utilities|FlowControl|Sequence
    (:then_0
      (bind _returnvalue (Game|SpawnActorfromClass "/Game/_Project/Characters/Junkrat/Weapon/JunkratBullet_BP.JunkratBullet_BP_C" (Transformation|GetWorldTransform (Variables|/Game/_Project/Characters/Junkrat/Junkrat_BP.Junkrat_BP_C|GetArrow1 (.AsJunkrat%20BP (Utilities|Casting|CastToJunkrat_BP (Variables|Default|GetOwningCharacter))))) "Undefined" "MultiplyWithRoot" 0 0))
      (Default|AddCharge (Variables|/Game/_Project/Characters/BaseCharacter_BP.BaseCharacter_BP_C|GetUltimate (Variables|Default|GetOwningCharacter)) 5e+01)
      (Collision|IgnoreActorwhenMoving (Variables|/Game/_Project/Characters/Junkrat/Weapon/JunkratBullet_BP.JunkratBullet_BP_C|GetSphere _returnvalue) (Variables|Default|GetOwningCharacter) false))
    (:then_1
      (|CallParentFunction))
    (:then_2
      (Default|Fire (Variables|Default|GetAnimator))
      (CallFunction|EnterFireCooldown))
    (:then_3
      (CallFunction|AddRecoil 0.2 0.0))))

(event EventInitialize
  (params (WeaponUI :type Weapon%20UI%20Object%20Reference) (OwningCharacter :type Base%20Character%20BP%20Object%20Reference))
  (|CallParentFunction WeaponUI OwningCharacter)
  (Variables|Default|SetAnimator (.AsRecruit%20Animation%20BP (Utilities|Casting|CastToRecruit_AnimationBP (Components|SkeletalMesh|GetAnimInstance (Variables|/Script/Engine.Character|GetMesh OwningCharacter))))))

(event EventReload
  (bind _currentammo (Variables|Default|GetCurrentAmmo))
  (bind _returnvalue (== _currentammo 0))
  (Utilities|FlowControl|Sequence
    (:then_0
      (Variables|Default|SetReloadTime (Math|Float|SelectFloat (Variables|Default|GetLong%20Reload%20Time) (Variables|Default|GetShort%20Reload%20Time) _returnvalue))
      (Default|DoReload (Variables|Default|GetAnimator) _returnvalue))
    (:then_1
      (|CallParentFunction))))