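; Junkrat's playable character Blueprint, extending a parent character with this hero's health and abilities.
; On BeginPlay it sets 250 health, then initializes the rocket launch and trap skill components with key labels and registers them in the Skills array.
; Input actions forward to those components: Skill_0 fires rocket launch, SecondaryFire detonates its launch pad, Skill_1 fires the trap, and Ultimate fires the ultimate.
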(event Input|EnhancedActionEvents|EnhancedInputActionSkill_0
  (params (ActionValue :type Boolean) (ElapsedSeconds :type Float%20%28double-precision%29) (TriggeredSeconds :type Float%20%28double-precision%29) (InputAction :type Input%20Action%20Object%20Reference :default "/Game/_Project/CommonSystems/Input/Skill_0.Skill_0"))
  (Default|Fire (Variables|Default|GetRocketLaunchSkill_Junkrat_BP)))

(event Input|EnhancedActionEvents|EnhancedInputActionSkill_1
  (params (ActionValue :type Boolean) (ElapsedSeconds :type Float%20%28double-precision%29) (TriggeredSeconds :type Float%20%28double-precision%29) (InputAction :type Input%20Action%20Object%20Reference :default "/Game/_Project/CommonSystems/Input/Skill_1.Skill_1"))
  (Default|Fire (Variables|Default|GetTrapSkill_Junkrat_BP)))

(event Input|EnhancedActionEvents|EnhancedInputActionSecondaryFire
  (params (ActionValue :type Boolean) (ElapsedSeconds :type Float%20%28double-precision%29) (TriggeredSeconds :type Float%20%28double-precision%29) (InputAction :type Input%20Action%20Object%20Reference :default "/Game/_Project/CommonSystems/Input/SecondaryFire.SecondaryFire"))
  (Default|EplodeLaunchPad (Variables|Default|GetRocketLaunchSkill_Junkrat_BP)))

(event Input|EnhancedActionEvents|EnhancedInputActionUltimate
  (params (ActionValue :type Boolean) (ElapsedSeconds :type Float%20%28double-precision%29) (TriggeredSeconds :type Float%20%28double-precision%29) (InputAction :type Input%20Action%20Object%20Reference :default "/Game/_Project/CommonSystems/Input/Ultimate.Ultimate"))
  (Default|Fire (Variables|Default|GetUltimate)))

(event EventBeginPlay
  (bind _rocketlaunchskill_junkrat_bp (Variables|Default|GetRocketLaunchSkill_Junkrat_BP))
  (bind _trapskill_junkrat_bp (Variables|Default|GetTrapSkill_Junkrat_BP))
  (|CallParentFunction)
  (Utilities|FlowControl|Sequence
    (:then_0
      (CallFunction|InitializeHealth (Utilities|Struct|MakeHealthData 2.5e+02 2.5e+02 0.0 0.0 0.0 0.0 0.0 false)))
    (:then_1
      (Default|Initialize _rocketlaunchskill_junkrat_bp self "L SHIFT")
      (Utilities|Array|Add (Variables|Default|GetSkills) _rocketlaunchskill_junkrat_bp))
    (:then_2
      (Default|Initialize _trapskill_junkrat_bp self "E")
      (Utilities|Array|Add (Variables|Default|GetSkills) _trapskill_junkrat_bp))))

(fn ConstructionScript
  (|CallParentFunction))