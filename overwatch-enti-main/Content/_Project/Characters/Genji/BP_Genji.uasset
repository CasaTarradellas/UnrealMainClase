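; Playable Genji hero character with health, shuriken alt-fire, dash, deflect, ultimate and wall climb.
; Registers dash and reflect skill components; dashing finishes an active reflect and enables a collider that damages characters, nearly clearing cooldown on kills.
; Timelines rotate meshes while swapping regular and ultimate weapons.
; Holding Jump climbs via forward line trace and Flying movement, limited by a timer reset on landing.
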(event OnComponentBeginOverlap(dashColider)
  (params (OverlappedComponent :type Primitive%20Component%20Object%20Reference) (OtherActor :type Actor%20Object%20Reference) (OtherComp :type Primitive%20Component%20Object%20Reference) (OtherBodyIndex :type Integer) (bFromSweep :type Boolean) (SweepResult :type Hit%20Result%20Structure%20%28by%20ref%29))
  (if (!= OtherActor self)
    (bind _ascharacter (Utilities|Casting|CastToCharacter OtherActor))
    (Utilities|IsValid (Actor|GetComponentbyClass _ascharacter "/Game/_Project/CommonSystems/HealthSystem/HealthSystem.HealthSystem_C")
      (:Is%20Valid
        (Default|TakeDamage (Actor|GetComponentbyClass _ascharacter "/Game/_Project/CommonSystems/HealthSystem/HealthSystem.HealthSystem_C") false 3e+02)
        (if (Variables|/Game/_Project/CommonSystems/HealthSystem/HealthSystem.HealthSystem_C|GetIsDead (Actor|GetComponentbyClass _ascharacter "/Game/_Project/CommonSystems/HealthSystem/HealthSystem.HealthSystem_C"))
          (Variables|/Game/_Project/CommonSystems/Character_Skills/Character_Cooldown_Skill_BP.Character_Cooldown_Skill_BP_C|SetCurrentCooldown (Variables|Default|GetDash_Skill_coldown) 0.1))))))

(event Custom|ChangeToUltimateWeapon
  (Default|Store (Utilities|Array|Get(acopy) (Variables|Default|GetWeapons)))
  (bind _rotationx (Timeline|Timeline PlayFromStart)
    (:Update
      (Transformation|SetRelativeRotation (Variables|Character|GetMesh) (Math|Rotator|MakeRotator _rotationx 0.0 -9e+01) false false)
      (Transformation|SetRelativeRotation (Variables|Default|GetUltimateMesh) (Math|Rotator|MakeRotator (+ -1.1 _rotationx) -1e+01 -9e+01) false false))
    (:ChangeWeapons
      (Rendering|SetVisibility (Variables|Character|GetMesh) false false)
      (Rendering|SetVisibility (Variables|Default|GetUltimateMesh) true false)
      (CallFunction|ChangeWeapon 1)
      (Default|Draw (Utilities|Array|Get(acopy) (Variables|Default|GetWeapons) 1)))))

(event Custom|ChangeToRegularWeapon
  (Default|Store (Utilities|Array|Get(acopy) (Variables|Default|GetWeapons) 1))
  (bind _rotationx (Timeline|Timeline_0 PlayFromStart)
    (:Update
      (Transformation|SetRelativeRotation (Variables|Character|GetMesh) (Math|Rotator|MakeRotator _rotationx 0.0 -9e+01) false false)
      (Transformation|SetRelativeRotation (Variables|Default|GetUltimateMesh) (Math|Rotator|MakeRotator (+ -1.1 _rotationx) -1e+01 -9e+01) false false))
    (:ChangeWeapons
      (Rendering|SetVisibility (Variables|Character|GetMesh) true false)
      (Rendering|SetVisibility (Variables|Default|GetUltimateMesh) false false)
      (CallFunction|ChangeWeapon)
      (Default|Draw (Utilities|Array|Get(acopy) (Variables|Default|GetWeapons))))))

(event Input|EnhancedActionEvents|EnhancedInputActionJump
  (params (ActionValue :type Boolean) (ElapsedSeconds :type Float%20%28double-precision%29) (TriggeredSeconds :type Float%20%28double-precision%29) (InputAction :type Input%20Action%20Object%20Reference :default "/Game/_Project/CommonSystems/Input/Jump.Jump"))
  (:Started
    (Character|Jump))
  (:Ongoing
    (bind _detec_wall (CallFunction|WallClime))
    (if _detec_wall
      (Pawn|Components|CharacterMovement|SetMovementMode (Variables|Character|GetCharacterMovement) "MOVE_Flying" 0)
      (Pawn|Input|AddMovementInput "0.000000,0.000000,0.500000" 1.0 false)
      (bind _output_get (Variables|Default|SetWallClimeTime (- (Variables|Default|GetWallClimeTime) (Utilities|Time|GetWorldDeltaSeconds))))
      (if (< _output_get 0.0)
        (Variables|Default|SetCanClime false)
        (Pawn|Components|CharacterMovement|SetMovementMode (Variables|Character|GetCharacterMovement) "MOVE_Falling" 0))
      (else
        (Pawn|Components|CharacterMovement|SetMovementMode (Variables|Character|GetCharacterMovement) "MOVE_Falling" 0))))
  (:Canceled
    (Character|StopJumping :!label _label)
    (Pawn|Components|CharacterMovement|SetMovementMode (Variables|Character|GetCharacterMovement) "MOVE_Falling" 0)
    (Variables|Default|SetCanClime false))
  (:Completed
    (goto _label)))

(event Input|EnhancedActionEvents|EnhancedInputActionSecondaryFire
  (params (ActionValue :type Boolean) (ElapsedSeconds :type Float%20%28double-precision%29) (TriggeredSeconds :type Float%20%28double-precision%29) (InputAction :type Input%20Action%20Object%20Reference :default "/Game/_Project/CommonSystems/Input/SecondaryFire.SecondaryFire"))
  (bind _weapons (Variables|Default|GetWeapons))
  (bind _currentweaponindex (Variables|Default|GetCurrentWeaponIndex))
  (bind _output (Utilities|Array|Get(acopy) _weapons _currentweaponindex))
  (:Triggered
    (bind _asshuriken_base_bp (Utilities|Casting|CastToShuriken_base_BP (Utilities|Array|Get(acopy) (Variables|Default|GetWeapons)) :!label _label))
    (Variables|/Game/_Project/Characters/Genji/Weapon/Shuriken_base_BP.Shuriken_base_BP_C|SetprimariFire _asshuriken_base_bp false)
    (Default|StartFireWeapon _output))
  (:Started
    (goto _label))
  (:Canceled
    (Default|StopFireWeapon _output :!label _label_2))
  (:Completed
    (goto _label_2)))

(event Input|EnhancedActionEvents|EnhancedInputActionUltimate
  (params (ActionValue :type Boolean) (ElapsedSeconds :type Float%20%28double-precision%29) (TriggeredSeconds :type Float%20%28double-precision%29) (InputAction :type Input%20Action%20Object%20Reference :default "/Game/_Project/CommonSystems/Input/Ultimate.Ultimate"))
  (:Started
    (Default|Fire (Variables|Default|GetUltimate))))

(event Input|EnhancedActionEvents|EnhancedInputActionSkill_0
  (params (ActionValue :type Boolean) (ElapsedSeconds :type Float%20%28double-precision%29) (TriggeredSeconds :type Float%20%28double-precision%29) (InputAction :type Input%20Action%20Object%20Reference :default "/Game/_Project/CommonSystems/Input/Skill_0.Skill_0"))
  (if (Utilities|Enum|Equal(Enum) (Variables|/Game/_Project/CommonSystems/Character_Skills/Character_Skill_BP.Character_Skill_BP_C|GetState (Variables|Default|GetReflect_Skill_BP)) "NewEnumerator1")
    (Default|Finish (Variables|Default|GetReflect_Skill_BP)))
  (Collision|SetCollisionEnabled (Variables|Default|GetdashColider) "QueryAndPhysics")
  (Default|Fire (Variables|Default|GetDash_Skill_coldown)))

(event Input|EnhancedActionEvents|EnhancedInputActionSkill_1
  (params (ActionValue :type Boolean) (ElapsedSeconds :type Float%20%28double-precision%29) (TriggeredSeconds :type Float%20%28double-precision%29) (InputAction :type Input%20Action%20Object%20Reference :default "/Game/_Project/CommonSystems/Input/Skill_1.Skill_1"))
  (bind _reflect_skill_bp (Variables|Default|GetReflect_Skill_BP))
  (Variables|/Game/_Project/Characters/Genji/Skils/Reflect/Reflect_Skill_BP.Reflect_Skill_BP_C|SetSpawnPoint _reflect_skill_bp (Transformation|GetWorldTransform (Variables|Default|GetDeflectSpawn)))
  (Default|Fire _reflect_skill_bp))

(event EventBeginPlay
  (bind _reflect_skill_bp (Variables|Default|GetReflect_Skill_BP))
  (bind _dash_skill_coldown (Variables|Default|GetDash_Skill_coldown))
  (bind _dashcolider (Variables|Default|GetdashColider))
  (|CallParentFunction)
  (Utilities|FlowControl|Sequence
    (:then_0
      (CallFunction|InitializeHealth (Utilities|Struct|MakeHealthData 2.5e+02 2.5e+02 0.0 0.0 0.0 0.0 0.0 false)))
    (:then_1
      (Default|Initialize _dash_skill_coldown self "leftShift")
      (Utilities|Array|Add (Variables|Default|GetSkills) _dash_skill_coldown)
      (Variables|/Game/_Project/Characters/Genji/Skils/Dash/Dash_Skill_coldown.Dash_Skill_coldown_C|Setdash%20collider _dash_skill_coldown _dashcolider)
      (Collision|SetCollisionEnabled _dashcolider "NoCollision"))
    (:then_2
      (Default|Initialize _reflect_skill_bp self "E")
      (Utilities|Array|Add (Variables|Default|GetSkills) _reflect_skill_bp))))

(event Collision|EventActorBeginOverlap
  (params (OtherActor :type Actor%20Object%20Reference)))

(event EventTick
  (params (DeltaSeconds :type Float%20%28single-precision%29))
  (|CallParentFunction DeltaSeconds) ; This node is disabled and will not be called.\nDrag off pins to build functionality.
)

(event EventOnLanded
  (params (Hit :type Hit%20Result%20Structure%20%28by%20ref%29))
  (Variables|Default|SetWallClimeTime (Variables|Default|GetMaxWallClimeTime))
  (Variables|Default|SetCanClime true))

(fn ConstructionScript
  (|CallParentFunction))

(fn WallClime
  (bind _returnvalue (Collision|LineTraceByChannel (Transformation|GetActorLocation) (+ (Transformation|GetActorLocation) (* (Transformation|GetActorForwardVector) 1e+02)) "TraceTypeQuery1" false 0 "ForOneFrame"))
  (return (and _returnvalue (Variables|Default|GetCanClime))))