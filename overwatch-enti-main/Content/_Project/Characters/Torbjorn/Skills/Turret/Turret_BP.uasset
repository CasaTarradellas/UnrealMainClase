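; Torbjorn's turret skill actor, a destructible turret whose deployment is signaled to its AI controller.
; Its health system starts at a fixed maximum, and Tick polls it to destroy the turret at zero health.
; Any hit starts a short delay before calling Deployed on Turret_AIController, as the Character cast gates nothing.
; A sphere's overlap events maintain the DummiesInRange list of Dummy actors.
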(event OnComponentBeginOverlap(Sphere)
  (params (OverlappedComponent :type Primitive%20Component%20Object%20Reference) (OtherActor :type Actor%20Object%20Reference) (OtherComp :type Primitive%20Component%20Object%20Reference) (OtherBodyIndex :type Integer) (bFromSweep :type Boolean) (SweepResult :type Hit%20Result%20Structure%20%28by%20ref%29))
  (bind _asdummy (Utilities|Casting|CastToDummy OtherActor))
  (Utilities|Set|Add (Variables|Default|GetDummiesInRange) _asdummy))

(event OnComponentEndOverlap(Sphere)
  (params (OverlappedComponent :type Primitive%20Component%20Object%20Reference) (OtherActor :type Actor%20Object%20Reference) (OtherComp :type Primitive%20Component%20Object%20Reference) (OtherBodyIndex :type Integer))
  (bind _asdummy (Utilities|Casting|CastToDummy OtherActor))
  (Utilities|Set|Remove (Variables|Default|GetDummiesInRange) _asdummy))

(event EventBeginPlay
  (Utilities|FlowControl|Sequence
    (:then_0
      (Default|Initialize (Variables|Default|GetHealthSystem) (Utilities|Struct|MakeHealthData 2.5e+02 2.5e+02 0.0 0.0 0.0 0.0 0.0 false)))
    (:then_1
      (|CallParentFunction))))

(event EventTick
  (params (DeltaSeconds :type Float%20%28single-precision%29))
  (if (<= (.currenthealth (Default|GetHealthData (Variables|Default|GetHealthSystem))) 0.0)
    (Actor|DestroyActor self)))

(event Collision|EventHit
  (params (MyComp :type Primitive%20Component%20Object%20Reference) (Other :type Actor%20Object%20Reference) (OtherComp :type Primitive%20Component%20Object%20Reference) (bSelfMoved :type Boolean) (HitLocation :type Vector :default "0, 0, 0") (HitNormal :type Vector :default "0, 0, 0") (NormalImpulse :type Vector :default "0, 0, 0") (Hit :type Hit%20Result%20Structure%20%28by%20ref%29))
  (Utilities|FlowControl|Sequence
    (:then_0
      (Utilities|Casting|CastToCharacter Other))
    (:then_1
      (Utilities|FlowControl|Delay 3.0)
      (Default|Deployed (.AsTurret%20AIController (Utilities|Casting|CastToTurret_AIController (Pawn|GetController)))))))

(fn ConstructionScript)