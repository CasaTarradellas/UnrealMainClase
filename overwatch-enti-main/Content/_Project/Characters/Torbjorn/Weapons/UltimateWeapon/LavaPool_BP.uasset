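; Lava pool actor for Torbjorn's ultimate weapon that deals periodic damage to Dummy actors inside it and destroys itself after a fixed lifetime.
; Begin and end overlap events add and remove Dummies from a unique target list.
; A looping timer started on BeginPlay damages each listed target through its HealthSystem as a non-headshot hit, printing a debug string per hit.
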(event Custom|DamagePerTick
  (for _array_element (Variables|Default|GetLavaObjectives)
    (Default|TakeDamage (Variables|/Game/_Project/Characters/Dummy/Dummy.Dummy_C|GetHealthSystem _array_element) false 5e+01)
    (Development|PrintString "Lava damage")))

(event Collision|EventActorBeginOverlap
  (params (OtherActor :type Actor%20Object%20Reference))
  (bind _asdummy (Utilities|Casting|CastToDummy OtherActor))
  (Utilities|IsValid _asdummy
    (:Is%20Valid
      (Utilities|Array|AddUnique (Variables|Default|GetLavaObjectives) _asdummy))))

(event Collision|EventActorEndOverlap
  (params (OtherActor :type Actor%20Object%20Reference))
  (bind _asdummy (Utilities|Casting|CastToDummy OtherActor))
  ;[0.15 0.15 0.15 0.5] acabar esto
  (Utilities|IsValid _asdummy
    (:Is%20Valid
      (Utilities|Array|RemoveItem (Variables|Default|GetLavaObjectives) _asdummy))))

(event EventBeginPlay
  (Utilities|FlowControl|Sequence
    (:then_0
      (Utilities|FlowControl|Delay 1e+01)
      (Actor|DestroyActor))
    (:then_1
      (Utilities|Time|SetTimerbyEvent (delegate Custom|DamagePerTick) 0.2 true true))))

(fn ConstructionScript)