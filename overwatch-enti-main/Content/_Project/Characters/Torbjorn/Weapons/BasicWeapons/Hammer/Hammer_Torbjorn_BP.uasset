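; Torbjorn's hammer weapon, a melee attack that heals turrets and damages other actors with a health component.
; Fire runs the parent logic, enters cooldown, then does a box trace at a single point ahead of the owner's camera, with debug drawing on.
; Each hit Turret_BP regains health through its HealthSystem and prints the new value, while any other actor with a HealthSystem takes damage.
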(event EventInitialize
  (params (WeaponUI :type Weapon%20UI%20Object%20Reference) (OwningCharacter :type Base%20Character%20BP%20Object%20Reference))
  (|CallParentFunction WeaponUI OwningCharacter))

(event EventFire
  (params (AmmoUsage :type Integer))
  (bind _owningcharacter (Variables|Default|GetOwningCharacter))
  (bind _firedistance (Variables|Default|GetFireDistance))
  (bind _camera (Variables|/Game/_Project/Characters/BaseCharacter_BP.BaseCharacter_BP_C|GetCamera _owningcharacter))
  (bind _returnvalue (Transformation|GetWorldLocation _camera))
  (bind _returnvalue_2 (Math|Vector|GetForwardVector _camera))
  (bind _returnvalue_3 (* _returnvalue_2 _firedistance))
  (bind _returnvalue_4 (+ _returnvalue _returnvalue_3))
  (|CallParentFunction 0)
  (Utilities|FlowControl|Sequence
    (:then_0
      (CallFunction|EnterFireCooldown))
    (:then_1
      ;[0.15 0.15 0.15 0.5] aqui hay que modificar esto para comprobar si es una torreta o no, en caso de que lo sea, tiene que hacerle recuperar salud (50 puntos exactamente)
      (bind _outhits (Class|KismetSystemLibrary|BoxTraceMulti _returnvalue_4 _returnvalue_4 "20.000000,20.000000,20.000000" (Transformation|GetWorldRotation _camera) "TraceTypeQuery1" false (Utilities|Array|MakeArray (Variables|Default|GetOwningCharacter)) "ForDuration" true))
      (for _array_element _outhits
        (Utilities|IsValid (.HitActor (Collision|BreakHitResult _array_element))
          (:Is%20Valid
            (Utilities|IsValid (Actor|GetComponentbyClass (.HitActor (Collision|BreakHitResult _array_element)) "/Game/_Project/CommonSystems/HealthSystem/HealthSystem.HealthSystem_C")
              (:Is%20Valid
                (Utilities|IsValid (.AsTurret%20BP (Utilities|Casting|CastToTurret_BP (.HitActor (Collision|BreakHitResult _array_element))))
                  (:Is%20Valid
                    (Default|AddHealthType (Variables|/Game/_Project/Characters/Torbjorn/Skills/Turret/Turret_BP.Turret_BP_C|GetHealthSystem (.AsTurret%20BP (Utilities|Casting|CastToTurret_BP (.HitActor (Collision|BreakHitResult _array_element))))) "NewEnumerator0" 4e+01)
                    (Development|PrintString (Utilities|String|ToString(Float) (.currenthealth (Default|GetHealthData (Variables|/Game/_Project/Characters/Torbjorn/Skills/Turret/Turret_BP.Turret_BP_C|GetHealthSystem (.AsTurret%20BP (Utilities|Casting|CastToTurret_BP (.HitActor (Collision|BreakHitResult _array_element))))))))))
                  (:Is%20Not%20Valid
                    (Default|TakeDamage (Actor|GetComponentbyClass (.HitActor (Collision|BreakHitResult _array_element)) "/Game/_Project/CommonSystems/HealthSystem/HealthSystem.HealthSystem_C") false 4e+01)))))))))))