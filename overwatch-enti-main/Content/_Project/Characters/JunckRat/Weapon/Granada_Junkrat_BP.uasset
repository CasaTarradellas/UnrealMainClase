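; Junkrat's grenade projectile, which bounces and explodes on a damageable target or on its third bounce.
; The projectile movement's bounce event counts bounces, then spawns the explosion particle and destroys the actor at the limit.
; Overlapping an actor with a HealthSystem component applies non-headshot damage through that component, then triggers the same effect and destruction.
; The bounce-limit explosion is visual only and deals no damage.
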(event OnProjectileBounce(ProjectileMovement)
  (params (ImpactResult :type Hit%20Result%20Structure%20%28by%20ref%29) (ImpactVelocity :type Vector%20%28by%20ref%29 :default "0, 0, 0"))
  (bind _result (Math|Integer|IncrementInt (Variables|Default|GetReboteCount))
    (:%20%20
      (if (>= _result 3)
        (Effects|SpawnEmitteratLocation "/Game/StarterContent/Particles/P_Explosion.P_Explosion" (Transformation|GetActorLocation))
        (Actor|DestroyActor)))))

(event OnComponentBeginOverlap(Sphere1)
  (params (OverlappedComponent :type Primitive%20Component%20Object%20Reference) (OtherActor :type Actor%20Object%20Reference) (OtherComp :type Primitive%20Component%20Object%20Reference) (OtherBodyIndex :type Integer) (bFromSweep :type Boolean) (SweepResult :type Hit%20Result%20Structure%20%28by%20ref%29))
  (bind _returnvalue (Actor|GetComponentbyClass OtherActor "/Game/_Project/CommonSystems/HealthSystem/HealthSystem.HealthSystem_C"))
  (Utilities|IsValid _returnvalue
    (:Is%20Valid
      (Default|TakeDamage _returnvalue false (Variables|Default|GetDamage))
      (Effects|SpawnEmitteratLocation "/Game/StarterContent/Particles/P_Explosion.P_Explosion" (Transformation|GetActorLocation))
      (Actor|DestroyActor))))

(fn ConstructionScript)