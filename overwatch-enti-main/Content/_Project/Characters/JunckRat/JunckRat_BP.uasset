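; JunckRat_BP is a playable character Blueprint that layers JunckRat's health pools and abilities onto a parent class.
; On BeginPlay it runs the parent logic, then initializes health, armor and shield values.
; Skill_6 input passes the GrenadeSpawnPoint world transform to RecruitGrenadeSkillBPC before firing it.
; Ultimate input fires the Ultimate object when it starts, leaving the ability logic outside this Blueprint.
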(event Input|EnhancedActionEvents|EnhancedInputActionUltimate
  (params (ActionValue :type Boolean) (ElapsedSeconds :type Float%20%28double-precision%29) (TriggeredSeconds :type Float%20%28double-precision%29) (InputAction :type Input%20Action%20Object%20Reference :default "/Game/_Project/CommonSystems/Input/Ultimate.Ultimate"))
  (:Started
    (Default|Fire (Variables|Default|GetUltimate))))

(event Input|EnhancedActionEvents|EnhancedInputActionSkill_6
  (params (ActionValue :type Boolean) (ElapsedSeconds :type Float%20%28double-precision%29) (TriggeredSeconds :type Float%20%28double-precision%29) (InputAction :type Input%20Action%20Object%20Reference :default "/Game/_Project/CommonSystems/Input/Skill_6.Skill_6"))
  (bind _recruit_grenade_skill_bpc (Variables|Default|GetRecruit_Grenade_Skill_BPC))
  (Variables|/Game/_Project/Characters/Recruit/Skills/Grenade/Recruit_Grenade_Skill_BPC.Recruit_Grenade_Skill_BPC_C|SetSpawnPoint _recruit_grenade_skill_bpc (Transformation|GetWorldTransform (Variables|Default|GetGrenadeSpawnPoint)))
  (Default|Fire _recruit_grenade_skill_bpc))

(event EventBeginPlay
  (|CallParentFunction)
  (Utilities|FlowControl|Sequence
    (:then_0
      (CallFunction|InitializeHealth (Utilities|Struct|MakeHealthData 125.0 125.0 5e+01 5e+01 5e+01 5e+01 0.0 false)))))

(fn ConstructionScript
  (|CallParentFunction))