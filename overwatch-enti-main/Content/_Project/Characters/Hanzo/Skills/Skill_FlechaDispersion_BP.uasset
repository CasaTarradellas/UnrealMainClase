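; Hanzo skill that temporarily switches his current weapon to an alternate arrow type, the dispersion arrow going by the asset name.
; Fire runs the parent logic and, in the required skill state, sets the weapon's active arrow index, starts a looping one-second timer and immediately calls Finish.
; The timer counts down ten seconds with debug prints, then restores the default index on the then-current Hanzo weapon and clears itself.
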(event Custom|ContarSegundo
  (bind _owningcharacter (Variables|Default|GetOwningCharacter))
  (bind _output_get (Variables|Default|SetTiempoRestante (- (Variables|Default|GetTiempoRestante) 1)))
  (Development|PrintString (Utilities|String|ToString(Integer) _output_get))
  (if (<= (Variables|Default|GetTiempoRestante) 0)
    (bind _ashanzo_weapon (Utilities|Casting|CastToHanzo_Weapon (Utilities|Array|Get(acopy) (Variables|/Game/_Project/Characters/BaseCharacter_BP.BaseCharacter_BP_C|GetWeapons _owningcharacter) (Variables|/Game/_Project/Characters/BaseCharacter_BP.BaseCharacter_BP_C|GetCurrentWeaponIndex _owningcharacter))))
    (Variables|/Game/_Project/Characters/Hanzo/Weapon/MainWeapon/Hanzo_Weapon.Hanzo_Weapon_C|SetIndiceFlechaActiva _ashanzo_weapon 0)
    (Utilities|Time|ClearandInvalidateTimerbyHandle (Variables|Default|GetManejadorTemporizador))))

(event EventFire
  (bind _owningcharacter (Variables|Default|GetOwningCharacter))
  (|CallParentFunction)
  (if (Utilities|Enum|Equal(Enum) (Variables|Default|GetState) "NewEnumerator1")
    (bind _ashanzo_weapon (Utilities|Casting|CastToHanzo_Weapon (Utilities|Array|Get(acopy) (Variables|/Game/_Project/Characters/BaseCharacter_BP.BaseCharacter_BP_C|GetWeapons _owningcharacter) (Variables|/Game/_Project/Characters/BaseCharacter_BP.BaseCharacter_BP_C|GetCurrentWeaponIndex _owningcharacter))))
    (Variables|/Game/_Project/Characters/Hanzo/Weapon/MainWeapon/Hanzo_Weapon.Hanzo_Weapon_C|SetIndiceFlechaActiva _ashanzo_weapon 1)
    (Variables|Default|SetTiempoRestante 10)
    (bind _returnvalue (Utilities|Time|SetTimerbyEvent (delegate Custom|ContarSegundo) 1.0 true))
    (Variables|Default|SetManejadorTemporizador _returnvalue)
    (CallFunction|Finish)))