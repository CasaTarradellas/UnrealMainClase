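; Hanzo's Sonic Arrow (Flecha Sónica) skill, which switches his bow to a special arrow type.
; Its Fire override runs the parent logic, then, in one specific skill state, casts the owner's current weapon to Hanzo_Weapon.
; It sets that weapon's active arrow index to the sonic slot and finishes the skill, with no arrow behavior of its own.
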(event EventFire
  (bind _owningcharacter (Variables|Default|GetOwningCharacter))
  (|CallParentFunction)
  (if (Utilities|Enum|Equal(Enum) (Variables|Default|GetState) "NewEnumerator1")
    (bind _ashanzo_weapon (Utilities|Casting|CastToHanzo_Weapon (Utilities|Array|Get(acopy) (Variables|/Game/_Project/Characters/BaseCharacter_BP.BaseCharacter_BP_C|GetWeapons _owningcharacter) (Variables|/Game/_Project/Characters/BaseCharacter_BP.BaseCharacter_BP_C|GetCurrentWeaponIndex _owningcharacter))))
    (Variables|/Game/_Project/Characters/Hanzo/Weapon/MainWeapon/Hanzo_Weapon.Hanzo_Weapon_C|SetIndiceFlechaActiva _ashanzo_weapon 2)
    (CallFunction|Finish)))