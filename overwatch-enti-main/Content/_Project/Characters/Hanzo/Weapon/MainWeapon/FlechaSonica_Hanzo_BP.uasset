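; Hanzo's sonic arrow projectile, which reveals nearby characters that have a HealthSystem.
; Its launch speed scales with the weapon's charge; on impact it stops and replays a timeline that pulses the Radar's scale five times before destroying itself.
; Radar overlaps toggle custom depth on character meshes, setting a stencil value for highlighting.
; On destruction, a sphere overlap sends zero-damage hits to pawns with a HealthSystem.
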(event OnComponentBeginOverlap(Radar)
  (params (OverlappedComponent :type Primitive%20Component%20Object%20Reference) (OtherActor :type Actor%20Object%20Reference) (OtherComp :type Primitive%20Component%20Object%20Reference) (OtherBodyIndex :type Integer) (bFromSweep :type Boolean) (SweepResult :type Hit%20Result%20Structure%20%28by%20ref%29))
  (Utilities|IsValid (Actor|GetComponentbyClass OtherActor "/Game/_Project/CommonSystems/HealthSystem/HealthSystem.HealthSystem_C")
    (:Is%20Valid
      (bind _ascharacter (Utilities|Casting|CastToCharacter OtherActor))
      (Rendering|SetRenderCustomDepth (Variables|/Script/Engine.Character|GetMesh _ascharacter) true)
      (Rendering|SetCustomDepthStencilValue (Variables|/Script/Engine.Character|GetMesh _ascharacter) 2))))

(event OnComponentHit(Sphere1)
  (params (HitComponent :type Primitive%20Component%20Object%20Reference) (OtherActor :type Actor%20Object%20Reference) (OtherComp :type Primitive%20Component%20Object%20Reference) (NormalImpulse :type Vector :default "0, 0, 0") (Hit :type Hit%20Result%20Structure%20%28by%20ref%29))
  (Components|Movement|StopMovementImmediately (Variables|Default|GetProjectileMovement))
  (bind _escala (Timeline|Timeline_Pulso PlayFromStart)
    (:Update
      (Transformation|SetRelativeScale3D (Variables|Default|GetRadar) (Math|Conversions|ToVector(Float) _escala)))
    (:Finished
      (Variables|Default|SetPulsosDados (+ (Variables|Default|GetPulsosDados) 1))
      (if (< (Variables|Default|GetPulsosDados) 5)
        (Timeline|Timeline_Pulso PlayFromStart)
        (else
          (Actor|DestroyActor))))))

(event OnComponentEndOverlap(Radar)
  (params (OverlappedComponent :type Primitive%20Component%20Object%20Reference) (OtherActor :type Actor%20Object%20Reference) (OtherComp :type Primitive%20Component%20Object%20Reference) (OtherBodyIndex :type Integer))
  (Utilities|IsValid (Actor|GetComponentbyClass OtherActor "/Game/_Project/CommonSystems/HealthSystem/HealthSystem.HealthSystem_C")
    (:Is%20Valid
      (Rendering|SetRenderCustomDepth (Actor|GetComponentbyClass OtherActor "/Script/Engine.SkeletalMeshComponent") false))))

(event Custom|CalcularVelocidadSonica
  (bind _miarma (Variables|Default|GetMiArma))
  (bind _output_get (Variables|/Script/Engine.MovementComponent|SetVelocity (Variables|Default|GetProjectileMovement) (* (Math|Float|Lerp 1.5e+03 6e+03 (/ (Variables|/Game/_Project/Characters/Hanzo/Weapon/MainWeapon/Hanzo_Weapon.Hanzo_Weapon_C|GetTiempoCargaActual _miarma) (Variables|/Game/_Project/Characters/Hanzo/Weapon/MainWeapon/Hanzo_Weapon.Hanzo_Weapon_C|GetTiempoCargaMax _miarma))) (Transformation|GetActorForwardVector))))
  (Development|PrintString (Utilities|String|ToString(Vector) _output_get)))

(event EventDestroyed
  (Utilities|FlowControl|Sequence
    (:then_1
      (bind (_outactors _returnvalue) (Collision|SphereOverlapActors (Transformation|GetActorLocation) 0.0 (Utilities|Array|MakeArray "ObjectTypeQuery3") 0))
      (if _returnvalue
        (for _array_element _outactors
          (Utilities|IsValid (Actor|GetComponentbyClass _array_element "/Game/_Project/CommonSystems/HealthSystem/HealthSystem.HealthSystem_C")
            (:Is%20Valid
              (Default|TakeDamage (Actor|GetComponentbyClass _array_element "/Game/_Project/CommonSystems/HealthSystem/HealthSystem.HealthSystem_C") false 0.0))))))
    (:then_3
      (Actor|DestroyActor))))

(fn ConstructionScript)