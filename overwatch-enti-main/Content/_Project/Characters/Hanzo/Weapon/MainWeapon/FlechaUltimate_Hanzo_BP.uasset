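; Hanzo's ultimate arrow projectile, which turns into a stationary emitter of dragon spheres (BP_EsferaDragon).
; Shortly after BeginPlay it freezes in the air, records its rotation and resets the owner's active arrow index.
; Parallel delays from a Sequence spawn five spheres at even intervals along that rotation, then destroy the arrow.
; A separate event sets launch speed from weapon charge, briefly disabling sphere collision.
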(event Custom|ActualizarVelocidadFisica
  (bind _miarma (Variables|Default|GetMiArma))
  (Collision|SetCollisionEnabled (Variables|Default|GetSphere1) "NoCollision")
  (bind _output_get (Variables|/Script/Engine.MovementComponent|SetVelocity (Variables|Default|GetProjectileMovement) (* (Math|Float|Lerp 1.5e+03 2.5e+03 (/ (Variables|/Game/_Project/Characters/Hanzo/Weapon/MainWeapon/Hanzo_Weapon.Hanzo_Weapon_C|GetTiempoCargaActual _miarma) (Variables|/Game/_Project/Characters/Hanzo/Weapon/MainWeapon/Hanzo_Weapon.Hanzo_Weapon_C|GetTiempoCargaMax _miarma))) (Transformation|GetActorForwardVector))))
  (Development|PrintString (Utilities|String|ToString(Vector) _output_get))
  (Utilities|FlowControl|Delay 0.05)
  (Collision|SetCollisionEnabled (Variables|Default|GetSphere1) "QueryAndPhysics"))

(event EventBeginPlay
  (bind _returnvalue (Transformation|GetActorLocation))
  (bind _projectilemovement (Variables|Default|GetProjectileMovement))
  (bind _owningcharacter (Variables|Default|GetOwningCharacter))
  (Utilities|FlowControl|Delay 0.15)
  (Components|Movement|StopMovementImmediately _projectilemovement)
  (Variables|/Script/Engine.ProjectileMovementComponent|SetProjectileGravityScale _projectilemovement 0.0)
  (bind _output_get (Variables|Default|SetDireccionDisparo (Transformation|GetActorRotation)))
  (bind _ashanzo_weapon (Utilities|Casting|CastToHanzo_Weapon (Utilities|Array|Get(acopy) (Variables|/Game/_Project/Characters/BaseCharacter_BP.BaseCharacter_BP_C|GetWeapons _owningcharacter) (Variables|/Game/_Project/Characters/BaseCharacter_BP.BaseCharacter_BP_C|GetCurrentWeaponIndex _owningcharacter))))
  (Variables|/Game/_Project/Characters/Hanzo/Weapon/MainWeapon/Hanzo_Weapon.Hanzo_Weapon_C|SetIndiceFlechaActiva _ashanzo_weapon 0)
  (Utilities|FlowControl|Sequence
    (:then_0
      (Game|SpawnActorfromClass "/Game/_Project/Characters/Hanzo/Weapon/MainWeapon/BP_EsferaDragon.BP_EsferaDragon_C" (Math|Transform|MakeTransform _returnvalue _output_get "1.000000,1.000000,1.000000") "Undefined" "MultiplyWithRoot" 0 0))
    (:then_1
      (Utilities|FlowControl|Delay 2.0)
      (Game|SpawnActorfromClass "/Game/_Project/Characters/Hanzo/Weapon/MainWeapon/BP_EsferaDragon.BP_EsferaDragon_C" (Math|Transform|MakeTransform _returnvalue _output_get "1.000000,1.000000,1.000000") "Undefined" "MultiplyWithRoot" 0 0))
    (:then_2
      (Utilities|FlowControl|Delay 4.0)
      (Game|SpawnActorfromClass "/Game/_Project/Characters/Hanzo/Weapon/MainWeapon/BP_EsferaDragon.BP_EsferaDragon_C" (Math|Transform|MakeTransform _returnvalue _output_get "1.000000,1.000000,1.000000") "Undefined" "MultiplyWithRoot" 0 0))
    (:then_3
      (Utilities|FlowControl|Delay 6.0)
      (Game|SpawnActorfromClass "/Game/_Project/Characters/Hanzo/Weapon/MainWeapon/BP_EsferaDragon.BP_EsferaDragon_C" (Math|Transform|MakeTransform _returnvalue _output_get "1.000000,1.000000,1.000000") "Undefined" "MultiplyWithRoot" 0 0))
    (:then_4
      (Utilities|FlowControl|Delay 8.0)
      (Game|SpawnActorfromClass "/Game/_Project/Characters/Hanzo/Weapon/MainWeapon/BP_EsferaDragon.BP_EsferaDragon_C" (Math|Transform|MakeTransform _returnvalue _output_get "1.000000,1.000000,1.000000") "Undefined" "MultiplyWithRoot" 0 0)
      (Actor|DestroyActor))))

(fn ConstructionScript)