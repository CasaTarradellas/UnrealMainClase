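; Arrow projectile for Hanzo's main weapon that damages any HealthSystem it strikes, in normal or ricochet (EsRebotada) mode.
; Launch speed scales with the weapon's charge time, with collision briefly disabled after firing.
; Normal hits feed the owner's ultimate charge with a headshot-specific amount; ricochet arrows damage through bounce events and expire after a bounce limit.
; On destruction, a sphere overlap sends zero-damage calls to nearby pawns.
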(event OnProjectileBounce(ProjectileMovement)
  (params (ImpactResult :type Hit%20Result%20Structure%20%28by%20ref%29) (ImpactVelocity :type Vector%20%28by%20ref%29 :default "0, 0, 0"))
  (bind _returnvalue (Actor|GetComponentbyClass (.hitactor ImpactResult) "/Game/_Project/CommonSystems/HealthSystem/HealthSystem.HealthSystem_C"))
  (if (Variables|Default|GetEsRebotada)
    (bind _output_get (Variables|Default|SetContadorRebotes (+ (Variables|Default|GetContadorRebotes) 1)))
    (if (>= _output_get 5)
      (Actor|DestroyActor)
      (else
        (Utilities|IsValid _returnvalue
          (:Is%20Valid
            (Default|TakeDamage _returnvalue false (Variables|Default|GetDamage))
            (Actor|DestroyActor)))))
    (else
      (Actor|DestroyActor))))

(event OnComponentHit(Sphere1)
  (params (HitComponent :type Primitive%20Component%20Object%20Reference) (OtherActor :type Actor%20Object%20Reference) (OtherComp :type Primitive%20Component%20Object%20Reference) (NormalImpulse :type Vector :default "0, 0, 0") (Hit :type Hit%20Result%20Structure%20%28by%20ref%29))
  (bind _returnvalue (Actor|GetComponentbyClass OtherActor "/Game/_Project/CommonSystems/HealthSystem/HealthSystem.HealthSystem_C"))
  (if (not (Variables|Default|GetEsRebotada))
    (Utilities|IsValid _returnvalue
      (:Is%20Valid
        (Default|TakeDamage _returnvalue false (Variables|Default|GetDamage))
        (Default|AddCharge (Variables|/Game/_Project/Characters/BaseCharacter_BP.BaseCharacter_BP_C|GetUltimate (Variables|Default|GetOwningCharacter)) (Math|Float|SelectFloat (Variables|Default|GetUltimateChargePerHeadshot) (Variables|Default|GetUltimateChargePerHit) (== (.HitBoneName (Collision|BreakHitResult Hit)) "Head")))
        (Actor|DestroyActor)))))

(event Custom|ActualizarVelocidadFisica
  (bind _miarma (Variables|Default|GetMiArma))
  (Collision|SetCollisionEnabled (Variables|Default|GetSphere1) "NoCollision")
  (bind _output_get (Variables|/Script/Engine.MovementComponent|SetVelocity (Variables|Default|GetProjectileMovement) (* (Math|Float|Lerp 1.5e+03 6e+03 (/ (Variables|/Game/_Project/Characters/Hanzo/Weapon/MainWeapon/Hanzo_Weapon.Hanzo_Weapon_C|GetTiempoCargaActual _miarma) (Variables|/Game/_Project/Characters/Hanzo/Weapon/MainWeapon/Hanzo_Weapon.Hanzo_Weapon_C|GetTiempoCargaMax _miarma))) (Transformation|GetActorForwardVector))))
  (Development|PrintString (Utilities|String|ToString(Vector) _output_get))
  (Utilities|FlowControl|Delay 0.05)
  (Collision|SetCollisionEnabled (Variables|Default|GetSphere1) "QueryAndPhysics"))

(event EventDestroyed
  (Utilities|FlowControl|Sequence
    (:then_1
      (bind (_outactors _returnvalue) (Collision|SphereOverlapActors (Transformation|GetActorLocation) 0.0 (Utilities|Array|MakeArray "ObjectTypeQuery3") 0))
      (if _returnvalue
        (for _array_element _outactors
          (Utilities|IsValid (Actor|GetComponentbyClass _array_element "/Game/_Project/CommonSystems/HealthSystem/HealthSystem.HealthSystem_C")
            (:Is%20Valid
              (Default|TakeDamage (Actor|GetComponentbyClass _array_element "/Game/_Project/CommonSystems/HealthSystem/HealthSystem.HealthSystem_C") false 0.0))))))
    (:then_3
      (Actor|DestroyActor))))

(fn ConstructionScript)