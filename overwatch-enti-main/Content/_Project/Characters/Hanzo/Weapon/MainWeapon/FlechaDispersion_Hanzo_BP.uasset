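; Projectile for Hanzo's dispersion arrow, which bursts into multiple arrows on impact.
; Its launch speed interpolates with the weapon's charge time.
; On hit it damages any HealthSystem, then spawns ten Flecha_Hanzo_BP arrows flagged as bounced, offset along the surface normal with random pitch and yaw spread, and destroys itself.
; On destruction, a pawn sphere overlap sends zero-damage hits and adds owner ultimate charge.
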(event OnComponentHit(Sphere1)
  (params (HitComponent :type Primitive%20Component%20Object%20Reference) (OtherActor :type Actor%20Object%20Reference) (OtherComp :type Primitive%20Component%20Object%20Reference) (NormalImpulse :type Vector :default "0, 0, 0") (Hit :type Hit%20Result%20Structure%20%28by%20ref%29))
  (bind (_bblockinghit _binitialoverlap _time _distance _location _impactpoint _normal _impactnormal) (Collision|BreakHitResult Hit))
  (bind _returnvalue (Actor|GetComponentbyClass OtherActor "/Game/_Project/CommonSystems/HealthSystem/HealthSystem.HealthSystem_C"))
  (bind _returnvalue_2 (Transformation|GetActorRotation))
  (bind (_roll _pitch _yaw) (Math|Rotator|BreakRotator _returnvalue_2))
  (Utilities|IsValid _returnvalue
    (:Is%20Valid
      (Default|TakeDamage _returnvalue false (Variables|Default|GetDamage)))
    (:Is%20Not%20Valid
      _))
  (for _index (range 1 10)
    (bind _returnvalue_3 (Game|SpawnActorfromClass "/Game/_Project/Characters/Hanzo/Weapon/MainWeapon/Flecha_Hanzo_BP.Flecha_Hanzo_BP_C" (Math|Transform|MakeTransform (+ (* _impactnormal 1e+02) _impactpoint) (Math|Rotator|MakeRotator _roll (+ _pitch (Math|Random|RandomFloatinRange -15.0 15.0)) (+ _yaw (Math|Random|RandomFloatinRange -15.0 15.0))) "1.000000,1.000000,1.000000") "AlwaysSpawn" "MultiplyWithRoot" 0 (Variables|Default|GetMiArma) true (Variables|Actor|GetInstigator)))
    (Default|ActualizarVelocidadFisica _returnvalue_3))
  (Actor|DestroyActor))

(event Custom|CalcularVelocidadDispersion
  (bind _miarma (Variables|Default|GetMiArma))
  (bind _output_get (Variables|/Script/Engine.MovementComponent|SetVelocity (Variables|Default|GetProjectileMovement) (* (Math|Float|Lerp 1.5e+03 6e+03 (/ (Variables|/Game/_Project/Characters/Hanzo/Weapon/MainWeapon/Hanzo_Weapon.Hanzo_Weapon_C|GetTiempoCargaActual _miarma) (Variables|/Game/_Project/Characters/Hanzo/Weapon/MainWeapon/Hanzo_Weapon.Hanzo_Weapon_C|GetTiempoCargaMax _miarma))) (Transformation|GetActorForwardVector))))
  (Development|PrintString (Utilities|String|ToString(Vector) _output_get)))

(event EventDestroyed
  (Utilities|FlowControl|Sequence
    (:then_1
      (bind (_outactors _returnvalue) (Collision|SphereOverlapActors (Transformation|GetActorLocation) 0.0 (Utilities|Array|MakeArray "ObjectTypeQuery3") 0))
      (if _returnvalue
        (for _array_element _outactors
          (Utilities|IsValid (Actor|GetComponentbyClass _array_element "/Game/_Project/CommonSystems/HealthSystem/HealthSystem.HealthSystem_C")
            (:Is%20Valid
              (Default|TakeDamage (Actor|GetComponentbyClass _array_element "/Game/_Project/CommonSystems/HealthSystem/HealthSystem.HealthSystem_C") false 0.0)
              (Default|AddCharge (Variables|/Game/_Project/Characters/BaseCharacter_BP.BaseCharacter_BP_C|GetUltimate (Variables|Default|GetOwningCharacter)) (Math|Float|SelectFloat (Variables|Default|GetUltimateChargePerHeadshot) (Variables|Default|GetUltimateChargePerHit) false)))))))
    (:then_3
      (Actor|DestroyActor))))

(fn ConstructionScript)