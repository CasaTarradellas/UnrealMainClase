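; Dragon sphere for Hanzo's main weapon that travels forward and repeatedly damages actors with a HealthSystem component.
; Tick adds a fixed local forward offset without sweep or delta-time scaling, and the actor destroys itself ten seconds after BeginPlay.
; Sphere overlap starts a looping damage timer on a single stored handle, applying non-headshot damage to the last overlapped actor.
; Any end overlap clears that timer.
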(event OnComponentBeginOverlap(Sphere)
  (params (OverlappedComponent :type Primitive%20Component%20Object%20Reference) (OtherActor :type Actor%20Object%20Reference) (OtherComp :type Primitive%20Component%20Object%20Reference) (OtherBodyIndex :type Integer) (bFromSweep :type Boolean) (SweepResult :type Hit%20Result%20Structure%20%28by%20ref%29))
  (Utilities|IsValid (Actor|GetComponentbyClass OtherActor "/Game/_Project/CommonSystems/HealthSystem/HealthSystem.HealthSystem_C")
    (:Is%20Valid
      (bind _returnvalue (Utilities|Time|SetTimerbyEvent (delegate Custom|HacerDañoDragón) 0.3 true))
      (bind _output_get (Variables|Default|SetTimerDaño _returnvalue)))))

(event OnComponentEndOverlap(Sphere)
  (params (OverlappedComponent :type Primitive%20Component%20Object%20Reference) (OtherActor :type Actor%20Object%20Reference) (OtherComp :type Primitive%20Component%20Object%20Reference) (OtherBodyIndex :type Integer))
  (Utilities|Time|ClearandInvalidateTimerbyHandle (stale OnComponentBeginOverlap(Sphere) _output_get)))

(event Custom|HacerDañoDragón
  (Utilities|IsValid (Actor|GetComponentbyClass (stale OnComponentBeginOverlap(Sphere) OtherActor) "/Game/_Project/CommonSystems/HealthSystem/HealthSystem.HealthSystem_C")
    (:Is%20Valid
      (Default|TakeDamage (Actor|GetComponentbyClass (stale OnComponentBeginOverlap(Sphere) OtherActor) "/Game/_Project/CommonSystems/HealthSystem/HealthSystem.HealthSystem_C") false (Variables|Default|GetDamage)))))

(event EventTick
  (params (DeltaSeconds :type Float%20%28single-precision%29))
  (Transformation|AddActorLocalOffset "10.000000,0.000000,0.000000" false false))

(event EventBeginPlay
  (Utilities|FlowControl|Delay 1e+01)
  (Actor|DestroyActor))

(fn ConstructionScript)