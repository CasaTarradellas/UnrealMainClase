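; Playable Hanzo hero character with layered health, armor and shield, destroyed when its health runs out.
; On BeginPlay it sets up health and registers the Dispersion and Sonic arrow skills, which fire from input actions alongside an Ultimate.
; Holding Jump climbs walls found by a forward line trace, using Flying movement and upward input within a time budget.
; Releasing Jump or running out of time ends the climb until landing restores it.
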(event OnTakenDamage(HealthSystem)
  (if (<= (.CurrentHealth (Utilities|Struct|BreakHealthData (Default|GetHealthData (Variables|Default|GetHealthSystem)))) 0.0)
    (Actor|DestroyActor)))

(event Input|EnhancedActionEvents|EnhancedInputActionSkill_3
  (params (ActionValue :type Boolean) (ElapsedSeconds :type Float%20%28double-precision%29) (TriggeredSeconds :type Float%20%28double-precision%29) (InputAction :type Input%20Action%20Object%20Reference :default "/Game/_Project/CommonSystems/Input/Skill_3.Skill_3"))
  (:Started
    (Default|Fire (Variables|Default|GetSkill_FlechaDispersion_BP))))

(event Input|EnhancedActionEvents|EnhancedInputActionSkill_4
  (params (ActionValue :type Boolean) (ElapsedSeconds :type Float%20%28double-precision%29) (TriggeredSeconds :type Float%20%28double-precision%29) (InputAction :type Input%20Action%20Object%20Reference :default "/Game/_Project/CommonSystems/Input/Skill_4.Skill_4"))
  (:Started
    (Default|Fire (Variables|Default|GetSkill_FlechaSonica_BP))))

(event Input|EnhancedActionEvents|EnhancedInputActionUltimate
  (params (ActionValue :type Boolean) (ElapsedSeconds :type Float%20%28double-precision%29) (TriggeredSeconds :type Float%20%28double-precision%29) (InputAction :type Input%20Action%20Object%20Reference :default "/Game/_Project/CommonSystems/Input/Ultimate.Ultimate"))
  (:Started
    (Default|Fire (Variables|Default|GetUltimate))))

(event Input|EnhancedActionEvents|EnhancedInputActionJump
  (params (ActionValue :type Boolean) (ElapsedSeconds :type Float%20%28double-precision%29) (TriggeredSeconds :type Float%20%28double-precision%29) (InputAction :type Input%20Action%20Object%20Reference :default "/Game/_Project/CommonSystems/Input/Jump.Jump"))
  (:Started
    (Character|Jump))
  (:Ongoing
    (bind _newparam (CallFunction|WallClimb))
    (if _newparam
      (Pawn|Components|CharacterMovement|SetMovementMode (Variables|Character|GetCharacterMovement) "MOVE_Flying" 0)
      (Pawn|Input|AddMovementInput "0.000000,0.000000,0.500000" 1.0 false)
      (bind _output_get (Variables|Default|SetWallClimbTime (- (Variables|Default|GetWallClimbTime) (Utilities|Time|GetWorldDeltaSeconds))))
      (if (< _output_get 0.0)
        (Variables|Default|SetCanClimb false)
        (Pawn|Components|CharacterMovement|SetMovementMode (Variables|Character|GetCharacterMovement) "MOVE_Falling" 0))
      (else
        (Pawn|Components|CharacterMovement|SetMovementMode (Variables|Character|GetCharacterMovement) "MOVE_Falling" 0))))
  (:Canceled
    (Character|StopJumping :!label _label)
    (Pawn|Components|CharacterMovement|SetMovementMode (Variables|Character|GetCharacterMovement) "MOVE_Falling" 0)
    (Variables|Default|SetCanClimb false))
  (:Completed
    (goto _label)))

(event EventBeginPlay
  (bind _skill_flechasonica_bp (Variables|Default|GetSkill_FlechaSonica_BP))
  (bind _skill_flechadispersion_bp (Variables|Default|GetSkill_FlechaDispersion_BP))
  (|CallParentFunction)
  (Utilities|FlowControl|Sequence
    (:then_0
      (CallFunction|InitializeHealth (Utilities|Struct|MakeHealthData 125.0 125.0 5e+01 5e+01 5e+01 5e+01 0.0 false)))
    (:then_1
      (Default|Initialize _skill_flechadispersion_bp self "E")
      (Utilities|Array|Add (Variables|Default|GetSkills) _skill_flechadispersion_bp))
    (:then_2
      (Default|Initialize _skill_flechasonica_bp self "L SHIFT")
      (Utilities|Array|Add (Variables|Default|GetSkills) _skill_flechasonica_bp))))

(event EventOnLanded
  (params (Hit :type Hit%20Result%20Structure%20%28by%20ref%29))
  (Variables|Default|SetWallClimbTime (Variables|Default|GetMaxWallClimbTime))
  (Variables|Default|SetCanClimb true))

(fn ConstructionScript
  (|CallParentFunction))

(fn WallClimb
  (bind _returnvalue (Collision|LineTraceByChannel (Transformation|GetActorLocation) (+ (Transformation|GetActorLocation) (* (Transformation|GetActorForwardVector) 1.5e+02)) "TraceTypeQuery1" false 0 "ForDuration"))
  (return (and _returnvalue (Variables|Default|GetCanClimb))))